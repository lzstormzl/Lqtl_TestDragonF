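; Inventory component that stores food, ingredient and key items, and creates inventory and cooking widgets, with B showing the player inventory.
; AddItemToInventory uses DT_ItemData to route stack changes into per-type arrays and an ItemID-to-amount map, firing OnItemChange only for existing stacks.
; Amount checks read that map, while UsingFood applies DT_Item_Food effects through the buff manager.
; RemoveItemFromInventory is an empty stub, and depleted stacks always remove index 0.
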(event EventBeginPlay
  (bind _returnvalue (UserInterface|CreateWidget "/Game/GeneralSocial/2_GameSystems/7_InventorySystem/Widget/WBP_PlayerInventory1.WBP_PlayerInventory1_C"))
  (Variables|Default|SetPlayerInventoryWidget _returnvalue)
  (bind _returnvalue_2 (UserInterface|CreateWidget "/Game/GeneralSocial/2_GameSystems/7_InventorySystem/Widget/W_CookInventory_VER2.W_CookInventory_VER2_C"))
  (Variables|Default|SetCookInventory _returnvalue_2)
  (bind _returnvalue_3 (UserInterface|CreateWidget "/Game/GeneralSocial/1_Social/Minigame-Resources/Cooking/W_Cooking.W_Cooking_C"))
  (Variables|Default|SetCookingMiniGame _returnvalue_3))

(event Input|KeyboardEvents|B
  (params (Key :type Key%20Structure))
  (:Pressed
    (UserInterface|Viewport|AddtoViewport (Variables|Default|GetPlayerInventoryWidget) 0)
    (Variables|/Script/Engine.PlayerController|SetbShowMouseCursor (Game|GetPlayerController 0) true)))

(fn AddItemtoInventory
  (params (ItemID :type Name) (Amount :type Integer))
  (bind _itemininventory (Variables|Default|GetItemInInventory))
  (bind _itemininventory_2 (Variables|Default|GetItemInInventory))
  (bind _itemininventory_3 (Variables|Default|GetItemInInventory))
  (bind _itemininventory_4 (Variables|Default|GetItemInInventory))
  (bind _itemininventory_5 (Variables|Default|GetItemInInventory))
  (bind _itemininventory_6 (Variables|Default|GetItemInInventory))
  (bind _returnvalue (Utilities|GetDataTableRow "/Game/GeneralSocial/Config/DataTableConfig/Item/DT_ItemData.DT_ItemData" ItemID)
    (:then
      (switch Utilities|FlowControl|Switch|SwitchonE_ItemCategory (.Type (Utilities|Struct|BreakF_ItemData _returnvalue))
        (:NewEnumerator1
          ;[0 0 0] Food Inventory
          (for (_array_element _array_index) (Variables|Default|GetFoodInventory)
            (if (== (.ItemID (Utilities|Struct|BreakF_InventorySlot _array_element)) (.ItemID (Utilities|Struct|BreakF_ItemData _returnvalue)))
              (if (<= (+ (.Amount (Utilities|Struct|BreakF_InventorySlot _array_element)) Amount) 0)
                (Utilities|Array|RemoveIndex (Variables|Default|GetFoodInventory))
                (Utilities|Map|Remove (Variables|Default|GetItemInInventory) ItemID)
                (else
                  (Utilities|Array|SetArrayElem (Variables|Default|GetFoodInventory) _array_index (Utilities|Struct|MakeF_InventorySlot (.ItemID (Utilities|Struct|BreakF_InventorySlot _array_element)) (+ (.Amount (Utilities|Struct|BreakF_InventorySlot _array_element)) Amount)))))
              (Utilities|Map|Add _itemininventory_3 ItemID (+ (.Value (Utilities|Map|Find _itemininventory_3 ItemID)) Amount))
              (Default|CallOnItemChange ItemID)
              (return)))
          (Utilities|Array|Add (Variables|Default|GetFoodInventory) (Utilities|Struct|MakeF_InventorySlot (.ItemID (Utilities|Struct|BreakF_ItemData _returnvalue)) Amount))
          (Utilities|Map|Add _itemininventory_4 ItemID (+ (.Value (Utilities|Map|Find _itemininventory_4 ItemID)) Amount)))
        (:NewEnumerator3
          ;[0 0 0] Ingredient Inventory
          (for (_array_element_2 _array_index_2) (Variables|Default|GetIngredientInventory)
            (if (== (.ItemID (Utilities|Struct|BreakF_InventorySlot _array_element_2)) ItemID)
              (if (<= (+ (.Amount (Utilities|Struct|BreakF_InventorySlot _array_element_2)) Amount) 0)
                (Utilities|Array|RemoveIndex (Variables|Default|GetIngredientInventory))
                (Utilities|Map|Remove (Variables|Default|GetItemInInventory) ItemID)
                (else
                  (Utilities|Array|SetArrayElem (Variables|Default|GetIngredientInventory) _array_index_2 (Utilities|Struct|MakeF_InventorySlot (.ItemID (Utilities|Struct|BreakF_InventorySlot _array_element_2)) (+ (.Amount (Utilities|Struct|BreakF_InventorySlot _array_element_2)) Amount)))))
              (Utilities|Map|Add _itemininventory_5 ItemID (+ (.Value (Utilities|Map|Find _itemininventory_5 ItemID)) Amount))
              (Default|CallOnItemChange ItemID)
              (return)))
          (Utilities|Array|Add (Variables|Default|GetIngredientInventory) (Utilities|Struct|MakeF_InventorySlot ItemID Amount))
          (Utilities|Map|Add _itemininventory_6 ItemID (+ (.Value (Utilities|Map|Find _itemininventory_6 ItemID)) Amount)))
        (:NewEnumerator4
          ;[0 0 0] KeyItem Inventory
          (for (_array_element_3 _array_index_3) (Variables|Default|GetKeyItemInventory)
            (if (== (.ItemID (Utilities|Struct|BreakF_InventorySlot _array_element_3)) ItemID)
              (if (<= (+ (.Amount (Utilities|Struct|BreakF_InventorySlot _array_element_3)) Amount) 0)
                (Utilities|Array|RemoveIndex (Variables|Default|GetKeyItemInventory))
                (Utilities|Map|Remove (Variables|Default|GetItemInInventory) ItemID)
                (else
                  (Utilities|Array|SetArrayElem (Variables|Default|GetKeyItemInventory) _array_index_3 (Utilities|Struct|MakeF_InventorySlot (.ItemID (Utilities|Struct|BreakF_InventorySlot _array_element_3)) (+ (.Amount (Utilities|Struct|BreakF_InventorySlot _array_element_3)) Amount)))))
              (Utilities|Map|Add _itemininventory_2 ItemID (+ (.Value (Utilities|Map|Find _itemininventory_2 ItemID)) Amount))
              (Default|CallOnItemChange ItemID)
              (return)))
          (Utilities|Array|Add (Variables|Default|GetKeyItemInventory) (Utilities|Struct|MakeF_InventorySlot ItemID Amount))
          (Utilities|Map|Add _itemininventory ItemID (+ (.Value (Utilities|Map|Find _itemininventory ItemID)) Amount)))))))

(fn RemoveItemfromInventory
  (params (ItemID :type Name) (Amount :type Integer))
  (bind _returnvalue (Utilities|GetDataTableRow "/Game/GeneralSocial/Config/DataTableConfig/Item/DT_ItemData.DT_ItemData" ItemID)
    (:then
      (switch Utilities|FlowControl|Switch|SwitchonE_ItemCategory (.Type (Utilities|Struct|BreakF_ItemData _returnvalue))))))

(fn CheckItemAmountinInventory
  (params (ItemID :type Name) (Amount :type Integer))
  (return (>= (.Value (Utilities|Map|Find (Variables|Default|GetItemInInventory) ItemID)) Amount)))

(fn CheckItemsAmount
  (params (ItemID :type Array%20of%20F%20Check%20Item%20Inventory%20Structures))
  (for _array_element ItemID
    (if (not (CallFunction|CheckItemAmountinInventory (.ItemID (Utilities|Struct|BreakF_CheckItemInventory _array_element)) (.Amount (Utilities|Struct|BreakF_CheckItemInventory _array_element))))
      (return false)))
  (return true))

(fn FindIngredientinInventorybyID
  (params (IngredientID :type Name))
  (for (_array_element _array_index) (Variables|Default|GetIngredientInventory)
    (if (== IngredientID (.ItemID (Utilities|Struct|BreakF_InventorySlot _array_element)))
      (return true (Utilities|Struct|MakeF_Item_IngredientSlot (.ItemID (Utilities|Struct|BreakF_InventorySlot _array_element)) (.Amount (Utilities|Struct|BreakF_InventorySlot _array_element))) _array_index)))
  (return false "" 0))

(fn UsingFood
  (params (ItemID :type Name) (Actor :type Actor%20Object%20Reference))
  (bind _returnvalue (Utilities|GetDataTableRow "/Game/GeneralSocial/Config/DataTableConfig/Item/Food/DT_Item_Food.DT_Item_Food" ItemID)
    (:then
      (for _array_element (.EffectAfterUsing (Utilities|Struct|BreakF_Item_Food _returnvalue))
        (Default|AddBufftoActor (CallFunction|GetBuffManager) (.BuffID (Utilities|Struct|BreakAddBuffStruct _array_element)) (.Count (Utilities|Struct|BreakAddBuffStruct _array_element)) Actor)))))