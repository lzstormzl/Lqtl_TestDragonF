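; Schedule manager for the social game: tracks action cards in hand and across every date and session.
; BeginPlay creates the schedule widget and builds the day map from calendar and phase DataTables.
; Card functions add or remove cards in both maps; deadline checks on hand and previous slot apply buff and stat consequences.
; DoAction handles sleeping and house cleaning with energy checks, stat changes and CalendarManager phase advances.
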(event Custom|DoAction
  (params (Action :type E_SocialAction%20Enum :default "NewEnumerator0"))
  (bind _asthuy_tinh_game_instance (CallFunction|GetGameInstance))
  (bind _notifywidget (Variables|/Game/GeneralSocial/ThuyTinh_GameInstance.ThuyTinh_GameInstance_C|GetNotifyWidget _asthuy_tinh_game_instance))
  (switch Utilities|FlowControl|Switch|SwitchonE_SocialAction Action
    (:NewEnumerator0
      (if (>= (Utilities|Struct|BreakPlayerStatStruct (.Value (Utilities|Map|Find (Variables|Default|GetPlayerSocialStats (CallFunction|GetPlayerCharacterSocial)) "Energy"))) 8)
        (Default|ShowWidget _notifywidget "Bạn đang còn nhiều hơn 8 năng lượng, bạn có muốn đi ngủ sớm không?")
        (EventDispatchers|BindEventtoOnYesBtnClick _notifywidget (delegate Custom|SleepEarlyEvent))
        (else
          (Default|AdvancedPhasewithTransition (CallFunction|GetCalendarManager "__WorldContext")))))
    (:NewEnumerator1
      (if (>= (Utilities|Struct|BreakPlayerStatStruct (.Value (Utilities|Map|Find (Variables|Default|GetPlayerSocialStats (CallFunction|GetPlayerCharacterSocial)) "Energy"))) 8)
        (if (.ReturnValue (Utilities|Map|Find (Variables|Default|GetActionCardInHand) "CardDonNha"))
          (CallFunction|PlusPlayerStat (CallFunction|GetPlayerCharacterSocial) (Utilities|Name|MakeLiteralName "Energy") -8)
          (CallFunction|PlusPlayerStat (CallFunction|GetPlayerCharacterSocial) (Utilities|Name|MakeLiteralName "Mood") 2)
          (CallFunction|PlusPlayerStat (CallFunction|GetPlayerCharacterSocial) (Utilities|Name|MakeLiteralName "Empathy") 2)
          (CallFunction|RemoveActionCard "CardDonNha" 1)
          (Default|AdvancedPhasewithTransition (CallFunction|GetCalendarManager "__WorldContext"))
          (else
            (Default|ShowWidget (Variables|/Game/GeneralSocial/ThuyTinh_GameInstance.ThuyTinh_GameInstance_C|GetNotifyWidget (CallFunction|GetGameInstance)) "Bạn đã hết số lần dọn nhà trong ngày hôm nay")))
        (else
          (Default|ShowWidget (Variables|/Game/GeneralSocial/ThuyTinh_GameInstance.ThuyTinh_GameInstance_C|GetNotifyWidget (CallFunction|GetGameInstance)) "Không đủ năng lượng để làm việc này"))))))

(event Custom|SleepEarlyEvent
  (EventDispatchers|UnbindEventfromOnYesBtnClick (Variables|/Game/GeneralSocial/ThuyTinh_GameInstance.ThuyTinh_GameInstance_C|GetNotifyWidget (CallFunction|GetGameInstance)) (delegate Custom|SleepEarlyEvent))
  (CallFunction|PlusPlayerStat (CallFunction|GetPlayerCharacterSocial) (Utilities|Name|MakeLiteralName "Energy") -8)
  (CallFunction|PlusPlayerStat (CallFunction|GetPlayerCharacterSocial) (Utilities|Name|MakeLiteralName "Mood") 2)
  (Default|AdvancedPhasewithTransition (CallFunction|GetCalendarManager "__WorldContext")))

(event EventBeginPlay
  (bind _returnvalue (UserInterface|CreateWidget "/Game/GeneralSocial/2_GameSystems/ScheduleNActionSystem/Widget/WBP_Schedule.WBP_Schedule_C" 0 0))
  (Variables|Default|SetScheduleWidget _returnvalue)
  (bind _outrownames (DataTable|GetDataTableRowNames "/Game/GeneralSocial/Config/DataTableConfig/Calendar/calendar_config_DT.calendar_config_DT"))
  (for (_array_element _array_index) _outrownames
    (bind _returnvalue_2 (Utilities|GetDataTableRow "/Game/GeneralSocial/Config/DataTableConfig/Calendar/calendar_config_DT.calendar_config_DT" _array_element)
      (:then
        (for _array_element_2 0
          (bind _returnvalue_3 (Utilities|GetDataTableRow "/Game/GeneralSocial/Config/DataTableConfig/Calendar/phase_definition_DT.phase_definition_DT" _array_element_2)
            (:then
              (if (Utilities|Enum|Equal(Enum) (.LogicType (Utilities|Struct|Breakphase_definition_struct _returnvalue_3)) "NewEnumerator1")
                (Utilities|GetDataTableRow "/Game/GeneralSocial/Config/DataTableConfig/Schedule/CardAction/cardAction_DT.cardAction_DT" "Card1"
                  (:then
                    (Utilities|Map|Add (Variables|Default|GetAllDayOfTheGame) (Utilities|Struct|Makeday_struct (+ _array_index 1) (.DaySession (Utilities|Struct|Breakphase_definition_struct _returnvalue_3))) (Utilities|Struct|MakeSlotCardInfo (Utilities|Struct|MakeActionCardInstance "Card1" "(DateID_18_A54FD76948BCD213AB255C971713BD05=0,Session_14_6DEB00FF45B05840D15569ADE967686A=NewEnumerator0)" "(AddBuff_6_87218DC44706387E9EE1F08D67D90F3E=,AddStats_7_5679C485426186DCCA2402A51ED86910=)") true))))
                (elif (Utilities|Enum|Equal(Enum) (.LogicType (Utilities|Struct|Breakphase_definition_struct _returnvalue_3)) "NewEnumerator0")
                  (Utilities|Map|Add :TargetMap (Variables|Default|GetAllDayOfTheGame) :Key (Utilities|Struct|Makeday_struct (+ _array_index 1) (.DaySession (Utilities|Struct|Breakphase_definition_struct _returnvalue_3)))))))))))))

(fn ConstructionScript)

(fn AddActionCardtoTimeOftheGame
  (params (CardID :type Name) (Time :type Day%20Struct%20Structure) (Card%20Deadline :type Day%20Struct%20Structure) (Consequence :type Consequence%20Struct%20Structure))
  (Utilities|GetDataTableRow "/Game/GeneralSocial/Config/DataTableConfig/Schedule/CardAction/cardAction_DT.cardAction_DT" CardID
    (:then
      (Utilities|Map|Add (Variables|Default|GetAllDayOfTheGame) Time (Utilities|Struct|MakeSlotCardInfo (Utilities|Struct|MakeActionCardInstance CardID Card%20Deadline Consequence) true)))))

(fn RemoveActionCardfromTimeOftheGame
  (params (Time :type Day%20Struct%20Structure%20%28by%20ref%29))
  (Utilities|Map|Add :TargetMap (Variables|Default|GetAllDayOfTheGame) :Key Time))

(fn FindandRemoveActionCardonSchedule
  (params (CardID :type Name) (Amount :type Integer))
  (bind _keys (Utilities|Map|Keys (Variables|Default|GetAllDayOfTheGame)))
  (for _array_element _keys
    (if (>= (.DateID (Utilities|Struct|Breakday_struct _array_element)) (Variables|/Game/GeneralSocial/2_GameSystems/1_CalendarSystem/BP_CalendarManager.BP_CalendarManager_C|GetCurrentDateID (CallFunction|GetCalendarManager "__WorldContext")))
      (if (== (.CardID (Utilities|Struct|BreakActionCardInstance (Utilities|Struct|BreakSlotCardInfo (.Value (Utilities|Map|Find (Variables|Default|GetAllDayOfTheGame) (Utilities|Struct|Makeday_struct (.DateID (Utilities|Struct|Breakday_struct _array_element)) (.Session (Utilities|Struct|Breakday_struct _array_element)))))))) CardID)
        (Math|Integer|IncrementInt (LocalVariables|GetCount)
          (:%20%20
            (CallFunction|RemoveActionCardfromTimeOftheGame (Utilities|Struct|Makeday_struct (.DateID (Utilities|Struct|Breakday_struct _array_element)) (.Session (Utilities|Struct|Breakday_struct _array_element))))
            (if (== (LocalVariables|GetCount) Amount)
              (return))))))))

(fn AddActionCardtoHand
  (params (CardID :type Name) (Amount :type Integer) (Card%20Deadline :type Day%20Struct%20Structure) (Consequence :type Consequence%20Struct%20Structure))
  (Utilities|GetDataTableRow "/Game/GeneralSocial/Config/DataTableConfig/Schedule/CardAction/cardAction_DT.cardAction_DT" CardID
    (:then
      (Utilities|Map|Add (Variables|Default|GetActionCardInHand) CardID (Utilities|Struct|MakeCardInHand_Struct (Utilities|Struct|MakeActionCardInstance CardID Card%20Deadline Consequence) (+ (.amount (.Value (Utilities|Map|Find (Variables|Default|GetActionCardInHand) CardID))) Amount)))
      (return))))

(fn RemoveActionCardfromHand
  (params (CardID :type Name) (Amount :type Integer))
  (bind _actioncardinhand (Variables|Default|GetActionCardInHand))
  (bind _value (Utilities|Map|Find _actioncardinhand CardID))
  (LocalVariables|SetCard (.card _value))
  (LocalVariables|SetLastAmountValue (.amount _value))
  (LocalVariables|SetValueAfterSubtract (- (.amount _value) Amount))
  (if (<= (LocalVariables|GetValueAfterSubtract) 0)
    (Utilities|Map|Remove (Variables|Default|GetActionCardInHand) CardID)
    (LocalVariables|SetValue (Math|Integer|Absolute(Integer) (- (LocalVariables|GetLastAmountValue) Amount)))
    (else
      (Utilities|Map|Add (Variables|Default|GetActionCardInHand) CardID (Utilities|Struct|MakeCardInHand_Struct (LocalVariables|GetCard) (LocalVariables|GetValueAfterSubtract)))
      (LocalVariables|SetValue (LocalVariables|GetValueAfterSubtract))))
  (return (LocalVariables|GetValue)))

(fn RemoveActionCard
  (params (CardID :type Name) (Amount :type Integer))
  (bind _returnvalue (CallFunction|RemoveActionCardfromHand CardID Amount))
  (if (> _returnvalue 0)
    (CallFunction|FindandRemoveActionCardonSchedule CardID _returnvalue)))

(fn CheckMisstheDeadline
  (bind _calendarmanager (CallFunction|GetCalendarManager "__WorldContext"))
  (bind _alldayofthegame (Variables|Default|GetAllDayOfTheGame))
  (bind _previoustime (Default|GetPreviousTime _calendarmanager))
  (bind _value (Utilities|Map|Find _alldayofthegame _previoustime))
  (bind (_card _hascard) (Utilities|Struct|BreakSlotCardInfo _value))
  (bind (_cardid _deadline _consequence) (Utilities|Struct|BreakActionCardInstance _card))
  (bind _values (Utilities|Map|Values (Variables|Default|GetActionCardInHand)))
  (for _array_element _values
    (if (Utilities|Enum|Equal(Enum) (Utilities|Struct|BreakActionCardInfo_Struct (CallFunction|GetCardDatabyCardID (.CardID (Utilities|Struct|BreakActionCardInstance (.Card (Utilities|Struct|BreakCardInHand_Struct _array_element)))))) "NewEnumerator1")
      (if (Default|CheckDeadline (CallFunction|GetCalendarManager "__WorldContext") (.Deadline (Utilities|Struct|BreakActionCardInstance (.Card (Utilities|Struct|BreakCardInHand_Struct _array_element)))))
        ;[1 0 0] Consequence
        (Consequence|ActiveConsequence (.Consequence (Utilities|Struct|BreakActionCardInstance (.Card (Utilities|Struct|BreakCardInHand_Struct _array_element)))))
        (CallFunction|RemoveActionCardfromHand (.CardID (Utilities|Struct|BreakActionCardInstance (.Card (Utilities|Struct|BreakCardInHand_Struct _array_element)))) (.Amount (Utilities|Struct|BreakCardInHand_Struct _array_element))))))
  (if _hascard
    (if (Utilities|Enum|Equal(Enum) (Utilities|Struct|BreakActionCardInfo_Struct (CallFunction|GetCardDatabyCardID _cardid)) "NewEnumerator1")
      (if (Default|CheckDeadline (CallFunction|GetCalendarManager "__WorldContext") _deadline)
        (Development|PrintString "True")
        ;[1 0 0] Consequence
        (Consequence|ActiveConsequence _consequence)
        (CallFunction|RemoveActionCardfromTimeOftheGame _deadline)))))

(fn ActiveConsequence
  (params (Consequence :type Consequence%20Struct%20Structure))
  (bind (_addbuff _addstats) (Utilities|Struct|BreakConsequenceStruct Consequence))
  (Utilities|FlowControl|Sequence
    (:then_0
      (if (Utilities|Array|IsNotEmpty _addbuff)
        (for _array_element _addbuff
          (Default|AddBufftoActor (CallFunction|GetBuffManager) (.BuffID (Utilities|Struct|BreakAddBuffStruct _array_element)) (.Count (Utilities|Struct|BreakAddBuffStruct _array_element)) (Game|GetPlayerCharacter 0)))))
    (:then_1
      (if (Utilities|Array|IsNotEmpty _addstats)
        (for _array_element_2 _addstats
          (CallFunction|PlusPlayerStat (CallFunction|GetPlayerCharacterSocial) (.StatID (Utilities|Struct|BreakMCStatsStruct _array_element_2)) (.Amount (Utilities|Struct|BreakMCStatsStruct _array_element_2))))))))