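; One-shot quest trigger box that fires when the player character's root component overlaps it, and also carries a quest navigator widget.
; Overlap plays an async-loaded Level Sequence or, if none is set, starts a DataTable dialogue, then completes any valid objective; each action destroys the actor.
; The navigator shows when the player is on its map, otherwise forwards the map name to game-mode navigation, and hides on the quest manager's turn-off event.
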(event OnComponentBeginOverlap(Box)
  (params (OverlappedComponent :type Primitive%20Component%20Object%20Reference) (OtherActor :type Actor%20Object%20Reference) (OtherComp :type Primitive%20Component%20Object%20Reference) (OtherBodyIndex :type Integer) (bFromSweep :type Boolean) (SweepResult :type Hit%20Result%20Structure%20%28by%20ref%29))
  (bind _cutscene (Variables|Default|GetCutScene))
  (bind _dialogue (Variables|Default|GetDialogue))
  (if (== OtherComp (Variables|/Script/Engine.Actor|GetRootComponent (CallFunction|GetPlayerCharacterSocial)))
    (Utilities|FlowControl|Sequence
      (:then_0
        (if (Utilities|IsValidSoftObjectReference (.cutscene _cutscene))
          (bind _object (Utilities|AsyncLoadAsset (.cutscene _cutscene))
            (:Completed
              (bind _aslevel_sequence (Utilities|Casting|CastToLevelSequence _object))
              (bind _returnvalue (Sequencer|Player|CreateLevelSequencePlayer _aslevel_sequence (.settings _cutscene)))
              (Sequencer|Player|Play _returnvalue :!class /Script/MovieScene.MovieSceneSequencePlayer)
              (Actor|DestroyActor)))
          (else
            (Utilities|IsValid (.datatable _dialogue)
              (:Is%20Valid
                (CallFunction|StartDialogue (CallFunction|GetPlayerCharacterSocial) (.datatable _dialogue) (.rowname _dialogue))
                (Actor|DestroyActor))))))
      (:then_1
        (bind _objectivecomplete (Variables|Default|GetObjectiveComplete)
          (:then
            (Default|CallOnCompleteObjective _objectivecomplete)
            (Actor|DestroyActor))
          (:else))))))

(event Custom|TurnOffAllNavigator_Event
  (Rendering|SetVisibility (Variables|Default|GetQuestNavigatorWidget) false false))

(event EventBeginPlay
  (Rendering|SetVisibility (Variables|Default|GetQuestNavigatorWidget) false false)
  (EventDispatchers|AssignTurnOffAllNavigator (CallFunction|GetQuestManager) (delegate Custom|TurnOffAllNavigator_Event)))

(event EventTurnonNavigator
  (CallFunction|OpenMapFunction))

(fn ConstructionScript
  (EventDispatchers|BindEventtoOnOpenMap (.Thuy%20Tinh%20Social%20Game%20Mode (CallFunction|GetSocialGameMode)) (EventDispatchers|CreateEvent :!event OpenMapFunction)))

(fn BindObjectiveComplete
  (params (ObjectiveComplete :type %20Object%20Reference))
  (Variables|Default|SetObjectiveComplete 0 ObjectiveComplete))

(fn OpenMapFunction
  (if (== (Variables|Default|GetCurrentLocation (CallFunction|GetPlayerCharacterSocial)) (Variables|Default|GetCurrentMapName))
    (Rendering|SetVisibility (Variables|Default|GetQuestNavigatorWidget) true false)
    (else
      (Rendering|SetVisibility (Variables|Default|GetQuestNavigatorWidget) false false)
      (Default|CallTurnonNavigation (.Thuy%20Tinh%20Social%20Game%20Mode (CallFunction|GetSocialGameMode)) (Variables|Default|GetCurrentMapName)))))

(fn GetQuestNavigatorSocket
  (return (Variables|Default|GetQuestNavigatorWidget)))