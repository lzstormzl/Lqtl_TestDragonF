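; BP_BlockBox is a trigger box that turns the player back when they enter it, optionally explaining with dialogue.
; On overlap with the player character's root component, it starts the configured dialogue row if the data table is valid.
; It then uses SimpleMoveToLocation on the player controller to walk the player a short distance along the Arrow component's forward vector.
; BindObjectiveComplete is an empty stub.
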(event OnComponentBeginOverlap(Box)
  (params (OverlappedComponent :type Primitive%20Component%20Object%20Reference) (OtherActor :type Actor%20Object%20Reference) (OtherComp :type Primitive%20Component%20Object%20Reference) (OtherBodyIndex :type Integer) (bFromSweep :type Boolean) (SweepResult :type Hit%20Result%20Structure%20%28by%20ref%29))
  (bind _dialogue (Variables|Default|GetDialogue))
  (if (== OtherComp (Variables|/Script/Engine.Actor|GetRootComponent (Game|GetPlayerCharacter 0)))
    (Utilities|FlowControl|Sequence
      (:then_0
        (Utilities|IsValid (.datatable _dialogue)
          (:Is%20Valid
            (CallFunction|StartDialogue (CallFunction|GetPlayerCharacterSocial) (.datatable _dialogue) (.rowname _dialogue)))))
      (:then_1
        (AI|Navigation|SimpleMovetoLocation (Game|GetPlayerController 0) (+ (Transformation|GetActorLocation (Game|GetPlayerCharacter 0)) (* (Math|Vector|GetForwardVector (Variables|Default|GetArrow)) 2e+02)))))))

(fn ConstructionScript)

(fn BindObjectiveComplete
  (params (ObjectiveComplete :type %20Object%20Reference)))