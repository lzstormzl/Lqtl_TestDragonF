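; BP_Entity is an interactable social-world entity, such as an NPC, with dialogue and a quest navigator marker.
; Its sphere overlap adds or removes it from the player's interact widget, and its NPC logic starts the configured dialogue row.
; The navigator shows when the player shares its map; otherwise it notifies the game mode, so entities leading to that map can light up.
; A quest manager event hides the marker.
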(event OnComponentBeginOverlap(Sphere)
  (params (OverlappedComponent :type Primitive%20Component%20Object%20Reference) (OtherActor :type Actor%20Object%20Reference) (OtherComp :type Primitive%20Component%20Object%20Reference) (OtherBodyIndex :type Integer) (bFromSweep :type Boolean) (SweepResult :type Hit%20Result%20Structure%20%28by%20ref%29))
  (bind _thuy_tinh_social (CallFunction|GetPlayerCharacterSocial))
  (if (== OtherComp (Variables|/Script/Engine.Actor|GetRootComponent (Game|GetPlayerCharacter 0)))
    (bind _interactsequencewidget (Variables|Default|GetInteractSequenceWidget (CallFunction|GetPlayerCharacterSocial))
      (:then
        (Default|UpdateInteractWidget _interactsequencewidget self))
      (:else
        (bind _returnvalue (UserInterface|CreateWidget "/Game/GeneralSocial/2_GameSystems/3_InteractSystem/WBP_InteractSequence.WBP_InteractSequence_C"))
        (Variables|Default|SetInteractSequenceWidget _thuy_tinh_social _returnvalue)
        (Default|UpdateInteractWidget (Variables|Default|GetInteractSequenceWidget _thuy_tinh_social) self)))))

(event OnComponentEndOverlap(Sphere)
  (params (OverlappedComponent :type Primitive%20Component%20Object%20Reference) (OtherActor :type Actor%20Object%20Reference) (OtherComp :type Primitive%20Component%20Object%20Reference) (OtherBodyIndex :type Integer))
  (bind _returnvalue (Game|GetPlayerCharacter 0))
  (Utilities|IsValid _returnvalue
    (:Is%20Valid
      (if (== OtherComp (Variables|/Script/Engine.Actor|GetRootComponent _returnvalue))
        (Default|RemoveInteract (Variables|Default|GetInteractSequenceWidget (CallFunction|GetPlayerCharacterSocial)) self)))))

(event Custom|DoOwnLogicWithoutDialogue)

(event Custom|TurnOffAllNavigator_Event
  (Rendering|SetVisibility (Variables|Default|GetQuestNavigator) false false))

(event EventBeginPlay
  (Rendering|SetVisibility (Variables|Default|GetQuestNavigator) false false)
  (EventDispatchers|BindEventtoTurnonNavigation (.Thuy%20Tinh%20Social%20Game%20Mode (CallFunction|GetSocialGameMode)) (EventDispatchers|CreateEvent :!event TurnonQuestNavigation))
  (Utilities|FlowControl|Delay 0.2)
  (EventDispatchers|AssignTurnOffAllNavigator (CallFunction|GetQuestManager) (delegate Custom|TurnOffAllNavigator_Event)))

(event EventDoNPCOwnLogic
  (bind _dialogueid (Variables|Default|GetDialogueID))
  (bind (_datatable _rowname) (Utilities|Struct|BreakDataTableRowHandle _dialogueid))
  (Utilities|IsValid _datatable
    (:Is%20Valid
      (CallFunction|StartDialogue (CallFunction|GetPlayerCharacterSocial) _datatable _rowname))))

(event EventTurnonNavigator
  (if (== (Variables|Default|GetCurrentLocation (CallFunction|GetPlayerCharacterSocial)) (Variables|Default|GetCurrentMap))
    (Rendering|SetVisibility (Variables|Default|GetQuestNavigator) true false)
    (else
      (Rendering|SetVisibility (Variables|Default|GetQuestNavigator) false false)
      (Default|CallTurnonNavigation (.Thuy%20Tinh%20Social%20Game%20Mode (CallFunction|GetSocialGameMode)) (Variables|Default|GetCurrentMap)))))

(fn ConstructionScript)

(fn OpenNavigatorWidget
  (Rendering|SetVisibility (Variables|Default|GetQuestNavigator) true false))

(fn TurnonQuestNavigation
  (params (MapNavigation :type Name))
  (if (and (== (Variables|Default|GetCurrentMap) (Variables|Default|GetCurrentLocation (CallFunction|GetPlayerCharacterSocial))) (Utilities|Array|ContainsItem (Variables|Default|GetCanMoveToMap) MapNavigation))
    (CallFunction|OpenNavigatorWidget)
    (else
      (Rendering|SetVisibility (Variables|Default|GetQuestNavigator) false false))))

(fn GetName
  (return (Variables|Default|GetName)))

(fn GetQuestNavigatorSocket
  (return (Variables|Default|GetQuestNavigator)))