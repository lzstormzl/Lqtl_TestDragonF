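; BP_TieuQuy is a controllable companion character in the social mode that can prompt interactions with NPCs.
; While it is player-controlled, its InteractCheck overlaps add or remove NPC-tagged actors in an InteractSequence widget.
; That widget is created on demand and stored on the main social player character.
; Disconnected logic would move it behind that character, return possession and control state, and turn interaction off, but never runs.
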(event OnComponentBeginOverlap(InteractCheck)
  (params (OverlappedComponent :type Primitive%20Component%20Object%20Reference) (OtherActor :type Actor%20Object%20Reference) (OtherComp :type Primitive%20Component%20Object%20Reference) (OtherBodyIndex :type Integer) (bFromSweep :type Boolean) (SweepResult :type Hit%20Result%20Structure%20%28by%20ref%29))
  (bind _thuy_tinh_social (CallFunction|GetPlayerCharacterSocial))
  (if (and (Actor|ActorHasTag OtherActor "NPC") (Variables|Default|GetIsPlayerControlling?))
    (Variables|/Game/Characters/Main/Social/Main_Social_BP.Main_Social_BP_C|GetInteractSequenceWidget (CallFunction|GetPlayerCharacterSocial)
      (:then
        _)
      (:else
        (bind _returnvalue (UserInterface|CreateWidget "/Game/GeneralSocial/2_GameSystems/3_InteractSystem/WBP_InteractSequence.WBP_InteractSequence_C"))
        (Variables|/Game/Characters/Main/Social/Main_Social_BP.Main_Social_BP_C|SetInteractSequenceWidget _thuy_tinh_social _returnvalue)))
    (Default|UpdateInteractWidget (Variables|/Game/Characters/Main/Social/Main_Social_BP.Main_Social_BP_C|GetInteractSequenceWidget _thuy_tinh_social) OtherActor)))

(event OnComponentEndOverlap(InteractCheck)
  (params (OverlappedComponent :type Primitive%20Component%20Object%20Reference) (OtherActor :type Actor%20Object%20Reference) (OtherComp :type Primitive%20Component%20Object%20Reference) (OtherBodyIndex :type Integer))
  (if (and (Actor|ActorHasTag OtherActor "NPC") (Variables|Default|GetIsPlayerControlling?))
    (bind _interactsequencewidget (Variables|/Game/Characters/Main/Social/Main_Social_BP.Main_Social_BP_C|GetInteractSequenceWidget (CallFunction|GetPlayerCharacterSocial))
      (:then
        (Default|RemoveInteract _interactsequencewidget OtherActor))
      (:else))))

(event EventBeginPlay)

(event Input|KeyboardEvents|DebugKeyR
  (params (Key :type Key%20Structure) (ActionValue :type Input%20Action%20Value%20Structure)))

(fn ConstructionScript)