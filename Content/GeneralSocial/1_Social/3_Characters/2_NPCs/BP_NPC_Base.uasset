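; Base NPC for the social game that places itself by calendar and events and handles dialogue, bonding and a quest marker.
; Active event overrides take precedence; otherwise priority-sorted spawn table rows are filtered by phase, date and gameplay-tag flag.
; Without a match, it hides below the world.
; Dialogue starts from condition-checked triggers; calendar and map-open bindings exist but are unconnected.
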(event Custom|MoveToNewLocation
  (bind _npc_spawn_struct (Variables|Default|GetNPC_Spawn_Struct))
  (bind (_time _mapname _transform) (Utilities|Struct|Breaknpc_spawn_struct _npc_spawn_struct))
  (if (Utilities|Array|IsNotEmpty (Variables|Default|GetEvent))
    (bind (_returnvalue _location _transform_2) (CallFunction|CheckEventLocation))
    (if _returnvalue
      (Transformation|SetActorTransform _transform_2)
      (Variables|Default|SetCurrentLocation _location)
      (Rendering|SetActorHiddenInGame false)
      (else
        (Rendering|SetActorHiddenInGame true)
        (Transformation|SetActorLocationAndRotation "0.000000,0.000000,-1000.000000" "0, 0, 0")
        (Variables|Default|SetCurrentLocation "None")))
    (else
      (bind _returnarrayaftersort (CallFunction|GetSpawnInfoArrayAfterSortbyPriority (Variables|Default|GetSpawnSequence)))
      (bind _returnvalue_2 (CallFunction|CheckforLocation _returnarrayaftersort))
      (if _returnvalue_2
        (Rendering|SetActorHiddenInGame false)
        (Transformation|SetActorTransform _transform)
        (Variables|Default|SetCurrentLocation _mapname)
        (else
          (Rendering|SetActorHiddenInGame true)
          (Transformation|SetActorLocationAndRotation "0.000000,0.000000,-1000.000000" "0, 0, 0")
          (Variables|Default|SetCurrentLocation "None"))))))

(event EventDoNPCOwnLogic
  (bind _array_element (Utilities|Array|ForEachLoopwithBreak (Variables|Default|GetDialogueTriggerByCondition) :!label _label)
    (:LoopBody
      (if (CallFunction|CheckSocialCondition (.Conditions (Utilities|Struct|BreakDialogueTriggerByCondition _array_element)))
        (bind _returnvalue (Class|SocialComponent|StartDialogue (CallFunction|GetSocialComponent) (.DialogueClass (Utilities|Struct|BreakDialogueTriggerByCondition _array_element)) (.StartFromID (Utilities|Struct|BreakDialogueTriggerByCondition _array_element))))
        (if _returnvalue
          (goto _label Break))))))

(event EventTurnonNavigator
  (if (== (Variables|Default|GetCurrentLocation) (Variables|/Game/Characters/Main/Social/Main_Social_BP.Main_Social_BP_C|GetCurrentLocation (CallFunction|GetPlayerCharacterSocial)))
    (Rendering|SetVisibility (Variables|Default|GetQuestNavigatorWidget) true false)
    (else
      (Rendering|SetVisibility (Variables|Default|GetQuestNavigatorWidget) false false)
      (Default|CallTurnonNavigation (CallFunction|GetSocialGameMode) (Variables|Default|GetCurrentLocation)))))

(event EventBeginPlay
  (Utilities|FlowControl|Sequence))

(event Input|KeyboardEvents|DebugKeyR
  (params (Key :type Key%20Structure) (ActionValue :type Input%20Action%20Value%20Structure))
  (:Pressed
    (Pawn|Possess (Game|GetPlayerController 0) (CallFunction|GetPlayerCharacterSocial))))

(fn ConstructionScript)

(fn GetSpawnInfoArrayAfterSortbyPriority
  (params (Array :type Array%20of%20Names))
  (for _array_element Array
    (bind _returnvalue (Utilities|GetDataTableRow "/Game/GeneralSocial/Config/DataTableConfig/NPC/npc_spawn_DT.npc_spawn_DT" _array_element)
      (:then
        (Utilities|Map|Add (LocalVariables|GetIndex) _array_element (.Prioty (Utilities|Struct|Breaknpc_spawn_struct _returnvalue))))))
  (for _index (range 0 (- (Utilities|Array|Length Array) 1))
    (for _index_2 (range 0 (- (Utilities|Array|Length Array) 1))
      (if (> (.Value (Utilities|Map|Find (LocalVariables|GetIndex) (Utilities|Array|Get(acopy) Array _index_2))) (.Value (Utilities|Map|Find (LocalVariables|GetIndex) (Utilities|Array|Get(acopy) Array _index))))
        (LocalVariables|SetTempSort (Utilities|Array|Get(acopy) Array _index))
        (Utilities|Array|SetArrayElem Array _index (Utilities|Array|Get(acopy) Array _index_2))
        (Utilities|Array|SetArrayElem Array _index_2 (LocalVariables|GetTempSort)))))
  (return Array))

(fn CheckforLocation
  (params (Array :type Array%20of%20Names))
  (bind _array_element (Utilities|Array|ForEachLoopwithBreak Array)
    (:LoopBody
      (bind _returnvalue (Utilities|GetDataTableRow "/Game/GeneralSocial/DataTableConfig/NPC/npc_spawn_DT.npc_spawn_DT" _array_element)
        (:then
          (Variables|Default|SetNPC_Spawn_Struct _returnvalue)
          (if (Utilities|Array|IsNotEmpty (Utilities|Struct|Breaknpc_spawn_struct _returnvalue))
            (if (Utilities|Array|ContainsItem (Utilities|Struct|Breaknpc_spawn_struct _returnvalue) (Variables|/Game/GeneralSocial/2_GameSystems/1_CalendarSystem/BP_CalendarManager.BP_CalendarManager_C|GetCurrentPhaseType (CallFunction|GetCalendarManager self)))
              ;[0 0 0] Kiểm tra có nhập ngày trong tuần không? (Không nhập => thỏa hết các ngày trong tuần)
              (if (Utilities|Array|IsNotEmpty (Utilities|Struct|Breaknpc_spawn_struct (Variables|Default|GetNPC_Spawn_Struct)))
                ;[0 0 0] Kiểm tra đúng ngày trong tuần không?
                (if (Utilities|Array|ContainsItem (Utilities|Struct|Breaknpc_spawn_struct (Variables|Default|GetNPC_Spawn_Struct)) (Variables|/Game/GeneralSocial/2_GameSystems/1_CalendarSystem/BP_CalendarManager.BP_CalendarManager_C|GetDayOfTheWeek (CallFunction|GetCalendarManager self)))
                  ;[0 0 0] Kiểm tra data ngày có trống không
                  (if (Utilities|Array|IsNotEmpty (Utilities|Struct|Breaknpc_spawn_struct (Variables|Default|GetNPC_Spawn_Struct))) :!label _label
                    ;[0 0 0] Check ngày
                    (if (Utilities|Array|ContainsItem (Utilities|Struct|Breaknpc_spawn_struct (Variables|Default|GetNPC_Spawn_Struct)) (Variables|/Game/GeneralSocial/2_GameSystems/1_CalendarSystem/BP_CalendarManager.BP_CalendarManager_C|GetDayOfTheMonth (CallFunction|GetCalendarManager self)))
                      ;[0 0 0] Kiểm tra data tháng có trống không
                      (if (Utilities|Array|IsNotEmpty (Utilities|Struct|Breaknpc_spawn_struct (Variables|Default|GetNPC_Spawn_Struct))) :!label _label_2
                        ;[0 0 0] Check Tháng
                        (if (Utilities|Array|ContainsItem (Utilities|Struct|Breaknpc_spawn_struct (Variables|Default|GetNPC_Spawn_Struct)) (Variables|/Game/GeneralSocial/2_GameSystems/1_CalendarSystem/BP_CalendarManager.BP_CalendarManager_C|GetMonth (CallFunction|GetCalendarManager self)))
                          ;[0 0 0] Kiểm tra có nhập flag không
                          (if (GameplayTags|IsGameplayTagValid (.FlagCondition (Utilities|Struct|Breaknpc_spawn_struct (Variables|Default|GetNPC_Spawn_Struct)))) :!label _label_3
                            ;[0 0 0] Kiểm tra flag có đúng không
                            (if (GameplayTags|HasTag (Variables|/Game/GeneralSocial/ThuyTinh_GameInstance.ThuyTinh_GameInstance_C|GetGameplayTagInstance (CallFunction|GetGameInstance)) (.FlagCondition (Utilities|Struct|Breaknpc_spawn_struct (Variables|Default|GetNPC_Spawn_Struct))) true)
                              (return true))
                            (else
                              (return true))))
                        (else
                          (goto _label_3))))
                    (else
                      (goto _label_2))))
                (else
                  (goto _label))))))))
    (:Completed
      (return false))))

(fn CheckEventLocation
  (for _array_element (Variables|Default|GetEvent)
    (bind _returnvalue (Utilities|GetDataTableRow "/Game/GeneralSocial/DataTableConfig/EventInGame/eventInGame_DT.eventInGame_DT" _array_element)
      (:then
        (if (== (.NPCLocationLoopPhase (Utilities|Struct|Breakevent_setupInfo_struct (.EventSetup (Utilities|Struct|Breakevent_config_struct _returnvalue)))) "-1")
          (for _array_element_2 (.AdjustNPCLocation (Utilities|Struct|Breakevent_setupInfo_struct (.EventSetup (Utilities|Struct|Breakevent_config_struct _returnvalue)))) :!label _label
            (if (== (.NpcName (Utilities|Struct|Breakaddnpc_struct _array_element_2)) (Variables|Default|GetNPCID))
              (return true (.Location (Utilities|Struct|Breakaddnpc_struct _array_element_2)) (.Transform (Utilities|Struct|Breakaddnpc_struct _array_element_2)))))
          (elif (== (Variables|/Game/GeneralSocial/2_GameSystems/1_CalendarSystem/BP_CalendarManager.BP_CalendarManager_C|GetCurrentPhaseType (CallFunction|GetCalendarManager self)) (.NPCLocationLoopPhase (Utilities|Struct|Breakevent_setupInfo_struct (.EventSetup (Utilities|Struct|Breakevent_config_struct _returnvalue)))))
            (goto _label))))))
  (return false "None" ""))

(fn IncreaseBonding
  (params (Experience :type Integer))
  (Variables|Stats|SetBondingLevel (Utilities|Struct|MakeF_BondingInstance (.Level (Utilities|Struct|BreakF_BondingInstance (Variables|Stats|GetBondingLevel))) (+ (.Experience (Utilities|Struct|BreakF_BondingInstance (Variables|Stats|GetBondingLevel))) Experience))))

(fn FindDialogueforStart
  (bind _keys (Utilities|Map|Keys (Variables|Default|GetDialogueStarts)))
  (bind _output_get (LocalVariables|SetSortingPriotyArray _keys))
  (Class|KismetArrayLibrary|SortIntArray _output_get false "Descending")
  (for _array_element (LocalVariables|GetSortingPriotyArray)
    (if true
      (return (.DialogueID (Utilities|Struct|BreakS_OwnNPCDialogueStart (.Value (Utilities|Map|Find (Variables|Default|GetDialogueStarts) _array_element)))) true)))
  (return "" false))

(fn GetName
  (return (Variables|Default|GetNPCName)))

(fn GetQuestNavigatorSocket
  (return (Variables|Default|GetQuestNavigatorWidget)))