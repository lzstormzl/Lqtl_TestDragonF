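; Afterimage actor for the MazeLong character that mirrors source meshes, then fades out and destroys itself.
; For its first half second, Tick copies poses onto its Base, Hair and Vay meshes from the matching source components.
; Each valid Base copy restarts the Fade timeline, which drives an opacity parameter in the shared MPC_MazeLongFX collection and destroys the actor on finish.
; Glow, light and Niagara spawn nodes are unconnected.
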(event EventTick
  (params (DeltaSeconds :type Float%20%28single-precision%29))
  (Variables|Default|SetCopyTime (+ (Variables|Default|GetCopyTime) (Utilities|Time|GetWorldDeltaSeconds)))
  (if (< (Variables|Default|GetCopyTime) (Variables|Default|GetMaxCopyTime))
    (Utilities|FlowControl|Sequence
      (:then_0
        (bind _basetocopy (Variables|Default|GetBaseToCopy)
          (:then
            (Class|PoseableMeshComponent|CopyPosefromSkeletalComponent (Variables|Default|GetBase) _basetocopy)
            (Utilities|FlowControl|Sequence
              (:then_1
                (bind _opacity (Timeline|Fade PlayFromStart)
                  (:Update
                    (Rendering|Material|SetScalarParameterValue "/Game/Characters/Main/Maze/Fx/MPC_MazeLongFX.MPC_MazeLongFX" "ThuyAnh_Opacity" _opacity :!class /Script/Engine.KismetMaterialLibrary))
                  (:Finished
                    (Actor|DestroyActor))))))
          (:else)))
      (:then_1
        (bind _hair_to_copy (Variables|Default|GetHair%20to%20Copy)
          (:then
            (Class|PoseableMeshComponent|CopyPosefromSkeletalComponent (Variables|Default|GetHair) _hair_to_copy))
          (:else)))
      (:then_2
        (bind _vay_to_copy (Variables|Default|GetVay%20to%20Copy)
          (:then
            (Class|PoseableMeshComponent|CopyPosefromSkeletalComponent (Variables|Default|GetVay) _vay_to_copy))
          (:else))))))

(event EventBeginPlay
  (Utilities|FlowControl|Sequence
    (:then_0
      (Variables|Default|SetMaxCopyTime 0.5))
    (:then_1
      (Variables|Default|SetCopyTime 0.0))))

(fn ConstructionScript)