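; Base character for player-summoned legion allies, pooled, hidden until summoned and returned to the pool on death.
; While summoned, it steadily loses health, periodically has its AI controller find enemies, and passes stagger reactions to it.
; Data tables supply stats, combos and montages to combat, attack and hitbox components.
; Assault plays a dive montage, then teleports into a ring around the player's lock-on target and attacks, or returns to the player.
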(event OnAttackHit(BPC_HitboxHandler)
  (params (Hit%20Actor :type Actor%20Object%20Reference) (Attack%20Data :type S%20Attack%20Data%20Structure) (Hit%20Count :type Integer) (In%20Hit%20Direction :type Vector :default "0, 0, 0"))
  ;[0.05313 0.05313 0.05313] Initialize
  (Class|BPIDamagable|OnDamaged(Message) Hit%20Actor Attack%20Data self In%20Hit%20Direction))

(event OnAttackInitiated(BPC_AttackActionHandler)
  (params (Attack%20Data :type S%20Attack%20Action%20Data%20Structure))
  ;[0.05313 0.05313 0.05313] Initialize
  (Default|ResetOverlapIDTrack (Variables|Default|GetBPC_HitboxHandler)))

(event Custom|Assault
  (bind _move_set (Data|GetMoveSetData))
  (bind _out_character (CallFunction|GetPlayerCombatCharacter))
  (bind _bpc_attackactionhandler (Variables|Default|GetBPC_AttackActionHandler))
  (bind _combosname (Utilities|Struct|BreakS_MoveSetData _move_set))
  (bind _advanced_camera_handler (Variables|/Game/GeneralCombat/Blueprints/Pawns/BP_DefaultCombatCharacter.BP_DefaultCombatCharacter_C|GetAdvanced%20Camera%20Handler _out_character))
  (bind _actor (Default|GetLockonActor _advanced_camera_handler))
  ;[1 1 1] anim nhìn bị k mượt
  (Default|CancelCombo _bpc_attackactionhandler)
  (Default|CancelCurrentAttackMontage _bpc_attackactionhandler 0.0)
  (CallFunction|IgnoreEnemy true)
  (bind _notifyname (Animation|Montage|PlayMontage (Variables|Character|GetMesh) (.Montage%20Dive (Data|GetLegionInfoData)))
    (:OnNotifyBegin
      (switch name _notifyname
        (:End%20Dive
          (Utilities|IsValid _actor
            (:Is%20Valid
              (CallFunction|TeleportAssault _actor (.Assault%20Radius (Data|GetLegionInfoData)))
              (bind _returnvalue (Utilities|GetDataTableRow "/Game/Developers/Admin/Data/DataTables/GeneralCombat/DT_AttackComboData.DT_AttackComboData" (Utilities|Array|Get(acopy) _combosname (- (Utilities|Array|Length _combosname) 1)))
                (:then
                  (CallFunction|Attack _actor _returnvalue))))
            (:Is%20Not%20Valid
              (CallFunction|TeleportAssault (.Out%20Character (CallFunction|GetPlayerCombatCharacter)) 0.0)
              (Animation|Montage|PlayMontage (Variables|Character|GetMesh) (.Montage%20Spawn (Data|GetLegionInfoData))))))))))

(event Custom|On%20Hit%20React%20Started_Event
  (params (Hit%20React%20Type :type E_HitReactType%20Enum :default "NewEnumerator3") (Knockback%20Direction :type Vector))
  ;[1 1 1] Sttager
  (if (or (Utilities|Enum|Equal(Enum) Hit%20React%20Type "NewEnumerator1") (Utilities|Enum|Equal(Enum) Hit%20React%20Type "NewEnumerator2"))
    (Default|SetStateStagger(Interrupt+) (Variables|AI|GetAs%20AIC%20ThuyTuong) true)
    (Development|PrintString (Utilities|String|EnumtoString Hit%20React%20Type) true true "(R=1.000000,G=0.000000,B=0.026414,A=1.000000)" 5.0)))

(event Custom|On%20Hit%20React%20Ended_Event
  ;[1 1 1] Sttager
  (Default|SetStateStagger(Interrupt+) (Variables|AI|GetAs%20AIC%20ThuyTuong) false)
  (Development|PrintString "End Stagger Legion" true true "(R=0.000000,G=0.660000,B=1.000000,A=1.000000)" 5.0))

(event Custom|Set%20is%20Summoning
  (params (is%20summonning :type Boolean))
  (bind _returnvalue (not is%20summonning))
  (bind _bpc_combatunit (Variables|Default|GetBPC_CombatUnit))
  ;[1 0.02851 0.8191] summoning
  (Variables|Default|SetIs%20summonning is%20summonning)
  (Collision|SetActorEnableCollision is%20summonning)
  (Rendering|SetActorHiddenInGame _returnvalue)
  (Actor|Tick|SetActorTickEnabled is%20summonning)
  (Variables|/Game/GeneralCombat/Blueprints/Components/BPC_CombatUnit.BPC_CombatUnit_C|SetIsDead (Variables|Default|GetBPC_CombatUnit) _returnvalue)
  (if is%20summonning
    (Default|SetCurrentStat (Variables|Default|GetBPC_CombatUnit) (Utilities|Struct|BreakS_CharacterCombatData (Data|GetCharacterCombatData)))
    (Utilities|Time|SetTimerbyEvent (delegate Custom|Decrease%20health%20overtime) 1.0 true false 1.0)
    (Animation|Montage|PlayMontage (Variables|Character|GetMesh) (.Montage%20Spawn (Data|GetLegionInfoData))
      (:OnCompleted
        _)
      (:OnInterrupted
        _))
    (Utilities|Time|SetTimerbyEvent (delegate Custom|Legion%20Perception) 1.0 true)
    ;[1 1 1] Sttager
    (EventDispatchers|AssignOnHitReactStarted _bpc_combatunit (delegate Custom|On%20Hit%20React%20Started_Event))
    (EventDispatchers|AssignOnHitReactEnded _bpc_combatunit (delegate Custom|On%20Hit%20React%20Ended_Event))
    (else
      ;;[1 1 1] service deactivate
      (Default|ResetKeyBlackboard (Variables|AI|GetAs%20AIC%20ThuyTuong))
      (EventDispatchers|UnbindEventfromOnHitReactStarted _bpc_combatunit (delegate Custom|On%20Hit%20React%20Started_Event))
      (EventDispatchers|UnbindEventfromOnHitReactEnded _bpc_combatunit (delegate Custom|On%20Hit%20React%20Ended_Event)))))

(event Custom|Legion%20Perception
  (Utilities|IsValid (Default|GetLockonActor (Variables|/Game/GeneralCombat/Blueprints/Pawns/BP_DefaultCombatCharacter.BP_DefaultCombatCharacter_C|GetAdvanced%20Camera%20Handler (.Out%20Character (CallFunction|GetPlayerCombatCharacter))))
    (:Is%20Valid
      (Utilities|IsValid (AI|Components|Blackboard|GetValueasObject (Variables|/Script/AIModule.AIController|GetBlackboard (Variables|AI|GetAs%20AIC%20ThuyTuong)) (Variables|AI|GetFocus%20Target%20Key%20Name))
        (:Is%20Not%20Valid
          _)))
    (:Is%20Not%20Valid
      _))
  (Default|FindNearestEnemy (Variables|AI|GetAs%20AIC%20ThuyTuong)))

(event Custom|Decrease%20health%20overtime
  (bind _bpc_combatunit (Variables|Default|GetBPC_CombatUnit))
  ;[1 0.02851 0.8191] summoning
  ;;[1 1 1] giam 2% hp moi giay
  (Default|AddCurrentStat _bpc_combatunit (Utilities|Struct|MakeS_CombatResource 0.0 (* (/ (Utilities|Struct|BreakS_CombatResource (Default|GetMaxStat _bpc_combatunit)) 1e+02) -2.0) 0.0 0.0 0.0) self))

(event Custom|Ignore%20Enemy
  (params (Should%20Ignore :type Boolean))
  (bind _capsulecomponent (Variables|Collision|GetCapsuleComponent))
  (if Should%20Ignore
    (Collision|SetCollisionResponsetoChannel _capsulecomponent "ECC_GameTraceChannel2" "ECR_Overlap")
    (else
      (Collision|SetCollisionResponsetoChannel _capsulecomponent "ECC_GameTraceChannel2" "ECR_Overlap"))))

(event EventReturnAttackTokenRange
  (params (Amount%20Range :type Integer))
  ;[0.3941 0.8491 1] Combat Ticket
  (Default|ReturnAttackTokenRange (Variables|Default|GetBPC_DamageSystem) Amount%20Range))

(event EventBeginPlay
  ;[0.05313 0.05313 0.05313] Initialize
  (bind _asaic_legions (Utilities|Casting|CastToAIC_Legions (AI|GetAIController self))
    (:then
      (Variables|AI|SetAs%20AIC%20ThuyTuong _asaic_legions)
      (CallFunction|InitializeWorldWidget)
      (UserInterface|SetWidget (Variables|Default|GetWidget_HealthBar) (Variables|Asset|GetHealth%20Bar%20Widget))
      (CallFunction|InitializeStat)
      (Default|InitializeComponent (Variables|Default|GetBPC_AttackActionHandler) (Variables|Character|GetMesh))
      (Default|InitializeAction (Variables|AI|GetAs%20AIC%20ThuyTuong) (Variables|Default|GetPlayer%20Actor))
      (Class|BlackboardComponent|SetValueasInt (Variables|/Script/AIModule.AIController|GetBlackboard (Variables|AI|GetAs%20AIC%20ThuyTuong)) (Variables|AI|GetSummon%20Index%20Key%20Name) (Variables|Default|GetLegion%20Index))
      (CallFunction|SetIsSummoning false)
      (Variables|Default|SetListCombo (Data|GetListComboData))
      ;[1 0.2649 0.1991] event binding
      (EventDispatchers|BindEventtoOnDeath (Variables|Default|GetBPC_CombatUnit) (EventDispatchers|CreateEvent :!event Custom|Event%20On%20Death)))
    (:CastFailed
      (Development|PrintString "fail cast to aic"))))

(event EventReturnAttackTokenMelee
  (params (Amount%20Melee :type Integer))
  ;[0.3941 0.8491 1] Combat Ticket
  (Default|ReturnAttackTokenMelee (Variables|Default|GetBPC_DamageSystem) Amount%20Melee))

(event EventLegionSpawn
  (CallFunction|IgnoreEnemy false)
  (Default|CallOnLegionSpawn))

(event EventAttack
  (params (Attack%20Target :type Actor%20Object%20Reference) (Combo%20Choosen :type S%20Attack%20Combo%20Data%20Structure))
  ;[0.7406 0.3597 0] Event Attack
  (Default|SetCurrentAttackCombo (Variables|Default|GetBPC_AttackActionHandler) Combo%20Choosen)
  (Default|TryRegisterAttack (Variables|Default|GetBPC_AttackActionHandler) true))

(event EventGetInfoMotionWarp
  (params (Montion%20Warp%20Data :type S%20Motion%20Warp%20Data%20Structure))
  (Variables|/Game/GeneralCombat/Blueprints/Components/BPC_AttackActionHandler.BPC_AttackActionHandler_C|SetS%20Motion%20Warp%20Data (Variables|Default|GetBPC_AttackActionHandler) Montion%20Warp%20Data))

(event EventOnDamaged
  (params (Source%20Attack :type S%20Attack%20Data%20Structure) (Initigator :type Actor%20Object%20Reference) (Hit%20Direction :type Vector :default "0, 0, 0"))
  (bind _bpc_combatunit (Variables|Default|GetBPC_CombatUnit))
  (bind _teamnumber (Class|BPIDamageSystem|GetTeamNumber(Message) Initigator))
  (if (not (== _teamnumber 1))
    (Default|ApplyDamage _bpc_combatunit Source%20Attack Initigator Hit%20Direction)
    (Development|PrintString (Utilities|String|ToString(Float) (.health (Default|GetCurrentStat _bpc_combatunit))))))

(event OnStatUpdated(BPC_CombatUnit)
  (params (New%20Data :type S%20Combat%20Resource%20Structure) (Delta%20Data :type S%20Combat%20Resource%20Structure) (Initigator :type Actor%20Object%20Reference))
  (if (!= Initigator self)
    (Callbacks|OnCombatInitiated)))

(event Custom|Event%20On%20Death
  (params (Initigator :type Actor%20Object%20Reference))
  (bind _player_actor (Variables|Default|GetPlayer%20Actor))
  (Components|Movement|StopMovementImmediately (Variables|Character|GetCharacterMovement))
  (Animation|StopAnimMontage (Animation|GetCurrentMontage :!class /Script/Engine.Character))
  (Collision|SetCollisionEnabled (Variables|Character|GetMesh) "NoCollision")
  (Utilities|Array|RemoveItem (Variables|/Game/Characters/Main/Maze/BP_DefaultCombatCharacter_Child.BP_DefaultCombatCharacter_Child_C|GetThuy%20tuong%20summoning _player_actor) self)
  (Default|ReturnLegion (Variables|/Game/Characters/Main/Maze/BP_DefaultCombatCharacter_Child.BP_DefaultCombatCharacter_Child_C|GetThuytuong_pool _player_actor) self))

(fn ConstructionScript
  (Variables|Default|SetTeam%20Number 1))

(fn GetLegionData
  (bind _legiondata (Variables|Data|GetLegionData))
  (bind _returnvalue (Utilities|GetDataTableRow (.datatable _legiondata) (.rowname _legiondata))
    (:then
      (return _returnvalue))
    (:RowNotFound
      (Development|PrintString "not found row"))))

(fn GetMoveSetData
  (bind _returnvalue (Utilities|GetDataTableRow "/Game/Developers/Admin/Data/DataTables/GeneralCombat/DT_MoveSets.DT_MoveSets" (.MoveSetName (Utilities|Struct|BreakS_AIUnitData (Data|GetLegionData))))
    (:then
      (return _returnvalue))))

(fn GetListComboData
  (bind _list_combo (Variables|Data|GetList%20Combo))
  (Utilities|Array|Clear _list_combo)
  (for (_array_element _array_index) (.CombosName (Utilities|Struct|BreakS_MoveSetData (Data|GetMoveSetData)))
    (bind _returnvalue (Utilities|GetDataTableRow "/Game/Developers/Admin/Data/DataTables/GeneralCombat/DT_AttackComboData.DT_AttackComboData" _array_element)
      (:then
        ;[1 1 1] list combo k dung assault
        (if (!= _array_index (Utilities|Array|Length (.aievaluation (Data|GetMoveSetData))))
          (Utilities|Array|AddUnique _list_combo _returnvalue)))))
  (return (Variables|Data|GetList%20Combo)))

(fn GetListAttackActionData
  (params (Combo%20Data :type S%20Attack%20Combo%20Data%20Structure))
  (Utilities|Array|Clear (LocalVariables|GetList%20Attack%20))
  (for _array_element (.AttacksName (Utilities|Struct|BreakS_AttackComboData Combo%20Data))
    (bind _returnvalue (Utilities|GetDataTableRow (.datatable _array_element) (.rowname _array_element))
      (:then
        (Utilities|Array|AddUnique (LocalVariables|GetList%20Attack%20) _returnvalue))))
  (return (LocalVariables|GetList%20Attack%20)))

(fn GetCharacterCombatData
  (bind _bpc_combatunit (Variables|Default|GetBPC_CombatUnit))
  (bind _default_character_combat_data (Variables|/Game/GeneralCombat/Blueprints/Components/BPC_CombatUnit.BPC_CombatUnit_C|GetDefault%20Character%20Combat%20Data _bpc_combatunit))
  (bind _returnvalue (Utilities|GetDataTableRow (.datatable _default_character_combat_data) (.rowname _default_character_combat_data))
    (:then
      (return _returnvalue))))

(fn OnStatUpdated
  (params (Stat :type S%20Combat%20Resource%20Structure%20%28by%20ref%29) (Initigator :type Actor%20Object%20Reference)))

(fn TeleportAssault
  (params (Actor%20LockOn :type Actor%20Object%20Reference) (Assault%20Radius :type Float%20%28double-precision%29))
  (bind _player_actor (Variables|Default|GetPlayer%20Actor))
  (bind _player_actor_2 (Variables|Default|GetPlayer%20Actor))
  (bind _returnvalue (Transformation|GetActorLocation Actor%20LockOn))
  (bind _thuy_tuong_summoning (Variables|/Game/Characters/Main/Maze/BP_DefaultCombatCharacter_Child.BP_DefaultCombatCharacter_Child_C|GetThuy%20tuong%20summoning _player_actor))
  (for (_ _array_index) _thuy_tuong_summoning
    (if (!= Actor%20LockOn (Game|GetPlayerCharacter 0))
      (Collision|IgnoreActorwhenMoving (Variables|Collision|GetCapsuleComponent) (Variables|/Game/GeneralCombat/AI/Legions/AIC_controller/AIC_Legions.AIC_Legions_C|GetAttack%20Target (Variables|AI|GetAs%20AIC%20ThuyTuong)) true)
      (Transformation|SetActorLocation 0 (+ (Math|Vector|MakeVector (* (Math|Trig|Cos(Radians) (Math|Trig|DegreesToRadians (Math|Conversions|ToFloat(Integer) (* (/ 360 (Utilities|Array|Length _thuy_tuong_summoning)) _array_index)))) Assault%20Radius) (* (Math|Trig|Sin(Radians) (Math|Trig|DegreesToRadians (Math|Conversions|ToFloat(Integer) (* (/ 360 (Utilities|Array|Length _thuy_tuong_summoning)) _array_index)))) Assault%20Radius) -2e+01) _returnvalue) false true)
      (Transformation|SetActorRotation 0 (Math|Rotator|FindLookatRotation (+ (Math|Vector|MakeVector (* (Math|Trig|Cos(Radians) (Math|Trig|DegreesToRadians (Math|Conversions|ToFloat(Integer) (* (/ 360 (Utilities|Array|Length _thuy_tuong_summoning)) _array_index)))) Assault%20Radius) (* (Math|Trig|Sin(Radians) (Math|Trig|DegreesToRadians (Math|Conversions|ToFloat(Integer) (* (/ 360 (Utilities|Array|Length _thuy_tuong_summoning)) _array_index)))) Assault%20Radius) -2e+01) _returnvalue) _returnvalue))
      (Rendering|Debug|DrawDebugSphere (+ (Math|Vector|MakeVector (* (Math|Trig|Cos(Radians) (Math|Trig|DegreesToRadians (Math|Conversions|ToFloat(Integer) (* (/ 360 (Utilities|Array|Length _thuy_tuong_summoning)) _array_index)))) Assault%20Radius) (* (Math|Trig|Sin(Radians) (Math|Trig|DegreesToRadians (Math|Conversions|ToFloat(Integer) (* (/ 360 (Utilities|Array|Length _thuy_tuong_summoning)) _array_index)))) Assault%20Radius) -2e+01) _returnvalue) 1e+02 12 "(R=1.000000,G=0.000000,B=0.008551,A=1.000000)" 1e+01)
      (else
        (Default|TeleportSummon _player_actor_2 (- (Utilities|Array|Length (Variables|/Game/Characters/Main/Maze/BP_DefaultCombatCharacter_Child.BP_DefaultCombatCharacter_Child_C|GetThuy%20tuong%20summoning _player_actor_2)) 1))))))

(fn OnCombatInitiated)

(fn InitializeWorldWidget
  (bind _returnvalue (UserInterface|CreateWidget "/Game/GeneralCombat/Blueprints/Widgets/Combat/HealthBar/WB_NormalEnemyHealthBar.WB_NormalEnemyHealthBar_C"))
  (bind _output_get (Variables|Asset|SetHealth%20Bar%20Widget _returnvalue))
  (Default|Initialize _output_get (Variables|Default|GetBPC_CombatUnit) (Data|GetCharacterCombatData))
  (Widget|SetRenderOpacity (Variables|Asset|GetHealth%20Bar%20Widget) 0.0)
  (UserInterface|SetWidget (Variables|Default|GetWidget_HealthBar) (Variables|Asset|GetHealth%20Bar%20Widget))
  (Transformation|SetWorldRotation (Variables|Default|GetWidget_HealthBar) "0.000000,90.000000,0.000000" false false)
  (Transformation|AttachComponentToComponent (Variables|Default|GetWidget_HealthBar) (Variables|Character|GetMesh) "Head" "SnapToTarget" "KeepWorld" "KeepWorld" true))

(fn GetLegionInfoData
  (bind _out_character (CallFunction|GetPlayerCombatCharacter))
  (bind _equipment_handler (Variables|/Game/GeneralCombat/Blueprints/Pawns/BP_DefaultCombatCharacter.BP_DefaultCombatCharacter_C|GetEquipment%20Handler _out_character))
  (if (.Result (Default|GetEquippedEquipment _equipment_handler))
    (switch int (Default|GetEquippedIndex _equipment_handler)
      (:0
        (bind _returnvalue (Utilities|GetDataTableRow "/Game/Developers/Admin/Data/DataTables/AIUnit/DT_LegionInfoData.DT_LegionInfoData" "SpearFish")
          (:then
            (return (.SpawnMontage (Utilities|Struct|BreakS_LegionData _returnvalue)) (.DiveMontage (Utilities|Struct|BreakS_LegionData _returnvalue)) (.AssaultMontage (Utilities|Struct|BreakS_LegionData _returnvalue)) (.AssaultRadius (Utilities|Struct|BreakS_LegionData _returnvalue)) (.Maxnumberofsummons (Utilities|Struct|BreakS_LegionData _returnvalue))))))
      (:1
        (bind _returnvalue_2 (Utilities|GetDataTableRow "/Game/Developers/Admin/Data/DataTables/AIUnit/DT_LegionInfoData.DT_LegionInfoData" "Shark")
          (:then
            (return (.SpawnMontage (Utilities|Struct|BreakS_LegionData _returnvalue_2)) (.DiveMontage (Utilities|Struct|BreakS_LegionData _returnvalue_2)) (.AssaultMontage (Utilities|Struct|BreakS_LegionData _returnvalue_2)) (.AssaultRadius (Utilities|Struct|BreakS_LegionData _returnvalue_2)) (.Maxnumberofsummons (Utilities|Struct|BreakS_LegionData _returnvalue_2)))))))
    (else
      (Development|PrintString "Đang không Equipment hoặc không có Summons !!!"))))

(fn InitializeStat
  (bind _combat_data (Data|GetCharacterCombatData))
  (Default|SetCharacterCombatData (Variables|Default|GetBPC_CombatUnit) _combat_data self)
  (Default|SetCurrentStat (Variables|Default|GetBPC_CombatUnit) (.MaxStats (Utilities|Struct|BreakS_CharacterCombatData _combat_data)) self))

(fn AttackStart
  (params (AttackTarget :type Actor%20Object%20Reference) (TokenNeededMelee :type Integer) (TokenNeededRange :type Integer))
  (return false))

(fn DestroyHitbox
  (params (Hitbox%20Data :type S%20Hitbox%20Data%20Structure))
  (Default|DestroyHitbox (Variables|Default|GetBPC_HitboxHandler) Hitbox%20Data)
  (return true))

(fn GenerateHitbox
  (params (Hitbox%20Data :type S%20Hitbox%20Data%20Structure))
  (bind _hitbox_generated (Default|GenerateHitbox (Variables|Default|GetBPC_HitboxHandler) Hitbox%20Data))
  (return _hitbox_generated))

(fn GetAttackTarget
  (return 0))

(fn GetRangeDefend(StrafeRadius)
  (return 0.0))

(fn GetEnemyRef
  (return 0))

(fn GetPatrolRoute
  (return 0))

(fn GetTeamNumber
  (return (Variables|Default|GetTeam%20Number)))

(fn ReserveAttackTokenMelee
  (params (Amount%20Melee :type Integer))
  (bind _success (Default|ReserveAttackTokenMelee (Variables|Default|GetBPC_DamageSystem) Amount%20Melee))
  (return _success))

(fn ReserveAttackTokenRange
  (params (Amount%20Range :type Integer))
  (bind _success (Default|ReserveAttackTokenRange (Variables|Default|GetBPC_DamageSystem) Amount%20Range))
  (return _success))

(fn SetMovementSpeed
  (params (Speed :type E_AI_Movement_State%20Enum :default "NewEnumerator0"))
  (bind _output_get (Variables|/Script/Engine.CharacterMovementComponent|SetMaxWalkSpeed (Variables|Character|GetCharacterMovement) (Utilities|Select :Index Speed :NewEnumerator0 0.0 :NewEnumerator1 4e+02 :NewEnumerator2 4e+02 :NewEnumerator3 7e+02 :NewEnumerator4 4e+02 :NewEnumerator5 0.0)))
  (return _output_get))