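; Tiger enemy character blueprint that handles death, spirit-break recovery and movement tuning for combat AI.
; The combat unit component's death event flags the AI controller as dead, disables mesh collision, plays a death montage and destroys the actor.
; When a spirit break ends, it refills depleted spirit orbs and clears the stagger-interrupt state after a short delay.
; Functions supply a fixed strafe radius and map AI speed states to walk speeds; the spirit-break hit montage chain is disconnected.
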(event EventBeginPlay
  (Utilities|FlowControl|DelayUntilNextTick)
  (Utilities|FlowControl|Delay 0 0.5)
  ;[1 0.2491 0.1635] Event binding
  (EventDispatchers|BindEventtoOnDeath (Variables|Default|GetBPC_CombatUnit) (EventDispatchers|CreateEvent :!event Custom|Event%20On%20Death)))

(event Custom|Event%20On%20Death
  (params (Initigator :type Actor%20Object%20Reference))
  (bind _as_aic_enermy (Variables|Default|GetAs%20AIC%20Enermy))
  (Utilities|IsValid _as_aic_enermy
    (:Is%20Valid
      (Default|SetStateDeath _as_aic_enermy true)
      (Animation|StopAnimMontage (Animation|GetCurrentMontage :!class /Script/Engine.Character))
      (Collision|SetCollisionEnabled (Variables|Character|GetMesh) "NoCollision")
      (Utilities|FlowControl|Delay 0 0.5)
      (Animation|Montage|PlayMontage (Variables|Character|GetMesh) (.DeathMontage (Utilities|Struct|BreakS_CharacterCombatData))
        (:OnCompleted
          _)
        (:OnBlendOut
          _))
      (Rendering|SetActorHiddenInGame true)
      (Actor|DestroyActor))
    (:Is%20Not%20Valid
      (Development|PrintString 0 "Death _ not valid aic"))))

(event OnSpiritBreakEnded(BPC_CombatUnit)
  (if (<= (Utilities|Struct|BreakS_CombatResource (Default|GetCurrentStat (Variables|Default|GetBPC_CombatUnit))) 0.0)
    (Default|AddCurrentStat (Variables|Default|GetBPC_CombatUnit) (Utilities|Struct|MakeS_CombatResource 0.0 0.0 0.0 (.spiritorb (Default|GetMaxStat (Variables|Default|GetBPC_CombatUnit))) 0.0)))
  (Utilities|FlowControl|Delay 0 0.5)
  (Default|SetStateStagger(Interrupt+) (Variables|Default|GetAs%20AIC%20Enermy) false))

(event Custom|HoBiDayVeTrongQuaTrinhNguoiChoiPerfectSpiritDodge)

(fn ConstructionScript)

(fn GetRangeDefend(StrafeRadius)
  (return 8e+02))

(fn SetMovementSpeed
  (params (Speed :type E_AI_Movement_State%20Enum :default "NewEnumerator0"))
  (bind _output_get (Variables|/Script/Engine.CharacterMovementComponent|SetMaxWalkSpeed (Variables|Character|GetCharacterMovement) (Utilities|Select :Index Speed :NewEnumerator0 0.0 :NewEnumerator1 3.5e+02 :NewEnumerator2 1.5e+02 :NewEnumerator3 183.333 :NewEnumerator4 2.5e+02 :NewEnumerator5 9e+02)))
  (return _output_get))