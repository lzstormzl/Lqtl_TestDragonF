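; Pawn camera component that handles target lock-on, velocity-driven FOV and eased spring-arm length changes.
; Tick drives lock-on and FOV, while looping timers ease lock-view blending in and out and animate arm length by curves.
; Lock view steers control rotation toward the target with distance-based pitch, scaling lag by speed and angle.
; SetLockOnActor sends focus messages and toggles an optional obscuration-trace timer, whose trace clears blocked targets.
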(event EventBeginPlay
  (bind _returnvalue (Components|GetOwner))
  (bind _aspawn (Utilities|Casting|CastToPawn _returnvalue))
  (Utilities|FlowControl|Sequence
    (:then_0
      (CallFunction|InitializeComponent _aspawn (Actor|GetComponentbyClass _aspawn "/Script/Engine.CameraComponent") (Actor|GetComponentbyClass _aspawn "/Script/Engine.SpringArmComponent") (Actor|GetComponentbyClass _aspawn "/Script/Engine.MovementComponent")))
    (:then_1
      (CallFunction|UpdateCameraLockon))))

(event EventTick
  (params (DeltaSeconds :type Float%20%28single-precision%29))
  (Utilities|FlowControl|Sequence
    (:then_0
      (CallFunction|UpdateCameraLockon))
    (:then_1
      (Controls|Internal|UpdateCameraDynamicFOV))))

(event Custom|Update%20Camera%20Lock%20On
  (Variables|CameraControl|LockOn|GetLock%20On%20Target
    (:then
      (Utilities|FlowControl|Sequence
        (:then_0
          (Utilities|FlowControl|DoOnce false :!label _label
            (:Completed
              (Utilities|FlowControl|Sequence
                (:then_0
                  (Variables|CameraControl|LockOn|SetLocking%20On%20Target false)
                  (Variables|InstancedData|SetElapsed%20Time%20Lock%20On 0.0)
                  (Variables|InstancedData|SetDelta%20Time%20Mult%20Lock%20On 1.0)
                  (bind _returnvalue (Utilities|Time|SetTimerbyEvent (EventDispatchers|CreateEvent :!event UpdateCameraProperties) 0.0001 true true :!label _label_2))
                  (Variables|CameraControl|LockOn|SetUpdate%20Camera%20Properties%20Timer%20Handle _returnvalue))
                (:then_1
                  (goto _label_3 Reset))))))
        (:then_1
          (if (Variables|CameraControl|LockOn|GetLocking%20On%20Target)
            (Controls|Internal|UpdateLockViewCameraProperties 1.0)))))
    (:else
      (Utilities|FlowControl|DoOnce false :!label _label_3
        (:Completed
          (Utilities|FlowControl|Sequence
            (:then_0
              (goto _label Reset))
            (:then_1
              (Variables|InstancedData|SetElapsed%20Time%20Lock%20On (Variables|CameraControl|LockOn|Ease|GetLock%20On%20Ease%20Duration))
              (Variables|InstancedData|SetDelta%20Time%20Mult%20Lock%20On -1.0)
              (goto _label_2))))))))

(fn GetTargetCameraRotation
  (bind _lock_on_target (Variables|CameraControl|LockOn|GetLock%20On%20Target)
    (:then
      (bind _out_vector (Class|BPILockonTarget|GetLockonLocation(Message) _lock_on_target))
      (if (<= (Transformation|GetDistanceTo _lock_on_target (Components|GetOwner)) 1e+03)
        (return (Math|Rotator|MakeRotator 0.0 (* (Math|Curves|GetFloatValue (Variables|Default|GetCurve) (/ (Transformation|GetDistanceTo _lock_on_target (Components|GetOwner)) 1e+03)) -1.0) (.yaw (Math|Rotator|FindLookatRotation (Transformation|GetActorLocation (Variables|References|GetOwner%20Pawn)) _out_vector))))
        (else
          (return (Math|Rotator|MakeRotator 0.0 (+ (.pitch (Math|Rotator|FindLookatRotation (Transformation|GetActorLocation (Variables|References|GetOwner%20Pawn)) _out_vector)) 0.0) (.yaw (Math|Rotator|FindLookatRotation (Transformation|GetActorLocation (Variables|References|GetOwner%20Pawn)) _out_vector)))))))
    (:else
      (return (Pawn|GetControlRotation (Variables|References|GetOwner%20Pawn) :!class /Script/Engine.Pawn)))))

(fn GetCameraLagSpeed
  (params (Free%20View :type Boolean))
  (if Free%20View
    (return (Variables|CameraControl|LockOn|SpeedLag|GetFree%20View%20Lag%20Speed))
    (else
      (return (+ (Variables|CameraControl|LockOn|SpeedLag|GetBase%20Lag%20Speed) (* (Math|Vector|VectorLengthXY (Variables|/Script/Engine.MovementComponent|GetVelocity (Variables|References|GetMovement%20Comp))) (Variables|CameraControl|LockOn|SpeedLag|GetLag%20Speed%20Multiplier)))))))

(fn GetCameraLagRotationSpeed
  (params (Free%20View :type Boolean))
  (bind _lock_on_target (Variables|CameraControl|LockOn|GetLock%20On%20Target))
  (if Free%20View
    (return (Variables|CameraControl|LockOn|RotationLag|GetFree%20View%20Rotation%20Lag))
    (else
      (Utilities|IsValid _lock_on_target
        (:Is%20Valid
          (bind _out_vector (Class|BPILockonTarget|GetLockonLocation(Message) _lock_on_target))
          (return (+ (Variables|CameraControl|LockOn|RotationLag|GetBase%20Rotation%20Lag%20Speed) (* (Math|Curves|GetFloatValue (Variables|CameraControl|LockOn|RotationLag|GetRotation%20Lag%20Curve) (Math|Float|Clamp(Float) (/ (- (CallFunction|FlatAngle(Vector) (Math|Vector|GetUnitDirection(Vector) (Transformation|GetActorLocation (Variables|References|GetOwner%20Pawn)) _out_vector) (Math|Vector|GetForwardVector (Transformation|GetWorldRotation (Variables|References|GetCamera)))) (Variables|CameraControl|LockOn|RotationLag|GetMin%20Angle)) (- (Variables|CameraControl|LockOn|RotationLag|GetMax%20Angle) (Variables|CameraControl|LockOn|RotationLag|GetMin%20Angle))))) (Variables|CameraControl|LockOn|RotationLag|GetRotation%20Lag%20Multiplier)))))))))

(fn UpdateLockViewCameraProperties
  (params (Lock%20View%20Weight :type Float%20%28double-precision%29))
  (Utilities|FlowControl|Sequence
    (:then_0
      (Variables|/Script/Engine.SpringArmComponent|SetCameraLagSpeed (Variables|References|GetSpringArm) (Math|Float|Lerp (Access|Internal|GetCameraLagSpeed true) (Access|Internal|GetCameraLagSpeed false) Lock%20View%20Weight)))
    (:then_1
      (Variables|/Script/Engine.SpringArmComponent|SetCameraRotationLagSpeed (Variables|References|GetSpringArm) (Math|Float|Lerp (Access|Internal|GetCameraLagRotationSpeed true) (Access|Internal|GetCameraLagRotationSpeed false) Lock%20View%20Weight)))
    (:then_2
      (Pawn|SetControlRotation (Pawn|GetController (Variables|References|GetOwner%20Pawn)) (Math|Rotator|Lerp(Rotator) (Pawn|GetControlRotation (Variables|References|GetOwner%20Pawn) :!class /Script/Engine.Pawn) (Access|Internal|GetTargetCameraRotation) Lock%20View%20Weight true)))))

(fn CheckLockViewTargetObscuration
  (bind _out_vector (Class|BPILockonTarget|GetCenterMassLocation(Message) (Variables|CameraControl|LockOn|GetLock%20On%20Target)))
  (bind _returnvalue (Collision|LineTraceForObjects (Transformation|GetWorldLocation (Variables|References|GetCamera)) _out_vector (Utilities|Array|MakeArray "ObjectTypeQuery1" "ObjectTypeQuery2") false 0 "None"))
  (if _returnvalue
    (Utilities|Time|ClearandInvalidateTimerbyHandle (Variables|CameraControl|LockOn|GetValid%20Lock%20On%20Target%20Timer))
    (Controls|SetLockonActor)))

(fn SetLockonActor
  (params (Actor :type Actor%20Object%20Reference))
  (if (!= Actor (Variables|CameraControl|LockOn|GetLock%20On%20Target))
    (Utilities|FlowControl|Sequence
      (:then_0
        (Utilities|IsValid Actor
          (:Is%20Valid
            (Class|BPILockonTarget|OnFocused(Message) Actor)
            (if (Variables|CameraControl|LockOn|ObscurationDetect|GetObscuration%20Check)
              (Utilities|Time|ClearandInvalidateTimerbyHandle (Variables|CameraControl|LockOn|GetValid%20Lock%20On%20Target%20Timer))))
          (:Is%20Not%20Valid
            (Class|BPILockonTarget|OnUnfocused(Message) (Variables|CameraControl|LockOn|GetLock%20On%20Target))
            (if (Variables|CameraControl|LockOn|ObscurationDetect|GetObscuration%20Check)
              (bind _returnvalue (Utilities|Time|SetTimerbyEvent (EventDispatchers|CreateEvent :!event CheckLockViewTargetObscuration) (Variables|CameraControl|LockOn|ObscurationDetect|GetObscuration%20Detect%20Loop%20Delay) true true))
              (Variables|CameraControl|LockOn|SetValid%20Lock%20On%20Target%20Timer _returnvalue)))))
      (:then_1
        (bind _output_get (Variables|CameraControl|LockOn|SetLock%20On%20Target Actor))
        (Default|CallOnLockonTargetUpdated _output_get)
        (bind _asbp_enemy (Utilities|Casting|CastToBP_Enemy Actor))
        (Widget|SetRenderOpacity (Variables|/Game/Characters/Enemies/BP_Enemy.BP_Enemy_C|GetLock%20On%20Indicator%20Widget _asbp_enemy) 1.0)))))

(fn InitializeComponent
  (params (Owner%20Pawn :type Pawn%20Object%20Reference) (Camera :type Camera%20Component%20Object%20Reference) (SpringArm :type Spring%20Arm%20Component%20Object%20Reference) (Movement%20Comp :type Movement%20Component%20Object%20Reference))
  (if (not (Variables|InstancedData|GetInitialized))
    (Utilities|FlowControl|Sequence
      (:then_0
        (Variables|References|SetOwner%20Pawn Owner%20Pawn)
        (Variables|References|SetCamera Camera)
        (Variables|References|SetSpringArm SpringArm)
        (Variables|References|SetMovement%20Comp Movement%20Comp))
      (:then_1
        (Variables|InstancedData|SetInitialized (Math|Boolean|ANDBoolean (Utilities|IsValid (Variables|References|GetCamera)) (Utilities|IsValid (Variables|References|GetSpringArm)) (Utilities|IsValid (Variables|References|GetOwner%20Pawn)) (Utilities|IsValid (Variables|References|GetMovement%20Comp))))))))

(fn IsLockViewActive
  (return (Utilities|IsValid (Variables|CameraControl|LockOn|GetLock%20On%20Target))))

(fn UpdateCameraProperties
  (Variables|InstancedData|SetElapsed%20Time%20Lock%20On (+ (Variables|InstancedData|GetElapsed%20Time%20Lock%20On) (* (Utilities|Time|GetWorldDeltaSeconds) (Variables|InstancedData|GetDelta%20Time%20Mult%20Lock%20On))))
  (if (Math|Float|InRange(Float) (Variables|InstancedData|GetElapsed%20Time%20Lock%20On) 0.0 (Variables|CameraControl|LockOn|Ease|GetLock%20On%20Ease%20Duration) false false)
    (Controls|Internal|UpdateLockViewCameraProperties (Math|Curves|GetFloatValue (Variables|CameraControl|LockOn|Ease|GetLock%20On%20Ease%20Curve) (/ (Variables|InstancedData|GetElapsed%20Time%20Lock%20On) (Variables|CameraControl|LockOn|Ease|GetLock%20On%20Ease%20Duration))))
    (else
      (Variables|CameraControl|LockOn|SetLocking%20On%20Target true)
      (Utilities|Time|ClearandInvalidateTimerbyHandle (Variables|CameraControl|LockOn|GetUpdate%20Camera%20Properties%20Timer%20Handle)))))

(fn GetLockonActor
  (return (Variables|CameraControl|LockOn|GetLock%20On%20Target)))

(fn SetDynamicFOV
  (params (Active :type Boolean) (Velocity%20Mult :type Float%20%28double-precision%29) (Min :type Float%20%28double-precision%29) (Max :type Float%20%28double-precision%29))
  (Variables|CameraControl|DynamicFOV|SetDynamic%20FOV%20Active Active)
  (Variables|CameraControl|DynamicFOV|SetFOV%20Velocity%20Mult Velocity%20Mult)
  (Variables|CameraControl|DynamicFOV|SetMin%20FOV%20 Min)
  (Variables|CameraControl|DynamicFOV|SetMax%20FOV Max)
  (if (not (Variables|CameraControl|DynamicFOV|GetDynamic%20FOV%20Active))
    (Camera|SetFieldOfView (Variables|References|GetCamera) (Variables|CameraControl|DynamicFOV|GetOrginal%20FOV))))

(fn SetTargetCameraArmLength
  (params (New%20Arm%20Length :type Float%20%28double-precision%29) (Ease%20Duration :type Float%20%28double-precision%29) (Ease%20Curve :type Curve%20Float%20Object%20Reference))
  (Variables|CameraControl|ManualArmLength|SetTarget%20Arm%20Length New%20Arm%20Length)
  (Variables|CameraControl|ManualArmLength|SetArm%20Length%20Ease%20Duration Ease%20Duration)
  (Variables|CameraControl|ManualArmLength|SetArm%20Length%20Ease%20Curve Ease%20Curve)
  (Utilities|FlowControl|Sequence
    (:then_0
      (Variables|InstancedData|SetElapsed%20Time%20Arm%20Length 0.0)
      (Variables|CameraControl|ManualArmLength|SetOrginal%20Arm%20Length (Variables|/Script/Engine.SpringArmComponent|GetTargetArmLength (Variables|References|GetSpringArm))))
    (:then_1
      (bind _returnvalue (Utilities|Time|SetTimerbyEvent (EventDispatchers|CreateEvent :!event UpdateCameraArmLength) 0.001 true true))
      (Variables|CameraControl|ManualArmLength|SetManual%20Arm%20Length%20Timer%20Handle _returnvalue))))

(fn UpdateCameraDynamicFOV
  (if (Variables|CameraControl|DynamicFOV|GetDynamic%20FOV%20Active)
    (Camera|SetFieldOfView (Variables|References|GetCamera) (Math|Float|Clamp(Float) (* (Math|Vector|VectorLengthXY (Variables|/Script/Engine.MovementComponent|GetVelocity (Variables|References|GetMovement%20Comp))) (Variables|CameraControl|DynamicFOV|GetFOV%20Velocity%20Mult)) (Variables|CameraControl|DynamicFOV|GetMin%20FOV%20) (Variables|CameraControl|DynamicFOV|GetMax%20FOV)))))

(fn UpdateCameraArmLength
  (Variables|InstancedData|SetElapsed%20Time%20Arm%20Length (+ (Variables|InstancedData|GetElapsed%20Time%20Arm%20Length) (Utilities|Time|GetWorldDeltaSeconds)))
  (if (< (Variables|InstancedData|GetElapsed%20Time%20Arm%20Length) (Variables|CameraControl|ManualArmLength|GetArm%20Length%20Ease%20Duration))
    (Variables|/Script/Engine.SpringArmComponent|SetTargetArmLength (Variables|References|GetSpringArm) (Math|Float|Lerp (Variables|CameraControl|ManualArmLength|GetOrginal%20Arm%20Length) (Variables|CameraControl|ManualArmLength|GetTarget%20Arm%20Length) (Math|Curves|GetFloatValue (Variables|CameraControl|ManualArmLength|GetArm%20Length%20Ease%20Curve) (/ (Variables|InstancedData|GetElapsed%20Time%20Arm%20Length) (Variables|CameraControl|ManualArmLength|GetArm%20Length%20Ease%20Duration)))))
    (else
      (Variables|/Script/Engine.SpringArmComponent|SetTargetArmLength (Variables|References|GetSpringArm) (Variables|CameraControl|ManualArmLength|GetTarget%20Arm%20Length))
      (Utilities|Time|ClearandInvalidateTimerbyHandle (Variables|CameraControl|ManualArmLength|GetManual%20Arm%20Length%20Timer%20Handle)))))