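; Actor component that spawns melee-style hitboxes on the owner's skeletal mesh and reports attack hits.
; GenerateHitbox and DestroyHitbox take capsules from a pool and return them, fitting each between two offset sockets.
; Overlaps, including manually checked ones on enable, fire OnAttackHit with DT_AttackData, hit count and direction.
; A per-actor bitmask of hitbox IDs blocks repeat hits until ResetOverlapIDTrack clears it.
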(event EventBeginPlay
  (CallFunction|InitializeComponent (Actor|GetComponentbyClass (Components|GetOwner) "/Script/Engine.SkeletalMeshComponent")))

(fn InitializeComponent
  (params (Mesh :type Skeletal%20Mesh%20Component%20Object%20Reference))
  (if (not (Variables|InstancedData|GetInitialized))
    (Utilities|FlowControl|Sequence
      (:then_0
        (Variables|References|SetAnimated%20Mesh Mesh))
      (:then_1
        (Variables|InstancedData|SetInitialized (Utilities|IsValid Mesh))))))

(fn InitializeHitboxEvent
  (params (Capsule%20Collision :type Capsule%20Component%20Object%20Reference))
  (Collision|BindEventtoOnComponentBeginOverlap Capsule%20Collision (EventDispatchers|CreateEvent :!event OnHitboxOverlap)))

(fn AcquireCollisionfromPool
  (Utilities|FlowControl|Sequence
    (:then_0
      (if (Utilities|Array|IsEmpty (Variables|Hitbox|Pool|GetCollision%20Pool))
        ;[0.02 0.02 0.02] Create New Component
        (bind _returnvalue (Game|AddComponentbyClass (Components|GetOwner) "/Script/Engine.CapsuleComponent" false))
        (LocalVariables|SetOut _returnvalue)
        (Collision|SetCollisionProfileName (LocalVariables|GetOut) "Hitbox" false :!class /Script/Engine.PrimitiveComponent)
        (Components|Tick|SetComponentTickEnabled (LocalVariables|GetOut) true)
        (HitboxControl|Internal|InitializeHitboxEvent (LocalVariables|GetOut))
        (Variables|/Script/Engine.PrimitiveComponent|SetbGenerateOverlapEvents (LocalVariables|GetOut) true)
        (Math|Integer|IncrementInt (Variables|Hitbox|Data|GetHitbox%20Collision%20Count))
        (else
          ;[0.02 0.02 0.02] Get From Pool
          (LocalVariables|SetOut (Utilities|Array|Get(acopy) (Variables|Hitbox|Pool|GetCollision%20Pool)))
          (Utilities|Array|RemoveIndex (Variables|Hitbox|Pool|GetCollision%20Pool)))))
    (:then_1
      (return (LocalVariables|GetOut)))))

(fn ReleaseCollisiontoPool
  (params (Collision :type Capsule%20Component%20Object%20Reference))
  (Utilities|Array|Add (Variables|Hitbox|Pool|GetCollision%20Pool) Collision))

(fn ApplyHitboxDatatoCapsuleCollision
  (params (Capsule%20Collision :type Capsule%20Component%20Object%20Reference) (Hitbox%20Data :type S%20Hitbox%20Data%20Structure))
  (Utilities|FlowControl|Sequence
    (:then_0
      (LocalVariables|SetStart%20Location (CallFunction|GetSocketLocationatOffset (Variables|References|GetAnimated%20Mesh) (.startsocket Hitbox%20Data) (.startoffset Hitbox%20Data)))
      (LocalVariables|SetEnd%20Location (CallFunction|GetSocketLocationatOffset (Variables|References|GetAnimated%20Mesh) (.endsocket Hitbox%20Data) (.endoffset Hitbox%20Data))))
    (:then_1
      (Transformation|AttachComponentToComponent Capsule%20Collision (Variables|References|GetAnimated%20Mesh) (.startsocket Hitbox%20Data) "SnapToTarget" "SnapToTarget" "SnapToTarget" true)
      (Components|Capsule|SetCapsuleRadius Capsule%20Collision (.radius Hitbox%20Data) false)
      (Transformation|AddWorldOffset Capsule%20Collision (* (- (/ (Math|Vector|Distance(Vector) (LocalVariables|GetStart%20Location) (LocalVariables|GetEnd%20Location)) 2.0) (Math|Vector|Distance(Vector) (Transformation|GetSocketLocation (Variables|References|GetAnimated%20Mesh) (.startsocket Hitbox%20Data)) (LocalVariables|GetStart%20Location))) (Math|Vector|GetUnitDirection(Vector) (LocalVariables|GetStart%20Location) (LocalVariables|GetEnd%20Location))) false true)
      (Transformation|SetWorldRotation Capsule%20Collision (CallFunction|GetCapsuleRotationfromto (LocalVariables|GetStart%20Location) (LocalVariables|GetEnd%20Location)) false false)
      (Components|Capsule|SetCapsuleHalfHeight Capsule%20Collision (/ (Math|Vector|Distance(Vector) (LocalVariables|GetStart%20Location) (LocalVariables|GetEnd%20Location)) 2.0) true))))

(fn OnHitboxOverlap
  (params (OverlappedComponent :type Primitive%20Component%20Object%20Reference) (OtherActor :type Actor%20Object%20Reference) (OtherComp :type Primitive%20Component%20Object%20Reference) (OtherBodyIndex :type Integer) (bFromSweep :type Boolean) (SweepResult :type Hit%20Result%20Structure%20%28by%20ref%29))
  (bind _overlap_id_track (Variables|Hitbox|Data|GetOverlap%20ID%20Track))
  (if (not (== (Components|GetOwner (Variables|References|GetAnimated%20Mesh)) OtherActor))
    (LocalVariables|SetHitbox%20Data (.Value (Utilities|Map|Find (Variables|Hitbox|Data|GetHitbox%20Data%20Lookup) OverlappedComponent)))
    (if (== (Class|KismetMathLibrary|AndInt64Int64 (.Value (Utilities|Map|Find (Variables|Hitbox|Data|GetOverlap%20ID%20Track) OtherActor)) (Class|KismetMathLibrary|Round64 (Math|Float|Power 2.0 (Math|Conversions|ToFloat(Integer) (Utilities|Struct|BreakS_HitboxData (LocalVariables|GetHitbox%20Data)))))) 0)
      (bind _returnvalue (Utilities|GetDataTableRow "/Game/Developers/Admin/Data/DataTables/GeneralCombat/DT_AttackData.DT_AttackData" (Utilities|Struct|BreakS_HitboxData (LocalVariables|GetHitbox%20Data)))
        (:then
          (LocalVariables|SetHit%20Count (.Value (Utilities|Map|Find (Variables|Hitbox|Data|GetHitbox%20Hit%20Count%20Lookup) OverlappedComponent)))
          (Default|CallOnAttackHit OtherActor _returnvalue (LocalVariables|GetHit%20Count) (Utility|CalculateRelativeHitDirection OtherComp (LocalVariables|GetHitbox%20Data)))
          (Utilities|Map|Add _overlap_id_track OtherActor (Class|KismetMathLibrary|OrInt64Int64 (.Value (Utilities|Map|Find _overlap_id_track OtherActor)) (Class|KismetMathLibrary|Round64 (Math|Float|Power 2.0 (Math|Conversions|ToFloat(Integer) (Utilities|Struct|BreakS_HitboxData (LocalVariables|GetHitbox%20Data)))))))
          (Utilities|Map|Add (Variables|Hitbox|Data|GetHitbox%20Hit%20Count%20Lookup) OverlappedComponent (+ (LocalVariables|GetHit%20Count) 1)))))))

(fn SetHitboxEnabled
  (params (Capsule%20Collision :type Capsule%20Component%20Object%20Reference) (Enable :type Boolean) (Hitbox%20Data :type S%20Hitbox%20Data%20Structure))
  (Utilities|FlowControl|Sequence
    (:then_0
      (Collision|SetCollisionEnabled Capsule%20Collision (select Enable "QueryAndPhysics" "NoCollision"))
      (Development|SetHiddeninGame Capsule%20Collision true false))
    (:then_1
      (if Enable
        (HitboxControl|Internal|ApplyHitboxDatatoCapsuleCollision Capsule%20Collision Hitbox%20Data)
        (else
          (Transformation|DetachFromComponent Capsule%20Collision "KeepRelative" "KeepRelative" "KeepRelative" true))))
    (:then_2
      ;[1 0.2135 0.2135] Manually detect overlapped Actors since PrimativeComponent does not automatically detect already overlapping objects when enabled
      (for _array_element (Class|PrimitiveComponent|GetOverlappingComponents Capsule%20Collision)
        (HitboxControl|Internal|OnHitboxOverlap Capsule%20Collision (Components|GetOwner _array_element) _array_element 0 false)))))

(fn GetUniqueHitboxKey
  (params (Hitbox%20Data :type S%20Hitbox%20Data%20Structure))
  (bind (_id _attackdataname _startsocket _endsocket _startoffset _endoffset _radius) (Utilities|Struct|BreakS_HitboxData Hitbox%20Data))
  (return (Utilities|String|Append (Utilities|String|ToString(Name) _startsocket) (Utilities|String|ToString(Name) _endsocket) (Utilities|String|ToString(Vector) _startoffset) (Utilities|String|ToString(Vector) _endoffset) (Utilities|String|ToString(Float) _radius) (Utilities|GetDisplayName (Components|GetOwner)))))

(fn ResetOverlapIDTrack
  (Utilities|Map|Clear (Variables|Hitbox|Data|GetOverlap%20ID%20Track)))

(fn GenerateHitbox
  (params (Hitbox%20Data :type S%20Hitbox%20Data%20Structure))
  (Utilities|FlowControl|Sequence
    (:then_0
      (LocalVariables|SetCapsule%20Comp (Pool|AcquireCollisionfromPool))
      (LocalVariables|SetKey (Utility|GetUniqueHitboxKey Hitbox%20Data)))
    (:then_1
      (Utilities|Map|Add (Variables|Hitbox|Data|GetHitbox%20Hit%20Count%20Lookup) (LocalVariables|GetCapsule%20Comp) 0)
      (Utilities|Map|Add (Variables|Hitbox|Data|GetHitbox%20Collision%20Lookup) (LocalVariables|GetKey) (LocalVariables|GetCapsule%20Comp))
      (Utilities|Map|Add (Variables|Hitbox|Data|GetHitbox%20Data%20Lookup) (LocalVariables|GetCapsule%20Comp) Hitbox%20Data))
    (:then_2
      (HitboxControl|Internal|SetHitboxEnabled (LocalVariables|GetCapsule%20Comp) true Hitbox%20Data)
      (return true))))

(fn DestroyHitbox
  (params (Hitbox%20Data :type S%20Hitbox%20Data%20Structure))
  (bind _output_get (LocalVariables|SetKey (Utility|GetUniqueHitboxKey Hitbox%20Data)))
  (bind _output_get_2 (LocalVariables|SetCollision (.Value (Utilities|Map|Find (Variables|Hitbox|Data|GetHitbox%20Collision%20Lookup) _output_get))))
  (Utilities|IsValid _output_get_2
    (:Is%20Valid
      (Utilities|FlowControl|Sequence
        (:then_0
          (HitboxControl|Internal|SetHitboxEnabled (LocalVariables|GetCollision) false)
          (Pool|ReleaseCollisiontoPool (LocalVariables|GetCollision)))
        (:then_1
          (Utilities|Map|Remove (Variables|Hitbox|Data|GetHitbox%20Data%20Lookup) (LocalVariables|GetCollision))
          (Utilities|Map|Remove (Variables|Hitbox|Data|GetHitbox%20Collision%20Lookup) (LocalVariables|GetKey))
          (Utilities|Map|Remove (Variables|Hitbox|Data|GetHitbox%20Hit%20Count%20Lookup) (LocalVariables|GetCollision)))))))

(fn CalculateRelativeHitDirection
  (params (Hit%20Comp :type Primitive%20Component%20Object%20Reference%20%28by%20ref%29) (Hitbox%20Data :type S%20Hitbox%20Data%20Structure))
  (bind (_startsocket _startoffset) (Utilities|Struct|BreakS_HitboxData Hitbox%20Data))
  (return (Math|Vector|SelectVector (Math|Vector|GetUnitDirection(Vector) (CallFunction|GetSocketLocationatOffset (Variables|References|GetAnimated%20Mesh) _startsocket _startoffset) (Transformation|GetWorldLocation Hit%20Comp)) (CallFunction|GetHitboxWorldHitDirection (Variables|References|GetAnimated%20Mesh) Hitbox%20Data) (Utilities|Operators|EqualEqual :A (Utilities|Struct|BreakS_HitboxData Hitbox%20Data)))))