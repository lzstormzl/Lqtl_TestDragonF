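; Actor component that manages a character's carried equipment, spawning BP_EquipmentBase actors from data and attaching them to skeletal mesh sockets.
; Equip and holster montages move items between hand and holster sockets on notifies, holstering the current item before equipping another and broadcasting change events.
; Holstered items fan out by an index-scaled rotation offset.
; A visibility mode controls which items show, and disabling equipment hides all and blocks actions.
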(event EventBeginPlay
  (CallFunction|InitializeComponent (Actor|GetComponentbyClass (Components|GetOwner) "/Script/Engine.SkeletalMeshComponent"))
  (Attach&Equip|SetEquipmentVisibilityMode (Variables|Data|GetDefault%20Visibility%20Mode))
  (Utilities|FlowControl|DelayUntilNextTick)
  (Default|CallOnEquippedEquipmentChanged))

(event Custom|Event%20Holster%20Equipment%20Montage
  (params (Equipment :type BP%20Equipment%20Base%20Object%20Reference) (Reset%20Equipped%20Index :type Boolean))
  ;[0.02 0.02 0.02] Holster Equipment
  (bind _notifyname (Animation|Montage|PlayMontage (Variables|Reference|GetSkeletal%20Mesh) (Utilities|Struct|BreakS_EquipmentData (Default|GetEquipmentData Equipment)))
    (:OnNotifyBegin
      (switch name _notifyname
        (:E
          (Attach&Equip|Internal|HolsterEquipment Equipment Reset%20Equipped%20Index))))))

(event Custom|Event%20Equip%20Equipment%20Montage
  (params (Equipment%20Index :type Integer))
  ;[0.02 0.02 0.02] Equip Equipment
  (Variables|Data|Internal|SetLocal_Equipment%20Index Equipment%20Index)
  (if (Access|HasEquippedEquipment)
    ;;[0.02 0.02 0.02] Holster Current Weapon If Has
    (bind _notifyname (Animation|Montage|PlayMontage (Variables|Reference|GetSkeletal%20Mesh) (.HolsterAnimation (Utilities|Struct|BreakS_EquipmentData (Default|GetEquipmentData (Utilities|Array|Get(acopy) (Variables|Equipment|GetAttached%20Equipments) (Variables|Data|Internal|GetLocal_Equipment%20Index))))) 1.2)
      (:OnNotifyBegin
        (switch name _notifyname
          (:E
            (Attach&Equip|Internal|HolsterEquipment (.Equipment (Access|GetEquippedEquipment)) true)
            (bind _notifyname_2 (Animation|Montage|PlayMontage (Variables|Reference|GetSkeletal%20Mesh) (.EquipAnimation (Utilities|Struct|BreakS_EquipmentData (Default|GetEquipmentData (Utilities|Array|Get(acopy) (Variables|Equipment|GetAttached%20Equipments) (Variables|Data|Internal|GetLocal_Equipment%20Index))))) 1.2 0.0 "Start")
              (:OnNotifyBegin
                (switch name _notifyname_2
                  (:E
                    _))))))))
    (else
      (bind _notifyname_3 (Animation|Montage|PlayMontage (Variables|Reference|GetSkeletal%20Mesh) (.EquipAnimation (Utilities|Struct|BreakS_EquipmentData (Default|GetEquipmentData (Utilities|Array|Get(acopy) (Variables|Equipment|GetAttached%20Equipments) (Variables|Data|Internal|GetLocal_Equipment%20Index))))))
        (:OnNotifyBegin
          (switch name _notifyname_3
            (:E
              _))))))
  (bind _result (Attach&Equip|Internal|AttachEquipmenttoSocket (Utilities|Array|Get(acopy) (Variables|Equipment|GetAttached%20Equipments) (Variables|Data|Internal|GetLocal_Equipment%20Index)) (.EquipSocket (Utilities|Struct|BreakS_EquipmentData (Default|GetEquipmentData (Utilities|Array|Get(acopy) (Variables|Equipment|GetAttached%20Equipments) (Variables|Data|Internal|GetLocal_Equipment%20Index))))) (.EquipOffset (Utilities|Struct|BreakS_EquipmentData (Default|GetEquipmentData (Utilities|Array|Get(acopy) (Variables|Equipment|GetAttached%20Equipments) (Variables|Data|Internal|GetLocal_Equipment%20Index)))))))
  (Utilities|FlowControl|Sequence
    (:then_0
      (if _result
        (bind _output_get (Variables|Equipment|SetEquipped%20Index (Variables|Data|Internal|GetLocal_Equipment%20Index)))
        (Variables|Equipment|SetLast%20Equipped%20Index _output_get)
        (Default|CallOnEquippedEquipmentChanged (.Equipment (Access|GetEquippedEquipment)))))
    (:then_1
      (switch Utilities|FlowControl|Switch|SwitchonE_EquipmentVisibilityMode (Variables|Data|Internal|GetCurrent%20Visibility%20Mode)
        (:NewEnumerator0
          _)
        (:NewEnumerator1
          _))
      (Rendering|SetActorHiddenInGame (.Equipment (Access|GetEquippedEquipment)) false))))

(fn Equip(ObjectReference)
  (params (Equipment :type BP%20Equipment%20Base%20Object%20Reference))
  (if (Variables|Data|Internal|GetEquipment%20Enabled)
    (bind _result (Attach&Equip|Internal|EquipEquipment (Utilities|Array|FindItem (Variables|Equipment|GetAttached%20Equipments) Equipment)))
    (return _result)))

(fn Equip(Index)
  (params (Index :type Integer))
  (if (Variables|Data|Internal|GetEquipment%20Enabled)
    (bind _result (Attach&Equip|Internal|EquipEquipment Index))
    (return _result)))

(fn HolsterCurrentEquipment
  (params (Play%20Animation :type Boolean))
  (bind (_equipment _result) (Access|GetEquippedEquipment))
  (if (Variables|Data|Internal|GetEquipment%20Enabled)
    (LocalVariables|SetCurrent%20Equipment _equipment)
    (if _result
      (if Play%20Animation
        (CallFunction|EventHolsterEquipmentMontage (LocalVariables|GetCurrent%20Equipment) true)
        (else
          (Attach&Equip|Internal|HolsterEquipment (LocalVariables|GetCurrent%20Equipment) true))))))

(fn GetAttachedEquipments
  (return (Variables|Equipment|GetAttached%20Equipments)))

(fn GetEquippedEquipment
  (if (Access|HasEquippedEquipment)
    (return (Utilities|Array|Get(acopy) (Variables|Equipment|GetAttached%20Equipments) (Variables|Equipment|GetEquipped%20Index)) true)
    (else
      (return 0 false))))

(fn AttachEquipment
  (params (Equipment%20Data :type S%20Equipment%20Data%20Structure))
  (bind _attached_equipments (Variables|Equipment|GetAttached%20Equipments))
  (if (Variables|Data|Internal|GetEquipment%20Enabled)
    (bind _output_get (LocalVariables|SetEquipment (Attach&Equip|Internal|SpawnEquipmentfromData Equipment%20Data)))
    (Utilities|IsValid _output_get
      (:Is%20Valid
        (bind _returnvalue (Utilities|Array|AddUnique _attached_equipments (LocalVariables|GetEquipment)))
        (if (Utilities|Array|IsValidIndex _attached_equipments _returnvalue)
          (Attach&Equip|Internal|HolsterEquipment (LocalVariables|GetEquipment) false)
          (Default|CallOnNewEquipmentAttached (LocalVariables|GetEquipment)))))))

(fn GetEquippedIndex
  (return (Variables|Equipment|GetEquipped%20Index)))

(fn DetachEquipment
  (params (Equipment :type BP%20Equipment%20Base%20Object%20Reference))
  (if (Variables|Data|Internal|GetEquipment%20Enabled)
    (bind _output_get (LocalVariables|SetRemoved%20Equipment%20Index (Utilities|Array|FindItem (Variables|Equipment|GetAttached%20Equipments) Equipment)))
    (if (!= _output_get -1)
      (Utilities|FlowControl|Sequence
        (:then_0
          ;[0.02 0.02 0.02] Detach from Player
          (Utilities|Array|RemoveItem (Variables|Equipment|GetAttached%20Equipments) Equipment)
          (Transformation|DetachFromActor Equipment "KeepWorld" "KeepWorld" "KeepWorld")
          (Default|CallOnEquipmentDetached Equipment))
        (:then_1
          ;[0.02 0.02 0.02] Unequip if currently equipped
          (if (== (LocalVariables|GetRemoved%20Equipment%20Index) (Variables|Equipment|GetEquipped%20Index))
            (Variables|Equipment|SetEquipped%20Index -1)))))))

(fn SpawnEquipmentfromData
  (params (Data :type S%20Equipment%20Data%20Structure))
  (bind _returnvalue (Game|SpawnActorfromClass "/Game/GeneralCombat/Blueprints/Equipment/BP_EquipmentBase.BP_EquipmentBase_C" (Math|Transform|MakeTransform "0, 0, 0" "0, 0, 0" "1.000000,1.000000,1.000000") "Undefined" "MultiplyWithRoot" 0 Data 0))
  (return _returnvalue))

(fn AttachEquipmenttoSocket
  (params (Equipment :type BP%20Equipment%20Base%20Object%20Reference) (Socket%20Name :type Name) (Offset%20 :type Transform))
  (bind _returnvalue (Transformation|AttachComponentToComponent Equipment (Variables|Reference|GetSkeletal%20Mesh) Socket%20Name "KeepRelative" "KeepRelative" "KeepRelative" true))
  (if _returnvalue
    (Transformation|SetRelativeTransform (Variables|/Script/Engine.Actor|GetRootComponent Equipment) Offset%20 false true)
    (return true)
    (else
      (return false))))

(fn InitializeComponent
  (params (Skeletal%20Mesh :type Skeletal%20Mesh%20Component%20Object%20Reference))
  (if (not (Variables|Reference|GetInitialized))
    (Utilities|FlowControl|Sequence
      (:then_0
        (Variables|Reference|SetSkeletal%20Mesh Skeletal%20Mesh))
      (:then_1
        (Variables|Reference|SetInitialized (Utilities|IsValid (Variables|Reference|GetSkeletal%20Mesh)))))))

(fn HasEquippedEquipment
  (return (and (!= (Variables|Equipment|GetEquipped%20Index) -1) (Variables|Data|Internal|GetEquipment%20Enabled))))

(fn GetHolsteredEquipmentCount
  (return (- (Utilities|Array|Length (Variables|Equipment|GetAttached%20Equipments)) (Math|Integer|SelectInt 1 0 (Access|HasEquippedEquipment)))))

(fn EquipEquipment
  (params (Index :type Integer))
  (if (Utilities|Array|IsValidIndex (Variables|Equipment|GetAttached%20Equipments) Index)
    (CallFunction|EventEquipEquipmentMontage Index)
    (return true)
    (else
      (return false))))

(fn HolsterEquipment
  (params (Equipment :type BP%20Equipment%20Base%20Object%20Reference) (Reset%20Equipped%20Index :type Boolean))
  (bind _equipment_data (Default|GetEquipmentData Equipment))
  (bind (_holstersocket _holsteroffset) (Utilities|Struct|BreakS_EquipmentData _equipment_data))
  (bind (_location _rotation _scale) (Math|Transform|BreakTransform _holsteroffset))
  (bind _result (Attach&Equip|Internal|AttachEquipmenttoSocket Equipment _holstersocket (Math|Transform|MakeTransform _location (Math|Rotator|CombineRotators _rotation (* (Math|Rotator|MakeRotator -5.0 0.0 -2e+01) (Utilities|Array|FindItem (Variables|Equipment|GetAttached%20Equipments) Equipment))) _scale)))
  (Utilities|FlowControl|Sequence
    (:then_0
      (if (and _result Reset%20Equipped%20Index)
        (Variables|Equipment|SetEquipped%20Index -1)
        (Default|CallOnEquippedEquipmentChanged)))
    (:then_1
      (switch Utilities|FlowControl|Switch|SwitchonE_EquipmentVisibilityMode (Variables|Data|Internal|GetCurrent%20Visibility%20Mode)
        (:NewEnumerator1
          _)
        (:NewEnumerator2
          _))
      (Rendering|SetActorHiddenInGame Equipment true))))

(fn SetEquipmentVisibilityMode
  (params (Visibility :type E_EquipmentVisibilityMode%20Enum :default "NewEnumerator0"))
  (if (Utilities|Enum|NotEqual(Enum) Visibility (Variables|Data|Internal|GetCurrent%20Visibility%20Mode))
    (bind _output_get (Variables|Data|Internal|SetCurrent%20Visibility%20Mode Visibility))
    (switch Utilities|FlowControl|Switch|SwitchonE_EquipmentVisibilityMode _output_get
      (:NewEnumerator0
        (|ShowAll))
      (:NewEnumerator1
        (|HideUnequipped))
      (:NewEnumerator2
        (|HideAll)))))

(fn SetEquipmentEnabled
  (params (Enabled :type Boolean))
  (bind _output_get (Variables|Data|Internal|SetEquipment%20Enabled Enabled))
  (if _output_get
    (Attach&Equip|SetEquipmentVisibilityMode (Variables|Data|GetDefault%20Visibility%20Mode))
    (Default|CallOnEquippedEquipmentChanged (.Equipment (Access|GetEquippedEquipment)))
    (else
      (Attach&Equip|SetEquipmentVisibilityMode "NewEnumerator2"))))

(fn GetEquipmentEnabled
  (return (Variables|Data|Internal|GetEquipment%20Enabled)))