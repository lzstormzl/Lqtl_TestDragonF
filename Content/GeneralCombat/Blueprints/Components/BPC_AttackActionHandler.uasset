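; Actor component that runs combo attacks for the player and for team 2 or Legion-tagged AI, with separate branches for each.
; Combos come from data tables; each attack deducts a combat-unit stat cost and plays its montage.
; Montage notifies open input registration, chain queued or auto-registered attacks, or end the combo.
; A looping timer updates motion-warp targets from the lock-on target, movement direction, or AI attack target, with range limits.
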(event EventBeginPlay
  (Setup|InitializeComponent (Actor|GetComponentbyClass (Components|GetOwner) "/Script/Engine.SkeletalMeshComponent")))

(event Custom|Handle%20Next%20Attack
  (bind _out_character (CallFunction|GetPlayerCombatCharacter))
  (bind _returnvalue (Components|GetOwner))
  (bind _returnvalue_2 (Components|GetOwner))
  (bind _teamnumber (Class|BPIDamageSystem|GetTeamNumber(Message) _returnvalue))
  ;[0.02 0.02 0.02 1 30] Handle Attack Register & Play Animation Montage
  (if (or (== _teamnumber 2) (Actor|ActorHasTag _returnvalue "Legion"))
    (Utilities|FlowControl|Sequence
      (:then_0
        ;;[0.1117 0.5677 0.3101] Get Next Attack Index
        (bind _result (Math|Integer|IncrementInt (Variables|ComboControl|GetAttack%20Index))
          (:%20%20
            (if (>= _result (Utilities|Array|Length (.attacksname (Variables|ComboControl|GetCurrent%20Attack%20Combo))))
              ;;[1 0.4863 0.2222] Reset combo when end attack reached, or stop attacking if auto register is enabled
              (Variables|AttackControl|SetAttacking false)
              (Variables|ComboControl|SetAttack%20Index 0)
              (Default|CallOnComboFinished)
              (if (Variables|AttackControl|GetAuto%20Register%20Next%20Attack)
                (Variables|AttackControl|SetAuto%20Register%20Next%20Attack false)
                (Variables|ComboControl|SetAttack%20Index -1)
                (Variables|AttackControl|SetAttack%20Registerd false)
                (else
                  ;[1 0.4863 0.2222] Cancel last attack animation on new attack
                  (Controls|CancelCurrentAttackMontage -1.0 :!label _label)
                  (Variables|AttackControl|SetCan%20Register%20Attack false)
                  (Variables|ComboControl|SetCan%20Chain%20Attack false)
                  (Variables|AttackControl|SetAttack%20Registerd false)
                  (Variables|AttackControl|SetAttacking true)
                  (bind _asbp_enemy (Utilities|Casting|CastToBP_Enemy _returnvalue_2))
                  (Default|AddCurrentStat (Variables|/Game/Characters/Enemies/BP_Enemy.BP_Enemy_C|GetBPC_CombatUnit _asbp_enemy) (Class|BFLCombatResource|MultFloat (Access|GetNextAttackCost) -1.0) _returnvalue_2)))
              (else
                (goto _label))))))
      (:then_1
        (if (Variables|AttackControl|GetAttacking)
          (Utilities|FlowControl|Sequence
            (:then_0
              ;[1 0.4863 0.2222] Initiate Attack
              (Default|CallOnAttackInitiated (Access|GetCurrentAttackActionData))
              (Utilities|Time|ClearandInvalidateTimerbyHandle (Variables|ComboControl|GetReset%20Combo%20Timer)))
            (:then_1
              (Controls|Internal|StartMotionWarping)
              (bind _output_get (Variables|ComboControl|SetCurrent%20Attack%20Montage (Access|Internal|GetAttackMontageatIndex (Variables|ComboControl|GetCurrent%20Attack%20Combo) (Variables|ComboControl|GetAttack%20Index))))
              (bind _notifyname (Animation|Montage|PlayMontage (Variables|References|GetAnimated%20Mesh) _output_get)
                (:then
                  (Utilities|FlowControl|DelayUntilNextTick)
                  (Variables|AttackControl|SetIn%20Attack%20Animation true))
                (:OnBlendOut
                  (Utilities|FlowControl|Sequence
                    (:then_0
                      (Variables|AttackControl|SetCan%20Register%20Attack true :!label _label_2)
                      (Variables|AttackControl|SetAttacking false)
                      (Variables|AttackControl|SetIn%20Attack%20Animation false)
                      (Variables|AttackControl|SetAttack%20Registerd false))
                    (:then_1
                      (Default|CallOnAttackFinished true))))
                (:OnInterrupted
                  (Utilities|FlowControl|Sequence
                    (:then_0
                      (goto _label_2))
                    (:then_1
                      (Default|CallOnAttackFinished false))))
                (:OnNotifyBegin
                  ;[0.1133 0.6619 0.6823] Handle Attack Combo
                  (switch name _notifyname
                    (:ATKB
                      (Variables|AttackControl|SetCan%20Register%20Attack true)
                      (Default|CallOnAttackRegisterActive))
                    (:ATKC
                      (Variables|ComboControl|SetCan%20Chain%20Attack true)
                      (if (or (Variables|AttackControl|GetAttack%20Registerd) (Variables|AttackControl|GetAuto%20Register%20Next%20Attack))
                        (CallFunction|HandleNextAttack)))
                    (:ATKE
                      (Controls|Internal|CancelCombo))))))))))
    (else
      (Utilities|FlowControl|Sequence
        (:then_0
          ;;[0.1117 0.5677 0.3101] Get Next Attack Index
          (bind _result_2 (Math|Integer|IncrementInt (Variables|ComboControl|GetAttack%20Index))
            (:%20%20
              (if (>= _result_2 (Utilities|Array|Length (.attacksname (Variables|ComboControl|GetCurrent%20Attack%20Combo))))
                ;;[1 0.4863 0.2222] Reset combo when end attack reached, or stop attacking if auto register is enabled
                (Variables|AttackControl|SetAttacking false)
                (Variables|ComboControl|SetAttack%20Index 0)
                (Default|CallOnComboFinished)
                (if (Variables|AttackControl|GetAuto%20Register%20Next%20Attack)
                  (Variables|AttackControl|SetAuto%20Register%20Next%20Attack false)
                  (Variables|ComboControl|SetAttack%20Index -1)
                  (else
                    ;;[1 0.4863 0.2222] Cancel last attack animation on new attack
                    (Controls|CancelCurrentAttackMontage -1.0 :!label _label_3)
                    (Variables|AttackControl|SetCan%20Register%20Attack false)
                    (Variables|AttackControl|SetAttack%20Registerd false)
                    (Default|AddCurrentStat (Variables|/Game/GeneralCombat/Blueprints/Pawns/BP_DefaultCombatCharacter.BP_DefaultCombatCharacter_C|GetCombat%20Unit _out_character) (Class|BFLCombatResource|MultFloat (Access|GetNextAttackCost) -1.0) _out_character)))
                (else
                  (goto _label_3))))))
        (:then_1
          (if (> (Variables|ComboControl|GetAttack%20Index) 0)
            (if (Variables|AttackControl|GetAttacking)
              (Utilities|FlowControl|Sequence :!label _label_4
                (:then_0
                  ;;[1 0.4863 0.2222] Initiate Attack
                  (Development|PrintString (Utilities|String|ToString(Boolean) (Variables|ComboControl|GetCan%20Chain%20Attack)))
                  (Variables|ComboControl|SetCan%20Chain%20Attack false)
                  (Variables|AttackControl|SetAttacking true)
                  (Default|CallOnAttackInitiated (Access|GetCurrentAttackActionData))
                  (Utilities|Time|ClearandInvalidateTimerbyHandle (Variables|ComboControl|GetReset%20Combo%20Timer)))
                (:then_1
                  (Controls|Internal|StartMotionWarping)
                  (bind _output_get_2 (Variables|ComboControl|SetCurrent%20Attack%20Montage (Access|Internal|GetAttackMontageatIndex (Variables|ComboControl|GetCurrent%20Attack%20Combo) (Variables|ComboControl|GetAttack%20Index))))
                  (bind _notifyname_2 (Animation|Montage|PlayMontage (Variables|References|GetAnimated%20Mesh) _output_get_2)
                    (:then
                      (Utilities|FlowControl|DelayUntilNextTick)
                      (Variables|AttackControl|SetIn%20Attack%20Animation true))
                    (:OnBlendOut
                      (Utilities|FlowControl|Sequence
                        (:then_0
                          (Variables|AttackControl|SetCan%20Register%20Attack true :!label _label_5)
                          (Variables|AttackControl|SetIn%20Attack%20Animation false)
                          (Variables|AttackControl|SetAttack%20Registerd false)
                          (Controls|Internal|StopMotionWarping))
                        (:then_1
                          (Default|CallOnAttackFinished true))))
                    (:OnInterrupted
                      (Utilities|FlowControl|Sequence
                        (:then_0
                          (goto _label_5))
                        (:then_1
                          (Default|CallOnAttackFinished false)
                          (if (Variables|AttackControl|GetDiscard%20Combo%20On%20Canceled)
                            _))))
                    (:OnNotifyBegin
                      ;;[0.1133 0.6619 0.6823] Handle Attack Combo
                      (switch name _notifyname_2
                        (:ATKB
                          (Variables|AttackControl|SetCan%20Register%20Attack true)
                          (Default|CallOnAttackRegisterActive))
                        (:ATKC
                          (Variables|ComboControl|SetCan%20Chain%20Attack true)
                          (if (or (Variables|AttackControl|GetAttack%20Registerd) (Variables|AttackControl|GetAuto%20Register%20Next%20Attack))
                            (CallFunction|HandleNextAttack)))
                        (:ATKE
                          (Controls|Internal|CancelCombo))))))))
            (else
              (goto _label_4))))))))

(fn InitializeComponent
  (params (Animated%20Mesh :type Skeletal%20Mesh%20Component%20Object%20Reference))
  (if (not (Variables|General|GetInitialized))
    (Utilities|FlowControl|Sequence
      (:then_0
        (Utilities|FlowControl|Sequence
          (:then_0
            (Variables|References|SetAnimated%20Mesh Animated%20Mesh))
          (:then_1
            (bind _output_get (Variables|References|SetMotion%20Warping%20Comp (Actor|GetComponentbyClass (Components|GetOwner) "/Script/MotionWarping.MotionWarpingComponent")))
            (Utilities|IsValid _output_get
              (:Is%20Not%20Valid
                (bind _returnvalue (Game|AddComponentbyClass (Components|GetOwner) "/Script/MotionWarping.MotionWarpingComponent"))
                (Variables|References|SetMotion%20Warping%20Comp _returnvalue))))
          (:then_2
            (Variables|References|SetAdvanced%20Movement%20Component (Actor|GetComponentbyClass (Components|GetOwner) "/Game/GeneralCombat/Blueprints/Components/BPC_AdvancedCharacterMovementHandler.BPC_AdvancedCharacterMovementHandler_C")))
          (:then_3
            (bind _aspawn (Utilities|Casting|CastToPawn (Components|GetOwner)))
            (Variables|References|SetOwner%20Pawn _aspawn))))
      (:then_1
        (Variables|General|SetInitialized (and (Utilities|IsValid (Variables|References|GetAnimated%20Mesh)) (Utilities|IsValid (Variables|References|GetOwner%20Pawn))))))))

(fn GetAttackMontageatIndex
  (params (Attack%20Combo :type S%20Attack%20Combo%20Data%20Structure) (Attack%20Index :type Integer))
  (if (Utilities|Array|IsValidIndex (.attacksname Attack%20Combo) Attack%20Index)
    (return (.Animation (Utilities|Struct|BreakS_AttackActionData (Access|Internal|GetAttackActionwithData (Utilities|Array|Get(acopy) (.attacksname Attack%20Combo) Attack%20Index)))))))

(fn TryRegisterAttack
  (params (Register%20All :type Boolean))
  (Variables|AttackControl|SetAuto%20Register%20Next%20Attack Register%20All)
  (if (and (Variables|AttackControl|GetCan%20Register%20Attack) (not (Variables|AttackControl|GetAttack%20Registerd)))
    (Variables|AttackControl|SetAttack%20Registerd true)
    (Utilities|FlowControl|Sequence
      (:then_0
        (if (or (not (Variables|AttackControl|GetAttacking)) (Variables|ComboControl|GetCan%20Chain%20Attack))
          (CallFunction|HandleNextAttack)))
      (:then_1
        (return true)))
    (else
      (return false))))

(fn AssignNewMoveSet
  (params (Move%20Set%20Data :type S%20Move%20Set%20Data%20Structure))
  (Utilities|FlowControl|Sequence
    (:then_0
      (Variables|ComboControl|SetAttack%20Index -1)
      (Utilities|Array|Clear (Variables|ComboControl|GetAttack%20Move%20Set))
      (Variables|ComboControl|SetCurrent%20Attack%20Combo ""))
    (:then_1
      (for _array_element (.CombosName (Utilities|Struct|BreakS_MoveSetData Move%20Set%20Data))
        (bind _returnvalue (Utilities|GetDataTableRow "/Game/Developers/Admin/Data/DataTables/GeneralCombat/DT_AttackComboData.DT_AttackComboData" _array_element)
          (:then
            (Utilities|Array|Add (Variables|ComboControl|GetAttack%20Move%20Set) _returnvalue)))))))

(fn CancelCurrentAttackMontage
  (params (Combo%20Reset%20Delay :type Float%20%28double-precision%29))
  (bind _returnvalue (Components|GetOwner))
  (Utilities|FlowControl|Sequence
    (:then_0
      (Animation|Montage|MontageStop (Components|SkeletalMesh|GetAnimInstance (Variables|References|GetAnimated%20Mesh)) 0.5 (Variables|ComboControl|GetCurrent%20Attack%20Montage))
      (Variables|AttackControl|SetCan%20Register%20Attack true)
      (Variables|AttackControl|SetAttack%20Registerd false)
      (bind _teamnumber (Class|BPIDamageSystem|GetTeamNumber(Message) _returnvalue))
      (if (or (== _teamnumber 2) (Actor|ActorHasTag _returnvalue "Legion"))
        (Variables|ComboControl|SetCan%20Chain%20Attack false)
        (Variables|AttackControl|SetAttacking false)))
    (:then_1
      (if (>= Combo%20Reset%20Delay 0.0)
        (bind _returnvalue_2 (Utilities|Time|SetTimerbyEvent (EventDispatchers|CreateEvent :!event CancelCombo) Combo%20Reset%20Delay))
        (Variables|ComboControl|SetReset%20Combo%20Timer _returnvalue_2)))))

(fn IsValidCombo
  (params (Combo%20Data :type S%20Attack%20Combo%20Data%20Structure))
  (return (> (Utilities|Array|Length (.AttacksName (Utilities|Struct|BreakS_AttackComboData Combo%20Data))) 0)))

(fn GetAttackActionwithData
  (params (Data :type Data%20Table%20Row%20Handle%20Structure))
  (Utilities|IsValid (.datatable Data)
    (:Is%20Valid
      (bind _returnvalue (Utilities|GetDataTableRow (.datatable Data) (.rowname Data))
        (:then
          (return _returnvalue))))))

(fn GetAttackState
  (return (Variables|AttackControl|GetAttacking) (Variables|AttackControl|GetIn%20Attack%20Animation)))

(fn SetCurrentAttackCombo
  (params (Combo%20Data :type S%20Attack%20Combo%20Data%20Structure))
  (if (not (Utility|IdenticalComboData Combo%20Data (Variables|ComboControl|GetCurrent%20Attack%20Combo)))
    (Variables|ComboControl|SetAttack%20Index -1)
    (Variables|ComboControl|SetCurrent%20Attack%20Combo Combo%20Data)))

(fn GetCurrentAttackActionData
  (return (Access|Internal|GetAttackActionwithData (Utilities|Array|Get(acopy) (Utilities|Struct|BreakS_AttackComboData (Variables|ComboControl|GetCurrent%20Attack%20Combo)) (Variables|ComboControl|GetAttack%20Index)))))

(fn IdenticalComboData
  (params (A :type S%20Attack%20Combo%20Data%20Structure) (B :type S%20Attack%20Combo%20Data%20Structure))
  (return (Utilities|Array|Identical (Utilities|Struct|BreakS_AttackComboData A) (Utilities|Struct|BreakS_AttackComboData B))))

(fn GetNextAttackCost
  (bind _current_attack_combo (Variables|ComboControl|GetCurrent%20Attack%20Combo))
  (bind _attacksname (Utilities|Struct|BreakS_AttackComboData _current_attack_combo))
  (if (Utility|IsValidCombo (Variables|ComboControl|GetCurrent%20Attack%20Combo))
    (return (.Cost (Utilities|Struct|BreakS_AttackActionData (Access|Internal|GetAttackActionwithData (Utilities|Array|Get(acopy) _attacksname (Math|Integer|%(Integer) (+ (Variables|ComboControl|GetAttack%20Index) 1) (Utilities|Array|Length _attacksname)))))))))

(fn CancelCombo
  (Utilities|FlowControl|Sequence
    (:then_0
      (Variables|AttackControl|SetCan%20Register%20Attack true)
      (Variables|AttackControl|SetAttack%20Registerd false)
      (Variables|ComboControl|SetCan%20Chain%20Attack false)
      (Variables|AttackControl|SetAttacking false))
    (:then_1
      (if (== (Variables|ComboControl|GetAttack%20Index) (- (Utilities|Array|Length (.attacksname (Variables|ComboControl|GetCurrent%20Attack%20Combo))) 1))
        (Default|CallOnComboFinished)
        (else
          (Default|CallOnComboInterrupted))))
    (:then_2
      (Variables|ComboControl|SetAttack%20Index -1) ; Reset combo counter if reached end of attack
    )))

(fn MotionWarpingInnerHandling
  (bind _returnvalue (Components|GetOwner))
  (bind _attack_data (Access|GetCurrentAttackActionData))
  (bind _returnvalue_2 (Components|GetOwner))
  (bind _returnvalue_3 (Components|GetOwner))
  (bind (_maxrange _minrange) (Utilities|Struct|BreakS_AttackActionData _attack_data))
  (bind _returnvalue_4 (Transformation|GetActorRotation _returnvalue_2))
  (bind _returnvalue_5 (Transformation|GetActorRotation _returnvalue_3))
  (bind _returnvalue_6 (Transformation|GetActorLocation _returnvalue_3))
  (if (or (Actor|ActorHasTag _returnvalue "Enemy") (Actor|ActorHasTag _returnvalue "Legion"))
    (if (CallFunction|CanMotionWarping (Variables|MotionWarping|GetS%20Motion%20Warp%20Data))
      (Class|MotionWarpingComponent|AddorUpdateWarpTargetfromLocationandRotation (Variables|References|GetMotion%20Warping%20Comp) "MW" (+ (* (Math|Vector|Normalize (- (Transformation|GetActorLocation (Components|GetOwner)) (Transformation|GetActorLocation (Access|GetFocusTarget)))) (Utilities|Struct|BreakS_MotionWarpData (Variables|MotionWarping|GetS%20Motion%20Warp%20Data))) (Transformation|GetActorLocation (Access|GetFocusTarget))) (Math|Rotator|MakeRotator (.roll _returnvalue_4) (.pitch _returnvalue_4) (.yaw (Math|Rotator|FindLookatRotation (Transformation|GetActorLocation _returnvalue_2) (Transformation|GetActorLocation (Access|GetFocusTarget))))))
      (else
        (Utilities|IsValid (Access|GetFocusTarget)
          (:Is%20Valid
            (Class|MotionWarpingComponent|AddorUpdateWarpTargetfromLocationandRotation (Variables|References|GetMotion%20Warping%20Comp) "MW" _returnvalue_6 (Math|Rotator|MakeRotator (.roll _returnvalue_5) (.pitch _returnvalue_5) (.yaw (Math|Rotator|FindLookatRotation _returnvalue_6 (Transformation|GetActorLocation (Access|GetFocusTarget)))))))
          (:Is%20Not%20Valid
            (Controls|Internal|StopMotionWarping)))))
    (elif (Utilities|IsValid (Variables|MotionWarping|GetFocus%20Target))
      (bind (_out_vector _returnvalue_7) (|GetLockOnTargetLocation&Rotation))
      (Class|MotionWarpingComponent|AddorUpdateWarpTargetfromLocationandRotation (Variables|References|GetMotion%20Warping%20Comp) "MW" _out_vector _returnvalue_7)
      (else
        (bind _returnvalue_8 (|GetMoveInputRotation))
        (if (< (Transformation|GetDistanceTo (Components|GetOwner) (Variables|MotionWarping|GetFocus%20Target)) _maxrange)
          (Class|MotionWarpingComponent|AddorUpdateWarpTargetfromLocationandRotation (Variables|References|GetMotion%20Warping%20Comp) "MW" (+ (* (Math|Vector|GetForwardVector _returnvalue_8) (- _maxrange _minrange)) (Variables|MotionWarping|GetInitial%20Motion%20Warp%20Location)) _returnvalue_8))))))

(fn SetFocusTarget
  (params (New%20Target :type Actor%20Object%20Reference))
  (if (!= New%20Target (Variables|MotionWarping|GetFocus%20Target))
    (bind _output_get (Variables|MotionWarping|SetFocus%20Target New%20Target))
    (Default|CallOnFocusTargetUpdated _output_get)))

(fn StartMotionWarping
  (Variables|MotionWarping|SetInitial%20Motion%20Warp%20Location (Transformation|GetActorLocation (Variables|References|GetOwner%20Pawn)))
  (Utility|MotionWarpingInnerHandling)
  (bind _returnvalue (Utilities|Time|SetTimerbyEvent (EventDispatchers|CreateEvent :!event MotionWarpingInnerHandling) (Variables|MotionWarping|GetMotion%20Warping%20Inner%20Delay) true true))
  (Variables|MotionWarping|SetMotion%20Warping%20Timer _returnvalue))

(fn StopMotionWarping
  (Utilities|Time|ClearandInvalidateTimerbyHandle (Variables|MotionWarping|GetMotion%20Warping%20Timer)))

(fn GetFocusTarget
  (bind _returnvalue (Components|GetOwner))
  (if (or (Actor|ActorHasTag _returnvalue "Enemy") (Actor|ActorHasTag _returnvalue "Legion"))
    (bind _target_actor (Class|BPIAttackable|GetAttackTarget(Message) (AI|GetAIController (Components|GetOwner))))
    (return _target_actor)
    (else
      (return (Variables|MotionWarping|GetFocus%20Target)))))

(fn CanMotionWarping
  (params (S_MotionWarpData :type S%20Motion%20Warp%20Data%20Structure%20%28by%20ref%29))
  (Utilities|IsValid (Access|GetFocusTarget)
    (:Is%20Valid
      (if (<= (Transformation|GetDistanceTo (Components|GetOwner) (Access|GetFocusTarget)) (Utilities|Struct|BreakS_MotionWarpData S_MotionWarpData))
        (if (<= (CallFunction|FlatAngle(Vector) (Transformation|GetActorForwardVector (Components|GetOwner)) (- (Transformation|GetActorLocation (Access|GetFocusTarget)) (Transformation|GetActorLocation (Components|GetOwner)))) (Utilities|Struct|BreakS_MotionWarpData S_MotionWarpData))
          (return true)
          (else
            (return false)))
        (else
          (return false))))))