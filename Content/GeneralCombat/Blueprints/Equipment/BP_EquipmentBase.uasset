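; Base Blueprint for combat equipment, built around an EquipmentData struct that also sets its static mesh at construction.
; Getters use row names from that struct to look up weapon combat data and separate physic and spirit attack combos in data tables.
; Equip and Unequip only call OnEquipped and OnUnequipped, which are empty here.
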(fn ConstructionScript
  (Components|StaticMesh|SetStaticMesh (Variables|Default|GetStaticMesh) (.mesh (Variables|Data|GetEquipment%20Data))))

(fn GetEquipmentData
  (return (Variables|Data|GetEquipment%20Data)))

(fn GetCombatData
  (bind _returnvalue (Utilities|GetDataTableRow "/Game/Developers/Admin/Data/DataTables/Player/Weapon/DT_WeaponCombatData.DT_WeaponCombatData" (.EquipmentCombatDataName (Utilities|Struct|BreakS_EquipmentData (Variables|Data|GetEquipment%20Data))))
    (:then
      (return _returnvalue))))

(fn GetPhysicComboData
  (bind _returnvalue (Utilities|GetDataTableRow "/Game/Developers/Admin/Data/DataTables/GeneralCombat/DT_AttackComboData.DT_AttackComboData" (.PhysicComboName (Utilities|Struct|BreakS_EquipmentData (Variables|Data|GetEquipment%20Data))))
    (:then
      (return _returnvalue))))

(fn GetSpiritComboData
  (bind _returnvalue (Utilities|GetDataTableRow "/Game/Developers/Admin/Data/DataTables/GeneralCombat/DT_AttackComboData.DT_AttackComboData" (.SpiritComboName (Utilities|Struct|BreakS_EquipmentData (Variables|Data|GetEquipment%20Data))))
    (:then
      (return _returnvalue))))

(fn OnEquipped)

(fn OnUnequipped)

(fn Equip
  (Abstract|OnEquipped))

(fn Unequip
  (Abstract|OnUnequipped))