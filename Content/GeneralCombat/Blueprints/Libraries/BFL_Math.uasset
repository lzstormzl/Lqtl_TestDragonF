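; Blueprint function library of math helpers for the general combat system, covering directions, vectors and angles, bitflags, camera frame size, socket and hitbox transforms, and diminishing returns.
; Direction lookups pick the 4- or 8-way enum with the highest dot product; unnormalized diagonals bias the 8-way result away from cardinals.
; AI decision scoring remaps a tracked value through a curve and multiplier, sampling the curve at -1 when below minimum.
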(fn GetClosestDirectionfromVector2D
  (params (Zero%20Direction :type E_Direction2D%20Enum :default "NewEnumerator8") (In%20Vector2D :type Vector%202D%20Structure))
  (Utilities|FlowControl|Sequence
    (:then_0
      (if (Utilities|Operators|EqualEqual :A In%20Vector2D :ErrorTolerance 0.01)
        (return Zero%20Direction)))
    (:then_1
      (bind _output_get (LocalVariables|SetNormalized%20Vector%202D (Math|Vector2D|Normalize2D In%20Vector2D)))
      (LocalVariables|SetMax%20Dot (Math|Vector2D|DotProduct(2D) :A _output_get)))
    (:then_2
      (for (_array_element _array_index) (Utilities|Array|MakeArray "(X=0.000000,Y=1.000000)" "(X=0.000000,Y=-1.000000)" "(X=-1.000000,Y=0.000000)" "(X=1.000000,Y=0.000000)" "(X=-1.000000,Y=1.000000)" "(X=1.000000,Y=1.000000)" "(X=-1.000000,Y=-1.000000)" "(X=1.000000,Y=-1.000000)")
        (bind _output_get_2 (LocalVariables|SetCurrent%20Dot (Math|Vector2D|DotProduct(2D) (LocalVariables|GetNormalized%20Vector%202D) _array_element)))
        (if (> _output_get_2 (LocalVariables|GetMax%20Dot))
          (LocalVariables|SetMax%20Dot (LocalVariables|GetCurrent%20Dot))
          (LocalVariables|SetClosest%20Direction%20Index _array_index)))
      (return (Utilities|Enum|ByteToEnumE_Direction2D (Math|Conversions|ToByte(Integer) (+ (LocalVariables|GetClosest%20Direction%20Index) 1)))))))

(fn GetClosestSimpleDirectionfromVector2D
  (params (Zero%20Direction :type E_Direction2DSimple%20Enum :default "NewEnumerator8") (In%20Vector2D :type Vector%202D%20Structure))
  (Utilities|FlowControl|Sequence
    (:then_0
      (if (Utilities|Operators|EqualEqual :A In%20Vector2D :ErrorTolerance 0.01)
        (return Zero%20Direction)))
    (:then_1
      (bind _output_get (LocalVariables|SetNormalized%20Vector%202D (Math|Vector2D|Normalize2D In%20Vector2D)))
      (LocalVariables|SetMax%20Dot (Math|Vector2D|DotProduct(2D) :A _output_get)))
    (:then_2
      (for (_array_element _array_index) (Utilities|Array|MakeArray "(X=0.000000,Y=1.000000)" "(X=0.000000,Y=-1.000000)" "(X=-1.000000,Y=0.000000)" "(X=1.000000,Y=0.000000)")
        (bind _output_get_2 (LocalVariables|SetCurrent%20Dot (Math|Vector2D|DotProduct(2D) (LocalVariables|GetNormalized%20Vector%202D) _array_element)))
        (if (> _output_get_2 (LocalVariables|GetMax%20Dot))
          (LocalVariables|SetMax%20Dot (LocalVariables|GetCurrent%20Dot))
          (LocalVariables|SetClosest%20Direction%20Index _array_index)))
      (return (Utilities|Enum|ByteToEnumE_Direction2DSimple (Math|Conversions|ToByte(Integer) (+ (LocalVariables|GetClosest%20Direction%20Index) 1)))))))

(fn GetVector2DfromDirection
  (params (Direction :type E_Direction2D%20Enum :default "NewEnumerator0") (Default%20Vector :type Vector%202D%20Structure))
  (return (Utilities|Select :Index Direction :NewEnumerator8 Default%20Vector :NewEnumerator0 "(X=0.000000,Y=1.000000)" :NewEnumerator1 "(X=0.000000,Y=-1.000000)" :NewEnumerator2 "(X=-1.000000,Y=0.000000)" :NewEnumerator3 "(X=1.000000,Y=0.000000)" :NewEnumerator4 "(X=-1.000000,Y=1.000000)" :NewEnumerator5 "(X=1.000000,Y=1.000000)" :NewEnumerator6 "(X=-1.000000,Y=-1.000000)" :NewEnumerator7 "(X=1.000000,Y=-1.000000)")))

(fn GetCameraSizeatDistance
  (params (Camera :type Camera%20Component%20Object%20Reference) (Distance :type Float%20%28double-precision%29))
  (bind _fieldofview (Variables|/Script/Engine.CameraComponent|GetFieldOfView Camera))
  (bind _returnvalue (/ _fieldofview 2.0))
  (bind _returnvalue_2 (Math|Trig|Tan(Degrees) _returnvalue))
  (bind _returnvalue_3 (* _returnvalue_2 2.0 Distance))
  (return (Math|Vector2D|MakeVector2D (* (Variables|/Script/Engine.CameraComponent|GetAspectRatio Camera) _returnvalue_3) _returnvalue_3)))

(fn FlatAngle(Vector)
  (params (Vector%20A :type Vector) (Vector%20B :type Vector))
  (return (Class|KismetMathLibrary|DegAcos (Math|Vector|DotProduct (Math|Vector|Normalize Vector%20A) (Math|Vector|Normalize Vector%20B)))))

(fn GetSocketLocationatOffset
  (params (Mesh%20Comp :type Skeletal%20Mesh%20Component%20Object%20Reference) (Socket%20Name :type Name) (Offset :type Vector))
  (return (Math|Transform|TransformLocation (Transformation|GetSocketTransform Mesh%20Comp Socket%20Name "RTS_World") Offset)))

(fn GetCapsuleRotationfromto
  (params (Start :type Vector) (End :type Vector))
  (return (Math|Rotator|MakeRotfromZ (- Start End))))

(fn Add(Flags)
  (params (A :type Integer) (B :type Integer))
  (return (Class|KismetMathLibrary|OrIntInt A B)))

(fn Remove(Flags)
  (params (A :type Integer) (B :type Integer))
  (return (Class|KismetMathLibrary|AndIntInt A (Class|KismetMathLibrary|NotInt B))))

(fn Contains(Flags)
  (params (Container%20Flags :type Integer) (Check%20Flags :type Integer) (Compare%20Type :type E_FlagCompareType%20Enum :default "NewEnumerator0"))
  (switch Utilities|FlowControl|Switch|SwitchonE_FlagCompareType Compare%20Type
    (:NewEnumerator0
      (return (!= (Class|KismetMathLibrary|AndIntInt Container%20Flags Check%20Flags) 0)))
    (:NewEnumerator1
      (return (== (Class|KismetMathLibrary|AndIntInt Container%20Flags Check%20Flags) Check%20Flags)))
    (:NewEnumerator2
      (return (== (Class|KismetMathLibrary|AndIntInt Container%20Flags (Class|KismetMathLibrary|NotInt Check%20Flags)) 0)))
    (:NewEnumerator3
      (return (== Container%20Flags Check%20Flags)))))

(fn Overlap(Flags)
  (params (A :type Integer) (B :type Integer))
  (return (Class|KismetMathLibrary|AndIntInt A B)))

(fn GetHitboxWorldHitDirection
  (params (Mesh%20Comp :type Skeletal%20Mesh%20Component%20Object%20Reference) (Hitbox%20Data :type S%20Hitbox%20Data%20Structure))
  (bind (_startsocket _hitdirection) (Utilities|Struct|BreakS_HitboxData Hitbox%20Data))
  (return (Math|Vector|Normalize (Math|Transform|TransformDirection (Transformation|GetSocketTransform Mesh%20Comp _startsocket "RTS_World") _hitdirection))))

(fn GetCloserVector
  (params (Origin :type Vector) (A :type Vector) (B :type Vector))
  (return (Math|Vector|SelectVector A B (< (Class|KismetMathLibrary|VectorDistanceSquared Origin A) (Class|KismetMathLibrary|VectorDistanceSquared Origin B)))))

(fn GetFurtherVector
  (params (Origin :type Vector) (A :type Vector) (B :type Vector))
  (return (Math|Vector|SelectVector A B (> (Class|KismetMathLibrary|VectorDistanceSquared Origin A) (Class|KismetMathLibrary|VectorDistanceSquared Origin B)))))

(fn GetDiminishingReturnsOfIndex
  (params (Index :type Integer) (Diminish%20Per%20Index :type Float%20%28double-precision%29) (Min%20Value :type Float%20%28double-precision%29))
  (return (Math|Float|Max(Float) (Math|Float|Power Diminish%20Per%20Index (Math|Conversions|ToFloat(Integer) Index)) Min%20Value)))

(fn EvaluateAIWeightedDecision
  (params (Data :type S%20Weighted%20Decision%20Data%20Structure) (Tracked%20Value :type Float%20%28double-precision%29))
  (bind (_mult _evaluationcurve _min _max) (Utilities|Struct|BreakS_WeightedDecisionData Data))
  (Utilities|IsValid _evaluationcurve
    (:Is%20Valid
      (if (< Tracked%20Value _min)
        (return (Math|Curves|GetFloatValue _evaluationcurve -1.0))
        (else
          (return (* _mult (Math|Curves|GetFloatValue _evaluationcurve (Math|Float|Clamp(Float) (/ (- Tracked%20Value _min) (- _max _min)))))))))))

(fn SignedFlatAngle(Vector2D)
  (params (Vector%20A :type Vector%202D%20Structure) (Vector%20B :type Vector%202D%20Structure))
  (bind _returnvalue (Math|Vector2D|Normalize2D Vector%20B))
  (bind _returnvalue_2 (Math|Vector2D|Normalize2D Vector%20A))
  (return (Class|KismetMathLibrary|DegAtan2 (Class|KismetMathLibrary|CrossProduct2D _returnvalue_2 _returnvalue) (Math|Vector2D|DotProduct(2D) _returnvalue_2 _returnvalue))))