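; BP_PlayerDecoy is a decoy actor that detects perfect dodges by taking hits at a given location.
; Enabling it moves it there, turns on query-only capsule collision and starts a timer spanning the dodge window.
; A hit without the excluded attack flags disables collision and, if inside the window, triggers a perfect dodge.
; The perfect dodge notifies via a call, then briefly shows a PoseableMesh afterimage copying the target skeletal mesh's pose.
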(event Custom|Event%20Perfect%20Dodge
  (Default|CallOnPerfectDodge)
  (Utilities|FlowControl|Delay 0.05)
  (Utilities|IsValid (Variables|Default|GetTarget%20Skeletal%20Mesh)
    (:Is%20Valid
      (Utilities|FlowControl|Sequence
        (:then_0
          (Transformation|SetWorldLocation (Variables|Default|GetPoseableMesh) (Transformation|GetWorldLocation (Variables|Default|GetTarget%20Skeletal%20Mesh)) false true)
          (Transformation|SetWorldRotation (Variables|Default|GetPoseableMesh) (Transformation|GetWorldRotation (Variables|Default|GetTarget%20Skeletal%20Mesh)) false false))
        (:then_1
          (Class|PoseableMeshComponent|CopyPosefromSkeletalComponent (Variables|Default|GetPoseableMesh) (Variables|Default|GetTarget%20Skeletal%20Mesh))
          (Rendering|SetVisibility (Variables|Default|GetPoseableMesh) true true))
        (:then_2
          (Utilities|FlowControl|Delay (Variables|Default|GetShow%20Duration))
          (CallFunction|DisableDecoy))))))

(event EventBeginPlay
  (Rendering|SetVisibility (Variables|Default|GetPoseableMesh) false true)
  (Collision|SetCollisionEnabled (Variables|Default|GetCapsule) "NoCollision"))

(event EventOnDamaged
  (params (Source%20Attack :type S%20Attack%20Data%20Structure) (Initigator :type Actor%20Object%20Reference) (Hit%20Direction :type Vector :default "0, 0, 0"))
  (if (not (CallFunction|Contains(Flags) (.attackFlags (Utilities|Struct|BreakS_AttackData Source%20Attack)) (|BitmaskLiteral 20) "NewEnumerator0"))
    (Collision|SetCollisionEnabled (Variables|Default|GetCapsule) "NoCollision")
    (if (<= (- (Utilities|Time|GetGameTimeinSeconds) (Variables|Default|GetStart%20Dodge%20Time)) (Variables|Default|GetPerfect%20Dodge%20Window))
      (CallFunction|EventPerfectDodge))))

(fn ConstructionScript)

(fn EnableDecoy
  (params (Location :type Vector))
  (Transformation|SetActorLocation Location false true)
  (Collision|SetCollisionEnabled (Variables|Default|GetCapsule) "QueryOnly")
  (Variables|Default|SetStart%20Dodge%20Time (Utilities|Time|GetGameTimeinSeconds))
  (Utilities|Time|ClearandInvalidateTimerbyHandle (Variables|Default|GetDisable%20Decoy%20Timer%20Handle))
  (bind _returnvalue (Utilities|Time|SetTimerbyEvent (EventDispatchers|CreateEvent :!event DisableDecoyCollision) (Variables|Default|GetPerfect%20Dodge%20Window)))
  (Variables|Default|SetDisable%20Decoy%20Timer%20Handle _returnvalue))

(fn DisableDecoy
  (CallFunction|DisableDecoyCollision)
  (Rendering|SetVisibility (Variables|Default|GetPoseableMesh) false true))

(fn DisableDecoyCollision
  (Collision|SetCollisionEnabled (Variables|Default|GetCapsule) "NoCollision"))