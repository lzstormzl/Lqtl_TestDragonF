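; Actor pool component that pre-spawns PoolSize actors of PoolActorClass on BeginPlay and stores them as not in use, in a projectile weapon folder.
; SpawnFromPool moves the first pooled actor to the given transform, activates it and removes it, then returns index 0 as read after removal.
; An empty pool triggers a batch refill without returning an actor.
; Nothing here puts used actors back into the pool.
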(event Custom|Spawn%20Actor%20Into%20Pool
  (for _index (range 0 (- (Variables|Default|GetPool%20size) 1))
    (bind _returnvalue (Game|SpawnActorfromClass (Variables|Default|GetPool%20Actor%20Class) (Math|Transform|MakeTransform "0, 0, 0" "0, 0, 0" "1.000000,1.000000,1.000000") "Undefined" "MultiplyWithRoot" 0 1e+01 0))
    (Utilities|Array|AddUnique (Variables|Default|GetObject%20Pool) _returnvalue)
    (Default|SetinUse _returnvalue false)))

(event EventBeginPlay
  (CallFunction|SpawnActorIntoPool))

(fn SpawnfromPool
  (params (SpawnTranform :type Transform))
  (bind _object_pool (Variables|Default|GetObject%20Pool))
  (bind _output (Utilities|Array|Get(acopy) _object_pool))
  (if (>= (Utilities|Array|Length _object_pool) 1)
    (Transformation|SetActorTransform _output SpawnTranform)
    (Default|SetinUse _output true)
    (Utilities|Array|RemoveItem (Variables|Default|GetObject%20Pool) _output)
    (return _output)
    (else
      (CallFunction|SpawnActorIntoPool))))