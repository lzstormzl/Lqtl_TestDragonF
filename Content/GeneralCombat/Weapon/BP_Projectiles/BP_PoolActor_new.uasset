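; BP_PoolActor_new is a poolable actor that switches between active and dormant states, starting dormant on BeginPlay.
; SetInUse toggles collision, visibility and tick together instead of spawning or destroying the actor.
; On activation it restarts a time-to-live timer, whose ReturnPool event sets the actor back to unused when it expires.
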(event Custom|Set%20in%20Use
  (params (InUse :type Boolean))
  (Variables|Default|SetInUse InUse)
  (Collision|SetActorEnableCollision InUse)
  (Rendering|SetActorHiddenInGame (not InUse))
  (Actor|Tick|SetActorTickEnabled InUse)
  (if InUse
    (Utilities|Time|ClearandInvalidateTimerbyHandle (Variables|Default|GetTime%20to%20live%20timer))
    (bind _returnvalue (Utilities|Time|SetTimerbyEvent (delegate Custom|Return%20Pool) (Variables|Default|GetTimetolive)))
    (Variables|Default|SetTime%20to%20live%20timer _returnvalue)))

(event Custom|Return%20Pool
  (CallFunction|SetinUse self false))

(event EventBeginPlay
  (CallFunction|SetinUse false))

(fn ConstructionScript)