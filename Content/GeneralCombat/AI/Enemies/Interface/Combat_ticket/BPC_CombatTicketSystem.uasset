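; Actor component that limits enemy AI attacks through a combat ticket system with separate melee and ranged token pools.
; Reserve functions deduct the requested amount when enough tokens remain and return whether they succeeded.
; Return functions add tokens back to their pool without any upper clamp.
; It runs no event logic, so all changes come from callers of these functions.
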(event EventBeginPlay)

(event EventTick
  (params (DeltaSeconds :type Float%20%28single-precision%29)))

(fn ReserveAttackTokenMelee
  (params (Amount%20Melee :type Integer))
  (if (>= (Variables|Combatticket|GetAttackTokensCount_Melee) Amount%20Melee)
    (Variables|Combatticket|SetAttackTokensCount_Melee (- (Variables|Combatticket|GetAttackTokensCount_Melee) Amount%20Melee))
    (return true)
    (else
      (return false))))

(fn ReturnAttackTokenMelee
  (params (Amount%20Melee :type Integer))
  (Variables|Combatticket|SetAttackTokensCount_Melee (+ Amount%20Melee (Variables|Combatticket|GetAttackTokensCount_Melee))))

(fn ReserveAttackTokenRange
  (params (Amount%20Range :type Integer))
  (if (>= (Variables|Combatticket|GetAttackTokensCount_Range) Amount%20Range)
    (Variables|Combatticket|SetAttackTokensCount_Range (- (Variables|Combatticket|GetAttackTokensCount_Range) Amount%20Range))
    (return true)
    (else
      (return false))))

(fn ReturnAttackTokenRange
  (params (Amount%20Range :type Integer))
  (Variables|Combatticket|SetAttackTokensCount_Range (+ Amount%20Range (Variables|Combatticket|GetAttackTokensCount_Range))))