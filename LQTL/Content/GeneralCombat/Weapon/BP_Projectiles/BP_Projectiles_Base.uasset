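; Base projectile Blueprint for combat weapons that can be switched in and out of use, apparently for pooling.
; The construction script applies Speed and Gravity to the ProjectileMovement component.
; SetinUse extends the parent logic, launching the projectile along its forward vector or zeroing its velocity.
; A HitBox hit calls OnProjectileHit, spawns impact effects and sound, then takes the projectile out of use instead of destroying it.
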(event OnComponentHit(HitBox)
  (params (HitComponent :type Primitive%20Component%20Object%20Reference) (OtherActor :type Actor%20Object%20Reference) (OtherComp :type Primitive%20Component%20Object%20Reference) (NormalImpulse :type Vector :default "0, 0, 0") (Hit :type Hit%20Result%20Structure%20%28by%20ref%29))
  (bind _location (Collision|BreakHitResult Hit))
  (Default|CallOnProjectileHit OtherActor Hit)
  (Effects|SpawnEmitteratLocation 0 _location)
  (Audio|PlaySoundatLocation (Variables|Sound|GetImpact%20Sound) _location "0, 0, 0" 1.0 1.0 0.0 0 0 0 0)
  (CallFunction|SetinUse false))

(event EventSetinUse
  (params (InUse :type Boolean))
  (|CallParentFunction InUse)
  (if InUse
    (Variables|/Script/Engine.MovementComponent|SetVelocity (Variables|Default|GetProjectileMovement) (* (Transformation|GetActorForwardVector) (Variables|ProjectilesSetting|GetSpeed)))
    (else
      (Variables|/Script/Engine.MovementComponent|SetVelocity (Variables|Default|GetProjectileMovement) "0, 0, 0"))))

(fn ConstructionScript
  (bind _projectilemovement (Variables|Default|GetProjectileMovement))
  (Variables|/Script/Engine.ProjectileMovementComponent|SetInitialSpeed _projectilemovement (Variables|ProjectilesSetting|GetSpeed))
  (Variables|/Script/Engine.ProjectileMovementComponent|SetMaxSpeed _projectilemovement (Variables|ProjectilesSetting|GetSpeed))
  (Variables|/Script/Engine.ProjectileMovementComponent|SetProjectileGravityScale _projectilemovement (Variables|ProjectilesSetting|GetGravity)))