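; Arrow projectile for combat that launches along its forward vector at Speed through ProjectileMovement.
; On a Hitbox hit, it checks the HitComponent's owner for the Enemy tag and sends that actor OnDamaged with the player character as initiator.
; Damage is a hardcoded base, plus a bonus when the player's BPCBlessing has a specific active effect.
; The arrow's own location is passed as HitDirection, and nothing here destroys it.
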(event OnComponentHit(Hitbox)
  (params (HitComponent :type Primitive%20Component%20Object%20Reference) (OtherActor :type Actor%20Object%20Reference) (OtherComp :type Primitive%20Component%20Object%20Reference) (NormalImpulse :type Vector :default "0, 0, 0") (Hit :type Hit%20Result%20Structure%20%28by%20ref%29))
  (bind _returnvalue (Components|GetOwner HitComponent))
  (if (Actor|ActorHasTag _returnvalue "Enemy")
    (if (Utilities|Map|Contains (Variables|/Game/ThirdPerson/BPC_Blessing.BPC_Blessing_C|GetActivating%20Effects (Variables|/Game/GeneralCombat/Blueprints/Pawns/BP_DefaultCombatCharacter.BP_DefaultCombatCharacter_C|GetBPC_Blessing (.Out%20Character (CallFunction|GetPlayerCombatCharacter)))) "NewEnumerator0")
      (Class|BPIDamagable|OnDamaged(Message) _returnvalue (Utilities|Struct|MakeS_AttackData (Utilities|Struct|MakeS_CombatResource (+ 8e+02 4e+02)) "(shield=0.000000,health=0.000000,spiritWater=0.000000,spiritOrb=0.000000,stagger=0.000000)" "None") (.Out%20Character (CallFunction|GetPlayerCombatCharacter)) (Transformation|GetActorLocation))
      (else
        (Class|BPIDamagable|OnDamaged(Message) _returnvalue (Utilities|Struct|MakeS_AttackData (Utilities|Struct|MakeS_CombatResource (+ 8e+02 0.0)) "(shield=0.000000,health=0.000000,spiritWater=0.000000,spiritOrb=0.000000,stagger=0.000000)" "None") (.Out%20Character (CallFunction|GetPlayerCombatCharacter)) (Transformation|GetActorLocation))))))

(event EventBeginPlay
  (Variables|/Script/Engine.MovementComponent|SetVelocity (Variables|Default|GetProjectileMovement) (* (Transformation|GetActorForwardVector) (Variables|Default|GetSpeed))))

(fn ConstructionScript)