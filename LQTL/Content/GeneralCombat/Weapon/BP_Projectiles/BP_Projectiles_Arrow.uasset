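; Arrow projectile Blueprint that sends a fixed-damage message when its HitBox begins an overlap.
; The message targets the owner of OverlappedComponent, which is the arrow's own HitBox rather than the other actor.
; It passes the arrow's forward vector as hit direction and always credits player character 0 as initiator.
; SetinUse only defers to the parent class, and Tick and actor overlap are disabled.
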(event OnComponentBeginOverlap(HitBox)
  (params (OverlappedComponent :type Primitive%20Component%20Object%20Reference) (OtherActor :type Actor%20Object%20Reference) (OtherComp :type Primitive%20Component%20Object%20Reference) (OtherBodyIndex :type Integer) (bFromSweep :type Boolean) (SweepResult :type Hit%20Result%20Structure%20%28by%20ref%29))
  (Class|BPIDamagable|OnDamaged(Message) (Components|GetOwner OverlappedComponent) (Utilities|Struct|MakeS_AttackData (Utilities|Struct|MakeS_CombatResource 0.0 3e+01 0.0 0.0 0.0) "(shield=0.000000,health=0.000000,spiritWater=0.000000,spiritOrb=0.000000,stagger=0.000000)" "None" 0) (Game|GetPlayerCharacter 0) (Transformation|GetActorForwardVector)))

(event Collision|EventActorBeginOverlap
  (params (OtherActor :type Actor%20Object%20Reference))
  (|CallParentFunction OtherActor) ; This node is disabled and will not be called.\nDrag off pins to build functionality.
)

(event EventTick
  (params (DeltaSeconds :type Float%20%28single-precision%29))
  (|CallParentFunction DeltaSeconds) ; This node is disabled and will not be called.\nDrag off pins to build functionality.
)

(event EventSetinUse
  (params (InUse :type Boolean))
  (|CallParentFunction InUse))

(fn ConstructionScript
  (|CallParentFunction))