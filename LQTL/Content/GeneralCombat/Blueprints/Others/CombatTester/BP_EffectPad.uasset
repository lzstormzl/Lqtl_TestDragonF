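; BP_EffectPad is a combat-tester pad meant to apply a repeating attack effect to tracked actors.
; EffectCountdown accumulates delta time and, at each loop interval, sends OnDamagedMessage with AttackEffect and zero hit direction to every AffectActors key.
; It also feeds loop progress to a countdown widget.
; BeginPlay and box overlap are empty, and the file shows neither a caller for the countdown nor code filling AffectActors.
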(event EventBeginPlay)

(event OnComponentBeginOverlap(Box)
  (params (OverlappedComponent :type Primitive%20Component%20Object%20Reference) (OtherActor :type Actor%20Object%20Reference) (OtherComp :type Primitive%20Component%20Object%20Reference) (OtherBodyIndex :type Integer) (bFromSweep :type Boolean) (SweepResult :type Hit%20Result%20Structure%20%28by%20ref%29)))

(fn ConstructionScript)

(fn EffectCountdown
  (bind _output_get (Variables|Data|SetElapsed%20Time (+ (Variables|Data|GetElapsed%20Time) (Utilities|Time|GetWorldDeltaSeconds))))
  (Utilities|FlowControl|Sequence
    (:then_0
      (if (>= _output_get (Variables|Effect|GetSeconds%20Per%20Loop))
        (Variables|Data|SetElapsed%20Time 0.0)
        (bind _keys (Utilities|Map|Keys (Variables|Data|GetAffect%20Actors)))
        (for _array_element _keys
          (Class|BPIDamagable|OnDamaged(Message) _array_element (Variables|Effect|GetAttack%20Effect) 0 "0, 0, 0"))))
    (:then_1
      (Default|SetValue (Variables|Components|GetCountdown%20Widget) (/ (Variables|Data|GetElapsed%20Time) (Variables|Effect|GetSeconds%20Per%20Loop))))))