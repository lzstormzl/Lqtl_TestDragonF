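; A combat test pad that periodically hits every actor inside its box with a configurable attack effect.
; Box overlap events keep a per-actor overlap count, so actors stay affected until their last overlapping component leaves.
; A near-zero looping timer, capped at once per frame, appears to drive EffectCountdown, which sends OnDamagedMessage each interval with a direction outward from the box.
; A widget progress bar displays the countdown.
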(event EventBeginPlay
  (Utilities|Time|SetTimerbyEvent (EventDispatchers|CreateEvent :!event EffectCountdown) 0.0001 true true)
  (bind _returnvalue (UserInterface|CreateWidget "/Game/GeneralCombat/Blueprints/Widgets/Master/WB_AnimatedProgressBarMaster.WB_AnimatedProgressBarMaster_C" 0 "(X=100.000000,Y=20.000000)" false 1.0 1.0))
  (bind _output_get (Variables|Components|SetCountdown%20Widget _returnvalue))
  (UserInterface|SetWidget (Variables|Default|GetWidget) _output_get))

(event OnComponentBeginOverlap(Box)
  (params (OverlappedComponent :type Primitive%20Component%20Object%20Reference) (OtherActor :type Actor%20Object%20Reference) (OtherComp :type Primitive%20Component%20Object%20Reference) (OtherBodyIndex :type Integer) (bFromSweep :type Boolean) (SweepResult :type Hit%20Result%20Structure%20%28by%20ref%29))
  (bind _output_get (Variables|Effect|SetCurrent%20Actor%20Count (+ (.Value (Utilities|Map|Find (Variables|Data|GetAffect%20Actors) OtherActor)) 1)))
  (Utilities|Map|Add (Variables|Data|GetAffect%20Actors) OtherActor _output_get))

(event OnComponentEndOverlap(Box)
  (params (OverlappedComponent :type Primitive%20Component%20Object%20Reference) (OtherActor :type Actor%20Object%20Reference) (OtherComp :type Primitive%20Component%20Object%20Reference) (OtherBodyIndex :type Integer))
  (bind _affect_actors (Variables|Data|GetAffect%20Actors))
  (bind _output_get (Variables|Effect|SetCurrent%20Actor%20Count (- (.Value (Utilities|Map|Find (Variables|Data|GetAffect%20Actors) OtherActor)) 1)))
  (if (<= _output_get 0)
    (Utilities|Map|Remove _affect_actors OtherActor)
    (else
      (Utilities|Map|Add _affect_actors OtherActor (Variables|Effect|GetCurrent%20Actor%20Count)))))

(fn ConstructionScript)

(fn EffectCountdown
  (bind _output_get (Variables|Data|SetElapsed%20Time (+ (Variables|Data|GetElapsed%20Time) (Utilities|Time|GetWorldDeltaSeconds))))
  (Utilities|FlowControl|Sequence
    (:then_0
      (if (>= _output_get (Variables|Effect|GetSeconds%20Per%20Loop))
        (Variables|Data|SetElapsed%20Time 0.0)
        (bind _keys (Utilities|Map|Keys (Variables|Data|GetAffect%20Actors)))
        (for _array_element _keys
          (Class|BPIDamagable|OnDamaged(Message) _array_element (Variables|Effect|GetAttack%20Effect) self (Math|Vector|GetUnitDirection(Vector) (Transformation|GetWorldLocation (Variables|Default|GetBox)) (Transformation|GetActorLocation _array_element))))))
    (:then_1
      (Default|SetValue (Variables|Components|GetCountdown%20Widget) (/ (Variables|Data|GetElapsed%20Time) (Variables|Effect|GetSeconds%20Per%20Loop))))))