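; Base Blueprint for combat equipment, driven by an EquipmentData struct that defines its weapon actor and data row names.
; The construction script sets the ChildActor component's class to the weapon actor from that struct.
; Getters resolve combat data and physic and spirit attack combos from data tables using those row names.
; Equip and Unequip call OnEquipped and OnUnequipped, which are empty hooks in this base.
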(fn ConstructionScript
  (ChildActorComponent|SetChildActorClass (Variables|Default|GetChildActor) (.weapon_actor (Variables|Data|GetEquipment%20Data))))

(fn GetEquipmentData
  (return (Variables|Data|GetEquipment%20Data)))

(fn GetCombatData
  (bind _returnvalue (Utilities|GetDataTableRow "/Game/GeneralCombat/Data/DataTables/Player/Weapon/DT_WeaponCombatData.DT_WeaponCombatData" (.EquipmentCombatDataName (Utilities|Struct|BreakS_EquipmentData (Variables|Data|GetEquipment%20Data))))
    (:then
      (return _returnvalue))))

(fn GetPhysicComboData
  (bind _returnvalue (Utilities|GetDataTableRow "/Game/GeneralCombat/Data/DataTables/GeneralCombat/DT_AttackComboData.DT_AttackComboData" (.PhysicComboName (Utilities|Struct|BreakS_EquipmentData (Variables|Data|GetEquipment%20Data))))
    (:then
      (return _returnvalue))))

(fn GetSpiritComboData
  (bind _returnvalue (Utilities|GetDataTableRow "/Game/GeneralCombat/Data/DataTables/GeneralCombat/DT_AttackComboData.DT_AttackComboData" (.SpiritComboName (Utilities|Struct|BreakS_EquipmentData (Variables|Data|GetEquipment%20Data))))
    (:then
      (return _returnvalue))))

(fn OnEquipped)

(fn OnUnequipped)

(fn Equip
  (Abstract|OnEquipped))

(fn Unequip
  (Abstract|OnUnequipped))