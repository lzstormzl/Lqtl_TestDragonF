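; Combat unit component that owns a character's stats, damage intake, hit reactions, spirit break and death, seeded from a data table.
; Incoming attacks check timed perfect-invincibility windows, then resolve damage by attack and defender flags, player blessing or non-player shield.
; Stagger and hit direction select reaction montages, with motion-warped knockback.
; Stat changes broadcast events, and reference-counted bitflags track combat states; effect functions are empty stubs.
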(event EventBeginPlay
  (bind _default_character_combat_data (Variables|Data|GetDefault%20Character%20Combat%20Data))
  (Utilities|FlowControl|Sequence
    (:then_0
      (CallFunction|InitializeComponent (Actor|GetComponentbyClass (Components|GetOwner) "/Script/Engine.SkeletalMeshComponent")))
    (:then_1
      ;[0.02 0.02 0.02 1 32] Apply Default Stats
      (Utilities|FlowControl|DelayUntilNextTick) ; Delay ini to avoid missed callbacks
      (bind _returnvalue (Utilities|GetDataTableRow (.datatable _default_character_combat_data) (.rowname _default_character_combat_data))
        (:then
          (CombatData|Stat|SetCharacterCombatData _returnvalue (Components|GetOwner))
          (CombatData|Stat|SetCurrentStat (.MaxStats (Utilities|Struct|BreakS_CharacterCombatData _returnvalue)) (Components|GetOwner)))))))

(event Custom|Play%20Hit%20React%20Montage
  (params (Montage :type Anim%20Montage%20Object%20Reference))
  (bind _notifyname (Animation|Montage|PlayMontage (Variables|References|GetSkeletal%20Mesh) Montage)
    (:OnNotifyBegin
      (switch name _notifyname
        (:End
          (Default|CallOnHitReactEnded))))))

(event Custom|Play%20Spirit%20Break%20End%20Montage
  (params (End%20Spirit%20Break%20Montage :type Anim%20Montage%20Object%20Reference))
  (if (not (Variables|Tạmđểtest|GetIsDead))
    (Animation|Montage|PlayMontage (Variables|References|GetSkeletal%20Mesh) End%20Spirit%20Break%20Montage
      (:OnCompleted
        _)
      (:OnInterrupted
        _))
    (Default|CallOnSpiritBreakEnded)))

(event Custom|Play%20Spirit%20Break%20Montage
  (params (Spirit%20Break%20Time :type Float%20%28double-precision%29) (Spirit%20Break%20Montage :type Array%20of%20Anim%20Montage%20Object%20References))
  (if (not (Variables|Tạmđểtest|GetIsDead))
    (Animation|Montage|PlayMontage (Variables|References|GetSkeletal%20Mesh) (Utilities|Array|Get(acopy) Spirit%20Break%20Montage)
      (:then
        (Utilities|FlowControl|Delay Spirit%20Break%20Time)
        (if (not (Variables|/Game/GeneralCombat/Blueprints/Pawns/BP_DefaultCombatCharacter.BP_DefaultCombatCharacter_C|GetisExecuting (.Out%20Character (CallFunction|GetPlayerCombatCharacter))))
          (CallFunction|PlaySpiritBreakEndMontage (Utilities|Array|Get(acopy) Spirit%20Break%20Montage 1))
          (if (<= (.spiritorb (CombatData|Stat|GetCurrentStat)) 0.0)
            (CombatData|Stat|AddCurrentStat (Utilities|Struct|MakeS_CombatResource 0.0 0.0 0.0 (.spiritorb (CombatData|Stat|GetMaxStat)) 0.0))))))))

(fn AddMaxStat
  (params (Delta :type S%20Combat%20Resource%20Structure) (Initigator :type Actor%20Object%20Reference))
  (CombatData|Stat|SetMaxStat (Class|BFLCombatResource|CombineResource Delta (.MaxStats (Utilities|Struct|BreakS_CharacterCombatData (Variables|Data|Stat|GetCharacter%20Combat%20Data)))) Initigator))

(fn AddCurrentStat
  (params (Delta :type S%20Combat%20Resource%20Structure) (Initigator :type Actor%20Object%20Reference))
  (CombatData|Stat|SetCurrentStat (Class|BFLCombatResource|CombineResource Delta (Variables|Data|Stat|GetCurrent%20Stat)) Initigator))

(fn SetMaxStat
  (params (Max%20Stat :type S%20Combat%20Resource%20Structure) (Initigator :type Actor%20Object%20Reference))
  (bind _structout (Utilities|Struct|SetmembersinS_CharacterCombatData (Variables|Data|Stat|GetCharacter%20Combat%20Data) (Class|BFLCombatResource|MaxFloat Max%20Stat 0.0)))
  (Default|CallOnMaxStatUpdated (.MaxStats (Utilities|Struct|BreakS_CharacterCombatData _structout)) Initigator))

(fn SetCurrentStat
  (params (Stat :type S%20Combat%20Resource%20Structure) (Initigator :type Actor%20Object%20Reference))
  (LocalVariables|SetLastStatsUpdated (CombatData|Stat|GetCurrentStat))
  (LocalVariables|SetDelta (Class|BFLCombatResource|SubtractResource Stat (Variables|Data|Stat|GetCurrent%20Stat)))
  (Variables|Data|Stat|SetCurrent%20Stat (Class|BFLCombatResource|ClampResource Stat (Utilities|Struct|MakeS_CombatResource 0.0 0.0 0.0 0.0 0.0) (.MaxStats (Utilities|Struct|BreakS_CharacterCombatData (Variables|Data|Stat|GetCharacter%20Combat%20Data)))))
  (Utilities|FlowControl|Sequence
    (:then_0
      ;[0.02 0.02 0.02 1 28] Spirit Break Check
      (bind _output_get (Variables|Data|Stat|SetSpirit%20Break (and (== (Utilities|Struct|BreakS_CombatResource (Variables|Data|Stat|GetCurrent%20Stat)) 0.0) (> (Utilities|Struct|BreakS_CombatResource (.MaxStats (Utilities|Struct|BreakS_CharacterCombatData (Variables|Data|Stat|GetCharacter%20Combat%20Data)))) 0.0))))
      (Default|CallOnSpiritBreakStateUpdated _output_get))
    (:then_1
      (Default|CallOnStatUpdated (Variables|Data|Stat|GetCurrent%20Stat) (LocalVariables|GetDelta) Initigator))
    (:then_2
      ;[0.02 0.02 0.02 1 28] Death Check
      (if (Math|Boolean|ANDBoolean (<= (Utilities|Struct|BreakS_CombatResource (Variables|Data|Stat|GetCurrent%20Stat)) 0.0) (> (Utilities|Struct|BreakS_CombatResource (.MaxStats (Utilities|Struct|BreakS_CharacterCombatData (Variables|Data|Stat|GetCharacter%20Combat%20Data)))) 0.0) (not (Variables|Tạmđểtest|GetIsDead)))
        (Default|CallOnDeath (Components|GetOwner))
        (Variables|Tạmđểtest|SetIsDead true)))
    (:then_3
      (if (and (> (Utilities|Struct|BreakS_CombatResource (LocalVariables|GetLastStatsUpdated)) (Utilities|Struct|BreakS_CombatResource (Variables|Data|Stat|GetCurrent%20Stat))) (!= Initigator (Components|GetOwner)))
        _))))

(fn ContainsFlags
  (params (Flags%20%28ECombatFlags%29 :type Integer) (Compare%20Type :type E_FlagCompareType%20Enum :default "NewEnumerator0"))
  (return (CallFunction|Contains(Flags) (Variables|Data|Flags|GetCombat%20Flags) Flags%20%28ECombatFlags%29 Compare%20Type)))

(fn GetCombatFlags
  (return (Variables|Data|Flags|GetCombat%20Flags)))

(fn IncreaseCombatFlagsCounter
  (params (Flags%20%28ECombatFlags%29 :type Integer))
  (CombatData|Flags|Internal|UpdateFlagsCounterMap Flags%20%28ECombatFlags%29 1))

(fn DecreaseCombatFlagsCounter
  (params (Flags%20%28ECombatFlags%29 :type Integer) (Remove%20All%20Counter :type Boolean))
  (CombatData|Flags|Internal|UpdateFlagsCounterMap Flags%20%28ECombatFlags%29 (Math|Integer|SelectInt -2147483648 -1 Remove%20All%20Counter)))

(fn UpdateFlagsCounterMap
  (params (Flags%20%28ECombatFlags%29 :type Integer) (Delta%20Value :type Integer))
  (LocalVariables|SetOrg%20Bitmask (Variables|Data|Flags|GetCombat%20Flags))
  (for _index (range 0 (- (|GetNumEnumEntries) 1))
    (bind _output_get (LocalVariables|SetCurrent%20Bitflag (Math|Float|Round (Math|Float|Power 2.0 (Math|Conversions|ToFloat(Integer) _index)))))
    (if (CallFunction|Contains(Flags) Flags%20%28ECombatFlags%29 _output_get "NewEnumerator0")
      (Utilities|FlowControl|Sequence
        (:then_0
          (if (not (.ReturnValue (Utilities|Map|Find (Variables|Data|Flags|GetFlags%20Counter%20Map) (LocalVariables|GetCurrent%20Bitflag))))
            (Variables|Data|Flags|SetCombat%20Flags (CallFunction|Add(Flags) (Variables|Data|Flags|GetCombat%20Flags) (LocalVariables|GetCurrent%20Bitflag)))))
        (:then_1
          (Utilities|Map|Add (Variables|Data|Flags|GetFlags%20Counter%20Map) (LocalVariables|GetCurrent%20Bitflag) (Math|Integer|Max(Integer) (+ (.Value (Utilities|Map|Find (Variables|Data|Flags|GetFlags%20Counter%20Map) (LocalVariables|GetCurrent%20Bitflag))) Delta%20Value)))
          (if (== (.Value (Utilities|Map|Find (Variables|Data|Flags|GetFlags%20Counter%20Map) (LocalVariables|GetCurrent%20Bitflag))) 0)
            (Utilities|Map|Remove (Variables|Data|Flags|GetFlags%20Counter%20Map) (LocalVariables|GetCurrent%20Bitflag))
            (Variables|Data|Flags|SetCombat%20Flags (CallFunction|Remove(Flags) (Variables|Data|Flags|GetCombat%20Flags) (LocalVariables|GetCurrent%20Bitflag))))))))
  (if (!= (LocalVariables|GetOrg%20Bitmask) (Variables|Data|Flags|GetCombat%20Flags))
    (Default|CallOnCombatFlagsUpdated (Variables|Data|Flags|GetCombat%20Flags))))

(fn ApplyEffect
  (params (Effect%20Tag :type Gameplay%20Tag%20Structure) (Stack :type Integer)))

(fn RemoveEffect)

(fn ApplyDamage
  (params (Attack%20Data :type S%20Attack%20Data%20Structure) (Initigator :type Actor%20Object%20Reference) (Hit%20Direction :type Vector))
  (LocalVariables|SetAttack%20Flags (.attackFlags (Utilities|Struct|BreakS_AttackData Attack%20Data)))
  (bind _keys (Utilities|Map|Keys (Variables|Data|Flags|GetPerfect%20Invincible%20Flags%20Map)))
  (for _array_element _keys
    (if (CallFunction|Contains(Flags) (LocalVariables|GetAttack%20Flags) _array_element (.Value (Utilities|Map|Find (Variables|Data|Flags|GetPerfect%20Invincible%20Flags%20Map) _array_element)))
      (Default|CallOnRecieveAttackWhileInvincible Attack%20Data Initigator Hit%20Direction)
      (return)))
  (Utilities|FlowControl|Sequence
    (:then_0
      (bind _output_get (LocalVariables|SetFinal%20Damage (CombatData|Stat|Internal|CalculateFinalDamage Attack%20Data)))
      (CombatData|Stat|AddCurrentStat (Class|BFLCombatResource|MultFloat _output_get -1.0) Initigator))
    (:then_1
      (if (not (<= (Utilities|Struct|BreakS_CombatResource (CombatData|Stat|GetCurrentStat)) 0.0))
        (HitReact|HandleHitReact (.Out%20Montage (HitReact|GetHitReactMontage (Utilities|Struct|BreakS_CombatResource (LocalVariables|GetFinal%20Damage)) Hit%20Direction)) Initigator (.Hit%20React%20Type (HitReact|GetHitReactMontage (Utilities|Struct|BreakS_CombatResource (LocalVariables|GetFinal%20Damage)) Hit%20Direction)))))))

(fn ApplyHeal
  (params (Heal%20Data :type S%20Combat%20Resource%20Structure) (Initigator :type Actor%20Object%20Reference))
  (CombatData|Stat|AddCurrentStat Heal%20Data Initigator))

(fn HasRequiredStats
  (params (Data :type S%20Combat%20Resource%20Structure))
  (return (Class|BFLCombatResource|LessorEqualResource Data (Variables|Data|Stat|GetCurrent%20Stat))))

(fn InitializeComponent
  (params (Skeletal%20Mesh%20Comp :type Skeletal%20Mesh%20Component%20Object%20Reference))
  (if (not (Variables|Data|GetInitialized))
    (Utilities|FlowControl|Sequence
      (:then_0
        (Variables|References|SetSkeletal%20Mesh Skeletal%20Mesh%20Comp)
        (bind _output_get (Variables|References|SetMotion%20Warping%20Comp (Actor|GetComponentbyClass (Components|GetOwner) "/Script/MotionWarping.MotionWarpingComponent")))
        (Utilities|IsValid _output_get
          (:Is%20Not%20Valid
            (bind _returnvalue (Game|AddComponentbyClass (Components|GetOwner) "/Script/MotionWarping.MotionWarpingComponent"))
            (Variables|References|SetMotion%20Warping%20Comp _returnvalue))))
      (:then_1
        (Variables|Data|SetInitialized (Utilities|IsValid (Variables|References|GetSkeletal%20Mesh)))))))

(fn SetCharacterCombatData
  (params (Character%20Combat%20Data :type S%20Character%20Combat%20Data%20Structure) (Initigator :type Actor%20Object%20Reference))
  (bind _output_get (Variables|Data|Stat|SetCharacter%20Combat%20Data Character%20Combat%20Data))
  (Default|CallOnMaxStatUpdated (.MaxStats (Utilities|Struct|BreakS_CharacterCombatData _output_get)) Initigator))

(fn GetMaxStat
  (return (.MaxStats (Utilities|Struct|BreakS_CharacterCombatData (Variables|Data|Stat|GetCharacter%20Combat%20Data)))))

(fn GetCurrentStat
  (return (Variables|Data|Stat|GetCurrent%20Stat)))

(fn GetHitReactMontage
  (params (Stagger%20Value :type Float%20%28double-precision%29) (Hit%20Direction :type Vector))
  (bind _character_combat_data (Variables|Data|Stat|GetCharacter%20Combat%20Data))
  (bind _character_combat_data_2 (Variables|Data|Stat|GetCharacter%20Combat%20Data))
  (bind _character_combat_data_3 (Variables|Data|Stat|GetCharacter%20Combat%20Data))
  (bind _hitreactdata (Utilities|Struct|BreakS_CharacterCombatData _character_combat_data))
  (bind _hitreactdata_2 (Utilities|Struct|BreakS_CharacterCombatData _character_combat_data_2))
  (bind _hitreactdata_3 (Utilities|Struct|BreakS_CharacterCombatData _character_combat_data_3))
  (bind (_knockdownforward _knockdownbackward) (Utilities|Struct|BreakS_HitReactData _hitreactdata))
  (bind (_flinchthreshold _interruptthreshold _knockdownthreshold) (Utilities|Struct|BreakS_HitReactData _hitreactdata_2))
  (bind (_interruptforward _interruptbackward _interruptleft _interruptright) (Utilities|Struct|BreakS_HitReactData _hitreactdata_3))
  (bind _outitem (Utilities|Array|Random _knockdownbackward))
  (bind _outitem_2 (Utilities|Array|Random _interruptbackward))
  (bind _outitem_3 (Utilities|Array|Random _knockdownforward))
  (if (and (Actor|ActorHasTag (Components|GetOwner) "Player") (Utilities|Map|Contains (Variables|/Game/ThirdPerson/BPC_Blessing.BPC_Blessing_C|GetActivating%20Effects (Variables|/Game/GeneralCombat/Blueprints/Pawns/BP_DefaultCombatCharacter.BP_DefaultCombatCharacter_C|GetBPC_Blessing (.Out%20Character (CallFunction|GetPlayerCombatCharacter)))) "NewEnumerator0"))
    (LocalVariables|SetStagger%20Value2 (- Stagger%20Value 15.0))
    (else
      (LocalVariables|SetStagger%20Value2 Stagger%20Value)))
  (if (Utilities|Operators|NotEqual(!=) :A Hit%20Direction)
    (LocalVariables|SetLocal%20Direction (Math|Transform|InverseTransformDirection (Transformation|GetWorldTransform (Variables|References|GetSkeletal%20Mesh)) Hit%20Direction))
    (Utilities|FlowControl|Sequence
      (:then_0
        (if (> (LocalVariables|GetStagger%20Value2) _knockdownthreshold)
          (return (Utilities|Select :Index (CallFunction|GetClosestDirectionfromVector2D "NewEnumerator8" (Math|Conversions|ToVector2D(Vector) (LocalVariables|GetLocal%20Direction))) :NewEnumerator8 _outitem_3 :NewEnumerator0 _outitem_3 :NewEnumerator1 _outitem :NewEnumerator2 _outitem_3 :NewEnumerator3 _outitem_3 :NewEnumerator4 _outitem_3 :NewEnumerator5 _outitem_3 :NewEnumerator6 _outitem :NewEnumerator7 _outitem) "NewEnumerator2")))
      (:then_1
        (if (> (LocalVariables|GetStagger%20Value2) _interruptthreshold)
          (return (Utilities|Select :Index (CallFunction|GetClosestSimpleDirectionfromVector2D "NewEnumerator8" (Math|Conversions|ToVector2D(Vector) (LocalVariables|GetLocal%20Direction))) :NewEnumerator8 _outitem_2 :NewEnumerator0 (.OutItem (Utilities|Array|Random _interruptforward)) :NewEnumerator1 _outitem_2 :NewEnumerator2 (.OutItem (Utilities|Array|Random _interruptright)) :NewEnumerator3 (.OutItem (Utilities|Array|Random _interruptleft))) "NewEnumerator1")))
      (:then_2
        (if (> (LocalVariables|GetStagger%20Value2) _flinchthreshold)
          (return (.OutItem (Utilities|Array|Random (.Flinch (Utilities|Struct|BreakS_HitReactData (.HitReactData (Utilities|Struct|BreakS_CharacterCombatData (Variables|Data|Stat|GetCharacter%20Combat%20Data))))))) "NewEnumerator0")))
      (:then_3
        (return 0 "NewEnumerator3")))))

(fn CalculateFinalDamage
  (params (Attack%20Data :type S%20Attack%20Data%20Structure))
  (bind _out_character (CallFunction|GetPlayerCombatCharacter))
  (bind _attackbasestat (Utilities|Struct|BreakS_AttackData Attack%20Data))
  (bind _bpc_blessing (Variables|/Game/GeneralCombat/Blueprints/Pawns/BP_DefaultCombatCharacter.BP_DefaultCombatCharacter_C|GetBPC_Blessing _out_character))
  (bind (_shield _health _spiritwater) (Utilities|Struct|BreakS_CombatResource _attackbasestat))
  (bind _blests_shield (Variables|/Game/ThirdPerson/BPC_Blessing.BPC_Blessing_C|GetBlesTS_Shield _bpc_blessing))
  (Utilities|FlowControl|Sequence
    (:then_0
      ;[0.02 0.02 0.02 1 24] Calculate Attack Against Differnet Forms
      (Utilities|GetAttackResponseType Attack%20Data
        (:Physical%20-%20Normal
          (LocalVariables|SetFinal%20Damage (Utilities|Struct|BreakS_AttackData Attack%20Data) :!label _label))
        (:Physical%20-%20Water%20Form
          (LocalVariables|SetFinal%20Damage (Utilities|Struct|MakeS_CombatResource 0.0 0.0 (+ _shield _health _spiritwater) 0.0 0.0) :!label _label_2))
        (:Physical%20-%20Guard%20Counter
          (goto _label_2))
        (:Spirit%20-%20Normal
          (goto _label))
        (:Spirit%20-%20Water%20Form
          (goto _label))
        (:Spirit%20-%20Guard%20Counter
          (goto _label))
        (:Overchagered%20-%20Normal
          (goto _label))
        (:Overchagered%20-%20Water%20Form
          (goto _label))
        (:True%20Damage
          (goto _label))))
    (:then_1
      (if (Actor|ActorHasTag (Components|GetOwner) "Player")
        (switch Utilities|FlowControl|Switch|SwitchonE_Blessing (Variables|/Game/ThirdPerson/BPC_Blessing.BPC_Blessing_C|GetBlessing%20Choosing _bpc_blessing)
          (:NewEnumerator1
            (if (< (.health (Utilities|Struct|BreakS_CombatResource (LocalVariables|GetFinal%20Damage))) _blests_shield)
              (Default|BlesTSReduceShield _bpc_blessing (* (- (.health (Utilities|Struct|BreakS_CombatResource (LocalVariables|GetFinal%20Damage))) _blests_shield) -1.0))
              (Utilities|Struct|SetmembersinS_CombatResource (LocalVariables|GetFinal%20Damage) 0.0)
              (else
                (Default|BlesTSReduceShield _bpc_blessing _blests_shield)
                (Utilities|Struct|SetmembersinS_CombatResource (LocalVariables|GetFinal%20Damage) (- (.health (Utilities|Struct|BreakS_CombatResource (LocalVariables|GetFinal%20Damage))) _blests_shield))))))
        (else
          ;[0.02 0.02 0.02 1 24] Ccalculate Shield Damage
          (Utilities|FlowControl|Sequence
            (:then_0
              (Utilities|Struct|SetmembersinS_CombatResource (LocalVariables|GetFinal%20Damage) (+ (.shield (Utilities|Struct|BreakS_CombatResource (LocalVariables|GetFinal%20Damage))) (.health (Utilities|Struct|BreakS_CombatResource (LocalVariables|GetFinal%20Damage))))))
            (:then_1
              (Utilities|Struct|SetmembersinS_CombatResource (LocalVariables|GetFinal%20Damage) (Math|Float|SelectFloat (Utilities|Struct|BreakS_CombatResource (LocalVariables|GetFinal%20Damage)) 0.0 (== (Utilities|Struct|BreakS_CombatResource (Variables|Data|Stat|GetCurrent%20Stat)) 0.0))))))))
    (:then_2
      (return (LocalVariables|GetFinal%20Damage)))))

(fn HandleHitReact
  (params (Anim%20Montage :type Anim%20Montage%20Object%20Reference) (Initigator :type Actor%20Object%20Reference) (Hit%20React%20Type :type E_HitReactType%20Enum :default "NewEnumerator0"))
  (bind _output_get (LocalVariables|SetKnockback%20Direction (Math|Vector|GetUnitDirection(Vector) (Transformation|GetActorLocation Initigator) (Transformation|GetWorldLocation (Variables|References|GetSkeletal%20Mesh)))))
  (Default|CallOnHitReactStarted Hit%20React%20Type _output_get)
  (HitReact|HandleKnockbackMotionWarping (LocalVariables|GetKnockback%20Direction))
  (CallFunction|PlayHitReactMontage Anim%20Montage)
  ;[0.5771 0.8493 1] Tiến comment: dùng để fix lỗi khi bị interupt không thể đánh tiếp hay đổi vũ khí được
  (Default|CancelCombo (Variables|/Game/GeneralCombat/Blueprints/Pawns/BP_DefaultCombatCharacter.BP_DefaultCombatCharacter_C|GetAttack%20Action%20Handler (.Out%20Character (CallFunction|GetPlayerCombatCharacter)))))

(fn GetSpiritBreakState
  (return (Variables|Data|Stat|GetSpirit%20Break)))

(fn SetPerferctInvincibleWindowAgainst
  (params (Flags%20Compare%20Map :type Map%20of%20Integers%20to%20Bytes) (Duration :type Float%20%28double-precision%29))
  (Variables|Data|Flags|SetPerfect%20Invincible%20Flags%20Map Flags%20Compare%20Map)
  (bind _returnvalue (Utilities|Time|SetTimerbyEvent (EventDispatchers|CreateEvent :!event RemovePerfectInvincibleWindow) Duration))
  (Variables|Data|Flags|SetDisable%20Invincible%20Flags%20Timer _returnvalue))

(fn RemovePerfectInvincibleWindow
  (Utilities|Map|Clear (Variables|Data|Flags|GetPerfect%20Invincible%20Flags%20Map))
  (Utilities|Time|ClearandInvalidateTimerbyHandle (Variables|Data|Flags|GetDisable%20Invincible%20Flags%20Timer)))

(fn HandleKnockbackMotionWarping
  (params (Knockback%20Direction :type Vector))
  (Class|MotionWarpingComponent|AddorUpdateWarpTargetfromLocationandRotation (Variables|References|GetMotion%20Warping%20Comp) "Knockback" (+ (* Knockback%20Direction 2.5e+02) (Transformation|GetActorLocation (Components|GetOwner))) "0, 0, 0"))

(fn HandleSpiritBreak
  (params (Spirit%20Break%20Time :type Float%20%28double-precision%29) (Anim%20Montage :type Array%20of%20Anim%20Montage%20Object%20References))
  (CallFunction|PlaySpiritBreakMontage Spirit%20Break%20Time Anim%20Montage))