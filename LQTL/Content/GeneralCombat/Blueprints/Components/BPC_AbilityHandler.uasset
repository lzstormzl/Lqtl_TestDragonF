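; Combat component that manages an owner's abilities and a blessing transform meter, broadcasting changes through event dispatchers.
; Abilities are capped in number, each spawned as an actor keyed by tag and activated by slot index when its normalized cooldown is full.
; Transform activation requires a minimum meter, which burns down while active and ends the transform at zero.
; Near-per-frame looping timers, rather than Tick, drive the updates.
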(event EventBeginPlay
  (Utilities|Time|SetTimerbyEvent (EventDispatchers|CreateEvent :!event UpdateAbilityCooldown) 0.001 true true))

(fn AddAbilities
  (params (New%20Abilities :type Array%20of%20S%20Ability%20Data%20Structures))
  (for _index (range 0 (Utilities|Operators|Subtract (Variables|Data|Ability|GetMax%20Abilities%20Count) (Utilities|Array|Length (Variables|Data|Ability|Internal|GetAbilities%20Data)) 1))
    (if (Utilities|Array|IsValidIndex New%20Abilities _index)
      (Control|Ability|Internal|AddAbility (Utilities|Array|Get(acopy) New%20Abilities _index)))))

(fn TriggerAbility
  (params (Index :type Integer) (Trigger%20Event :type ETriggerEvent%20Enum :default "None"))
  (bind (_out_data _result) (Access|Internal|GetSkillDataatIndex Index))
  (LocalVariables|SetAbility%20Data _out_data)
  (if (and _result (== (.Value (Utilities|Map|Find (Variables|Data|Ability|Internal|GetAbility%20Cooldown%20Lookup) (Utilities|Struct|BreakS_AbilityData (LocalVariables|GetAbility%20Data)))) 1.0))
    (Default|ActivateAbility (.Value (Utilities|Map|Find (Variables|Data|Ability|Internal|GetAbility%20Object%20Lookup) (Utilities|Struct|BreakS_AbilityData (LocalVariables|GetAbility%20Data)))) (Components|GetOwner) Trigger%20Event)
    (Control|Ability|Internal|StartAbilityCooldown (Utilities|Struct|BreakS_AbilityData (LocalVariables|GetAbility%20Data)))
    (Default|CallOnAbilityActivated (LocalVariables|GetAbility%20Data))))

(fn ReleaseAbility
  (params (Index :type Integer))
  (bind (_out_data _result) (Access|Internal|GetSkillDataatIndex Index))
  (if _result
    (Default|CallOnAbilityReleased _out_data)))

(fn GetCurrentAbilities
  (return (Variables|Data|Ability|Internal|GetAbilities%20Data)))

(fn GetSkillDataatIndex
  (params (Index :type Integer))
  (if (Utilities|Array|IsValidIndex (Variables|Data|Ability|Internal|GetAbilities%20Data) Index)
    (return (Utilities|Array|Get(acopy) (Variables|Data|Ability|Internal|GetAbilities%20Data) Index) true)
    (else
      (return "" false))))

(fn IncreaseTransformMeter
  (params (Amount :type Float%20%28double-precision%29))
  (bind _output_get (Variables|Data|BlessingTransform|Internal|SetTransform%20Meter (Math|Float|Clamp(Float) (+ Amount (Variables|Data|BlessingTransform|Internal|GetTransform%20Meter)) 0.0 1e+02)))
  (Default|CallOnTransformMeterUpdated (/ _output_get 1e+02)))

(fn SetCurrentBlessingTransform
  (params (Data :type S%20Blessing%20Transform%20Data%20Structure))
  (bind _output_get (Variables|Data|BlessingTransform|Internal|SetBlessing%20Transform%20Data Data))
  (Default|CallOnBlessingTransformUpdated _output_get))

(fn SetBlessingTransformActive
  (params (Active :type Boolean))
  (if (!= Active (Variables|Control|GetTransform%20Active))
    (|ConditionalGate)
    (Variables|Control|SetTransform%20Active Active)
    (Utilities|FlowControl|Sequence
      (:then_0
        (if Active
          (bind _returnvalue (Utilities|Time|SetTimerbyEvent (EventDispatchers|CreateEvent :!event CountdownTransformMeter) 0.001 true true))
          (Variables|Control|SetTransform%20Countdown%20Timer _returnvalue)
          (else
            (Utilities|Time|ClearandInvalidateTimerbyHandle (Variables|Control|GetTransform%20Countdown%20Timer)))))
      (:then_1
        (Default|CallOnBlessingTransformActiveChanged (Variables|Control|GetTransform%20Active))))))

(fn GetCurrentBlessingTransformData
  (return (Variables|Data|BlessingTransform|Internal|GetBlessing%20Transform%20Data)))

(fn CountdownTransformMeter
  (Control|BlessingTransform|IncreaseTransformMeter (* (Utilities|Time|GetWorldDeltaSeconds) (Variables|Data|BlessingTransform|GetTransform%20Meter%20Burn%20Per%20Seconds) -1.0))
  (if (== (Variables|Data|BlessingTransform|Internal|GetTransform%20Meter) 0.0)
    (Control|BlessingTransform|SetBlessingTransformActive false)))

(fn GetBlessingTransformActive
  (return (Variables|Control|GetTransform%20Active)))

(fn UpdateAbilityCooldown
  (for _array_element (Variables|Data|Ability|Internal|GetAbilities%20Data)
    (Utilities|FlowControl|Sequence
      (:then_0
        (bind _output_get (LocalVariables|SetCurrent%20Ability%20Data _array_element))
        (LocalVariables|SetCurrent%20Ability%20Tag (Utilities|Struct|BreakS_AbilityData _output_get))
        (LocalVariables|SetCurrent%20Cooldown%20Data (.Value (Utilities|Map|Find (Variables|Data|Ability|Internal|GetAbility%20Cooldown%20Lookup) (LocalVariables|GetCurrent%20Ability%20Tag)))))
      (:then_1
        (LocalVariables|SetCurrent%20Cooldown%20Data (Math|Float|Min(Float) (+ (LocalVariables|GetCurrent%20Cooldown%20Data) (/ (Utilities|Time|GetWorldDeltaSeconds) (Utilities|Struct|BreakS_AbilityData (LocalVariables|GetCurrent%20Ability%20Data)))) 1.0)))
      (:then_2
        (Control|Ability|Internal|SetAbilityCooldown (LocalVariables|GetCurrent%20Ability%20Tag) (LocalVariables|GetCurrent%20Cooldown%20Data))))))

(fn StartAbilityCooldown
  (params (Ability%20Tag :type Gameplay%20Tag%20Structure))
  (Control|Ability|Internal|SetAbilityCooldown Ability%20Tag 0.0))

(fn SetAbilityCooldown
  (params (Ability%20Tag :type Gameplay%20Tag%20Structure) (Cooldown%20Percent :type Float%20%28double-precision%29))
  (Utilities|Map|Add (Variables|Data|Ability|Internal|GetAbility%20Cooldown%20Lookup) Ability%20Tag Cooldown%20Percent)
  (Default|CallOnAbilityCooldownUpdated Ability%20Tag Cooldown%20Percent))

(fn AddAbility
  (params (Ability%20Data :type S%20Ability%20Data%20Structure))
  (if (!= (Utilities|Struct|BreakS_AbilityData Ability%20Data) "")
    (Utilities|FlowControl|Sequence
      (:then_0
        (bind _returnvalue (Utilities|Array|Add (Variables|Data|Ability|Internal|GetAbilities%20Data) Ability%20Data))
        (Default|CallOnNewAbilityAdded Ability%20Data _returnvalue))
      (:then_1
        (bind _returnvalue_2 (Game|SpawnActorfromClass (.AbilityClass (Utilities|Struct|BreakS_AbilityData Ability%20Data)) (Math|Transform|MakeTransform "0, 0, 0" "0, 0, 0" "1.000000,1.000000,1.000000") "AlwaysSpawn" "MultiplyWithRoot" 0 0))
        (Utilities|Map|Add (Variables|Data|Ability|Internal|GetAbility%20Object%20Lookup) (Utilities|Struct|BreakS_AbilityData Ability%20Data) _returnvalue_2)))))