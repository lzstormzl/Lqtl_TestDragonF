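; Character component that manages movement states (walk, run, sprint, slide) and directional dodges for a combat character.
; Each state applies its own speed, acceleration, rotation and friction values to the movement component.
; Registered input becomes camera-relative and either snaps or turns gradually on a looping timer, while a delay timer signals halted input.
; Dodges play montages from a swappable anim set, blocking movement, cancelling combos and broadcasting state changes.
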(event EventBeginPlay
  ;[0.364 1 0.2355] Setup initial properties
  (Utilities|FlowControl|Sequence
    (:then_0
      (CallFunction|InitializeComponent (.AsCharacter (Utilities|Casting|CastToCharacter (Components|GetOwner)))))
    (:then_1
      (Utilities|FlowControl|DelayUntilNextTick)
      (if (Utilities|Enum|NotEqual(Enum) (Variables|MovementModeData|GetInitial%20Movement%20State) "NewEnumerator0")
        (Controls|Movement|SetNewMovementState (Variables|MovementModeData|GetInitial%20Movement%20State) true)))))

(event Custom|Play%20Dodge%20Anim
  (params (Montage :type Anim%20Montage%20Object%20Reference))
  (bind (_out_character _valid) (CallFunction|GetPlayerCombatCharacter))
  (bind _output_get (Variables|InstanceData|Dodge|SetCurrent%20Dodge%20Montage Montage))
  (Utilities|IsValid _output_get
    (:Is%20Valid
      (Utilities|FlowControl|DelayUntilNextTick)
      (bind _notifyname (Animation|Montage|PlayMontage (Variables|References|GetSkeletal%20Mesh) _output_get)
        (:then
          (bind _output_get_2 (Variables|InstanceData|Dodge|SetIs%20Dodging true))
          (Default|CallOnDodgeStateChanged _output_get_2)
          (Variables|/Script/Engine.CharacterMovementComponent|SetbUseControllerDesiredRotation (Variables|References|GetMovement%20Comp) (not (Variables|InstanceData|Dodge|GetIs%20Dodging)) :!label _label)
          (if _valid
            (Default|CancelCombo (Variables|/Game/GeneralCombat/Blueprints/Pawns/BP_DefaultCombatCharacter.BP_DefaultCombatCharacter_C|GetAttack%20Action%20Handler _out_character))))
        (:OnBlendOut
          (bind _output_get_3 (Variables|InstanceData|Dodge|SetIs%20Dodging false :!label _label_2))
          (Default|CallOnDodgeStateChanged _output_get_3)
          (goto _label))
        (:OnInterrupted
          (goto _label_2))
        (:OnNotifyBegin
          (switch name _notifyname
            (:End
              (Utilities|FlowControl|Sequence
                (:then_0
                  (goto _label_2))
                (:then_1
                  (if (Utilities|Operators|NotEqual(!=) :A (Variables|InstanceData|Movement|GetMovement%20Input%20Vector) :ErrorTolerance 0.001)
                    (Animation|Montage|MontageStop (Components|SkeletalMesh|GetAnimInstance (Variables|References|GetSkeletal%20Mesh)) 0.4 (Variables|InstanceData|Dodge|GetCurrent%20Dodge%20Montage))))))))))))

(fn TryPerformDodge
  (params (Direction :type E_Direction2D%20Enum :default "NewEnumerator8") (Forward%20Rotation :type Rotator))
  (bind _current_dodge_anim_set (Variables|InstanceData|Dodge|GetCurrent%20Dodge%20Anim%20Set))
  (if (Access|GetIsDodging)
    (return false)
    (else
      (CallFunction|PlayDodgeAnim (Utilities|Select :Index Direction :NewEnumerator8 0 :NewEnumerator0 (.forward _current_dodge_anim_set) :NewEnumerator1 (.backward _current_dodge_anim_set) :NewEnumerator2 (.left _current_dodge_anim_set) :NewEnumerator3 (.right _current_dodge_anim_set) :NewEnumerator4 (.forwardleft _current_dodge_anim_set) :NewEnumerator5 (.forwardright _current_dodge_anim_set) :NewEnumerator6 (.backwardleft _current_dodge_anim_set) :NewEnumerator7 (.backwardright _current_dodge_anim_set)))
      (Transformation|SetActorRotation (Components|GetOwner) Forward%20Rotation)
      (return true))))

(fn GetMovementState
  (return (Variables|InstanceData|Movement|GetMovement%20State)))

(fn GetIsDodging
  (return (Variables|InstanceData|Dodge|GetIs%20Dodging)))

(fn GetIsSprinting
  (return (Utilities|Enum|Equal(Enum) (Variables|InstanceData|Movement|GetMovement%20State) "NewEnumerator3")))

(fn AssignDodgeAnimSet
  (params (new%20Dodge%20Anim%20Set :type S%20Dodge%20Anim%20Set%20Data%20Structure))
  (Variables|InstanceData|Dodge|SetCurrent%20Dodge%20Anim%20Set new%20Dodge%20Anim%20Set))

(fn SetNewMovementState
  (params (New%20Movement%20State :type E_MovementState%20Enum :default "NewEnumerator0") (Override%20Higher%20Mode :type Boolean))
  (if (Utilities|Enum|NotEqual(Enum) New%20Movement%20State (Variables|InstanceData|Movement|GetMovement%20State))
    (if (or Override%20Higher%20Mode (> (Math|Conversions|ToInteger(Byte) New%20Movement%20State) (Math|Conversions|ToInteger(Byte) (Variables|InstanceData|Movement|GetMovement%20State))))
      (Utilities|FlowControl|Sequence
        (:then_0
          (Variables|InstanceData|Movement|SetMovement%20State New%20Movement%20State)
          (Controls|Internal|UpdateMovementCompValues))
        (:then_1
          (if (Utilities|Operators|NotEqual(!=) :A (Variables|InstanceData|Movement|GetLast%20Movement%20Input))
            (Default|CallOnMovementStateChanged (Variables|InstanceData|Movement|GetMovement%20State))))))))

(fn InitializeComponent
  (params (Owner%20Character :type Character%20Object%20Reference))
  (if (not (Variables|InstanceData|General|GetInitialized))
    (Utilities|FlowControl|Sequence
      (:then_0
        (bind _output_get (Variables|References|SetOwner%20Character Owner%20Character))
        (Variables|References|SetSkeletal%20Mesh (Variables|/Script/Engine.Character|GetMesh _output_get))
        (Variables|References|SetMovement%20Comp (Variables|/Script/Engine.Character|GetCharacterMovement _output_get)))
      (:then_1
        (Variables|InstanceData|General|SetInitialized (Utilities|IsValid (Variables|References|GetOwner%20Character)))))))

(fn UpdateMovementCompValues
  (LocalVariables|SetMovement%20Data (Utilities|Select :Index (Variables|InstanceData|Movement|GetMovement%20State) :NewEnumerator0 "" :NewEnumerator1 (Variables|MovementModeData|GetWalk%20Movement) :NewEnumerator2 (Variables|MovementModeData|GetRun%20Movement) :NewEnumerator3 (Variables|MovementModeData|GetSprint%20Movement) :NewEnumerator5 (Variables|MovementModeData|GetSlide%20Movement)))
  (Utilities|FlowControl|Sequence
    (:then_0
      (Variables|/Script/Engine.CharacterMovementComponent|SetMaxWalkSpeed (Variables|References|GetMovement%20Comp) (Utilities|Struct|BreakS_MovementModeData (LocalVariables|GetMovement%20Data))))
    (:then_1
      (Variables|/Script/Engine.CharacterMovementComponent|SetMaxAcceleration (Variables|References|GetMovement%20Comp) (Utilities|Struct|BreakS_MovementModeData (LocalVariables|GetMovement%20Data))))
    (:then_2
      (Variables|/Script/Engine.CharacterMovementComponent|SetRotationRate (Variables|References|GetMovement%20Comp) (Utilities|Struct|BreakS_MovementModeData (LocalVariables|GetMovement%20Data))))
    (:then_3
      (Variables|/Script/Engine.CharacterMovementComponent|SetBrakingDecelerationWalking (Variables|References|GetMovement%20Comp) (Utilities|Struct|BreakS_MovementModeData (LocalVariables|GetMovement%20Data))))
    (:then_4
      (Variables|/Script/Engine.CharacterMovementComponent|SetGroundFriction (Variables|References|GetMovement%20Comp) (Utilities|Struct|BreakS_MovementModeData (LocalVariables|GetMovement%20Data))))
    (:then_5
      (bind _output_get (Variables|InstanceData|Movement|SetSnap%20to%20Input (Utilities|Struct|BreakS_MovementModeData (LocalVariables|GetMovement%20Data))))
      (if _output_get
        (Utilities|Time|ClearandInvalidateTimerbyHandle (Variables|InstanceData|Movement|GetTurning%20Vector%20Timer%20handle))))))

(fn RegisterMovementInputVector
  (params (Movement%20Input%20Vector :type Vector%202D%20Structure))
  (Variables|InstanceData|Movement|SetMovement%20Input%20Vector Movement%20Input%20Vector)
  (Variables|InstanceData|Movement|SetIs%20Movement%20Registered true)
  (Utilities|Time|SetTimerbyEvent (EventDispatchers|CreateEvent :!event MovementInputStopped) (Variables|MovementModeData|GetDelay%20Till%20Halt))
  (if (not (Variables|InstanceData|Dodge|GetIs%20Dodging))
    (Utilities|FlowControl|Sequence
      (:then_0
        ;[0.02 0.02 0.02 1 30] Move (or snap) movement vector to target input
        (if (Variables|InstanceData|Movement|GetSnap%20to%20Input)
          (Variables|InstanceData|Movement|SetCurrent%20Movement%20Vector (Utility|WorldtoControllerVector (Variables|InstanceData|Movement|GetMovement%20Input%20Vector)))
          (elif (not (Utilities|Time|IsTimerActivebyHandle (Variables|InstanceData|Movement|GetTurning%20Vector%20Timer%20handle)))
            (bind _returnvalue (Utilities|Time|SetTimerbyEvent (EventDispatchers|CreateEvent :!event TurnMovementVectorTowardsTargetInput) 0.001 true true))
            (Variables|InstanceData|Movement|SetTurning%20Vector%20Timer%20handle _returnvalue))))
      (:then_1
        ;[0.02 0.02 0.02 1 30] Apply movement input to referenced character
        (Class|PawnMovementComponent|AddInputVector (Variables|References|GetMovement%20Comp) (Math|Conversions|ToVector(Vector2D) (Variables|InstanceData|Movement|GetCurrent%20Movement%20Vector)) false)
        (Default|CallOnMovementVectorUpdated (Variables|InstanceData|Movement|GetCurrent%20Movement%20Vector)))
      (:then_2
        (if (Utilities|Operators|EqualEqual :A Movement%20Input%20Vector :ErrorTolerance 0.01)
          (Default|CallOnMovementStateChanged "NewEnumerator0")
          (elif (Utilities|Operators|EqualEqual :A (Variables|InstanceData|Movement|GetLast%20Movement%20Input) :ErrorTolerance 0.01)
            (Default|CallOnMovementStateChanged (Variables|InstanceData|Movement|GetMovement%20State)))))
      (:then_3
        (if (Variables|InstanceData|Movement|GetSnap%20to%20Input)
          (Variables|InstanceData|Movement|SetLast%20Movement%20Input Movement%20Input%20Vector)
          (Variables|InstanceData|Movement|SetMovement%20Input%20Vector "") ; Reset Movement input to allow dodge anim to register properly \nbased on movement state
        )))))

(fn TurnMovementVectorTowardsTargetInput
  (LocalVariables|SetController%20Input%20Vector (Utility|WorldtoControllerVector (Variables|InstanceData|Movement|GetMovement%20Input%20Vector)))
  (LocalVariables|SetAngle%20Step (* (Utilities|Time|GetWorldDeltaSeconds) (LocalVariables|GetChr_Slide_Rotate_Rate)))
  (LocalVariables|SetMax%20Angle (CallFunction|FlatAngle(Vector) (Math|Conversions|ToVector(Vector2D) (Variables|InstanceData|Movement|GetCurrent%20Movement%20Vector)) (Math|Conversions|ToVector(Vector2D) (LocalVariables|GetController%20Input%20Vector))))
  (if (>= (LocalVariables|GetAngle%20Step) (LocalVariables|GetMax%20Angle))
    (Variables|InstanceData|Movement|SetCurrent%20Movement%20Vector (LocalVariables|GetController%20Input%20Vector))
    (Utilities|Time|ClearandInvalidateTimerbyHandle (Variables|InstanceData|Movement|GetTurning%20Vector%20Timer%20handle))
    (else
      (Variables|InstanceData|Movement|SetCurrent%20Movement%20Vector (Math|Conversions|ToVector2D(Vector) (Math|Vector|RotateVectorAroundAxis (Math|Vector|MakeVector (.x (Variables|InstanceData|Movement|GetCurrent%20Movement%20Vector)) (.y (Variables|InstanceData|Movement|GetCurrent%20Movement%20Vector)) 0.0) (LocalVariables|GetAngle%20Step) (Math|Vector|SelectVector "0.000000,0.000000,1.000000" (Math|Vector|CrossProduct (Math|Conversions|ToVector(Vector2D) (Variables|InstanceData|Movement|GetCurrent%20Movement%20Vector)) (Math|Conversions|ToVector(Vector2D) (LocalVariables|GetController%20Input%20Vector))) (Math|Float|NearlyEqual(Float) (Math|Vector2D|DotProduct(2D) (Math|Vector2D|Normalize2D (Variables|InstanceData|Movement|GetCurrent%20Movement%20Vector)) (LocalVariables|GetController%20Input%20Vector)) -1.0 0.01))))))))

(fn WorldtoControllerVector
  (params (In%20Vect :type Vector%202D%20Structure))
  (return (Math|Conversions|ToVector2D(Vector) (+ (* (Math|Vector|GetRightVector (Math|Rotator|MakeRotator 0.0 0.0 (.yaw (Pawn|GetControlRotation (Variables|References|GetOwner%20Character) :!class /Script/Engine.Pawn)))) (.x In%20Vect)) (* (Math|Vector|GetForwardVector (Math|Rotator|MakeRotator 0.0 0.0 (.yaw (Pawn|GetControlRotation (Variables|References|GetOwner%20Character) :!class /Script/Engine.Pawn)))) (.y In%20Vect))))))

(fn MovementInputStopped
  (Default|CallOnMovementInputHalted)
  (Variables|InstanceData|Movement|SetIs%20Movement%20Registered false))

(fn GetIsMovementRegistered
  (return (Variables|InstanceData|Movement|GetIs%20Movement%20Registered)))

(fn GetCurrentMovementVector
  (return (Variables|InstanceData|Movement|GetCurrent%20Movement%20Vector)))