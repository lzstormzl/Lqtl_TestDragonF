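; Base enemy pawn that connects combat stats, damage intake and lock-on targeting to overhead UI.
; BPC_CombatUnit takes its data from a DataTable row, receives incoming damage, and has shield and health zeroed on destruction.
; Health bar and lock-on widgets attach to mesh sockets, appear on focus and fade out by timeline.
; Stat changes from others briefly reveal the health bar, while spirit break keeps the lock-on indicator visible.
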(event Custom|Set%20Focus%20Active
  (params (Focused :type Boolean))
  ;[0.02 0.02 0.02 1 32] Widget Control On Focus
  (if Focused
    (Utilities|FlowControl|Sequence
      (:then_0
        (Widget|SetRenderOpacity (Variables|Focus|GetHealth%20Bar%20Widget) 1.0))
      (:then_1
        (bind _alpha (Timeline|Timeline Stop)
          (:Update
            (Utilities|FlowControl|Sequence
              (:then_0
                (Widget|SetRenderOpacity (Variables|Focus|GetHealth%20Bar%20Widget) (Math|Float|Lerp (Variables|/Script/UMG.Widget|GetRenderOpacity (Variables|Focus|GetHealth%20Bar%20Widget)) 0.0 _alpha)))
              (:then_1
                (if (not (Default|GetSpiritBreakState (Variables|Default|GetBPC_CombatUnit)))
                  (Widget|SetRenderOpacity (Variables|Focus|GetLock%20On%20Indicator%20Widget) (Math|Float|Lerp (Variables|/Script/UMG.Widget|GetRenderOpacity (Variables|Focus|GetLock%20On%20Indicator%20Widget)) 0.0 _alpha)))))))))
    (else
      (Utilities|Time|ClearandInvalidateTimerbyHandle (Variables|Focus|GetHide%20Healthbar%20Display%20Timer))
      (Timeline|Timeline PlayFromStart))))

(event Custom|On%20Destroyed
  (params (DestroyedActor :type Actor%20Object%20Reference))
  ;[0.7812 0.1236 0.08138 1 28] Setup Death Event On Destroyed
  (Default|SetCurrentStat (Variables|Default|GetBPC_CombatUnit) (Utilities|Struct|MakeS_CombatResource 0.0 0.0) self))

(event EventBeginPlay
  (bind _out_row (Access|GetCombatData))
  (CallFunction|InitializeWidget)
  (Default|SetCharacterCombatData (Variables|Default|GetBPC_CombatUnit) _out_row self)
  (Default|SetCurrentStat (Variables|Default|GetBPC_CombatUnit) (.MaxStats (Utilities|Struct|BreakS_CharacterCombatData _out_row)) self)
  ;[0.7812 0.1236 0.08138 1 28] Setup Death Event On Destroyed
  (Game|BindEventtoOnDestroyed (delegate Custom|On%20Destroyed)))

(event EventOnFocused
  ;[0.02 0.02 0.02 1 32] Lock On Target
  (Variables|Focus|SetFocused true)
  (CallFunction|SetFocusActive true)
  (Widget|SetRenderOpacity (Variables|Focus|GetLock%20On%20Indicator%20Widget) 1.0)
  (Utilities|Time|ClearandInvalidateTimerbyHandle (Variables|Focus|GetHide%20Healthbar%20Display%20Timer)))

(event EventOnUnfocused
  ;[0.02 0.02 0.02 1 32] Lock On Target
  (Variables|Focus|SetFocused false)
  (CallFunction|SetFocusActive false))

(event EventOnDamaged
  (params (Source%20Attack :type S%20Attack%20Data%20Structure) (Initigator :type Actor%20Object%20Reference) (Hit%20Direction :type Vector :default "0, 0, 0"))
  ;[0.02 0.02 0.02 1 32] Damagable
  (Default|ApplyDamage (Variables|Default|GetBPC_CombatUnit) Source%20Attack Initigator Hit%20Direction))

(event OnSpiritBreakStateUpdated(BPC_CombatUnit)
  (params (State :type Boolean))
  (if State
    (Widget|SetRenderOpacity (Variables|Focus|GetLock%20On%20Indicator%20Widget) 1.0)))

(event OnStatUpdated(BPC_CombatUnit)
  (params (New%20Data :type S%20Combat%20Resource%20Structure) (Delta%20Data :type S%20Combat%20Resource%20Structure) (Initigator :type Actor%20Object%20Reference))
  (if (!= Initigator self)
    (Callbacks|OnCombatInitiated)))

(fn ConstructionScript)

(fn GetCombatData
  (bind _returnvalue (Utilities|GetDataTableRow "/Game/GeneralCombat/Data/DataTables/GeneralCombat/DT_CharacterCombatData.DT_CharacterCombatData" (Variables|Data|GetCombat%20Data%20Name))
    (:then
      (return _returnvalue))))

(fn InitializeWidget
  (Utilities|FlowControl|Sequence
    (:then_0
      ;[0.02 0.02 0.02 1 30] Heath Bar
      (bind _returnvalue (UserInterface|CreateWidget "/Game/GeneralCombat/Blueprints/Widgets/Combat/HealthBar/WB_NormalEnemyHealthBar.WB_NormalEnemyHealthBar_C"))
      (bind _output_get (Variables|Focus|SetHealth%20Bar%20Widget _returnvalue))
      (Default|Initialize _output_get (Variables|Default|GetBPC_CombatUnit) (Access|GetCombatData))
      (Widget|SetRenderOpacity (Variables|Focus|GetHealth%20Bar%20Widget) 0.0)
      (UserInterface|SetWidget (Variables|Default|GetWidget_HealthBar) (Variables|Focus|GetHealth%20Bar%20Widget))
      (Transformation|SetWorldRotation (Variables|Default|GetWidget_HealthBar) "0.000000,90.000000,0.000000" false false)
      (Transformation|AttachComponentToComponent (Variables|Default|GetWidget_HealthBar) (Variables|Character|GetMesh) "Head" "SnapToTarget" "KeepWorld" "KeepWorld" true))
    (:then_1
      ;[0.02 0.02 0.02 1 30] Lock On Target
      (bind _returnvalue_2 (UserInterface|CreateWidget "/Game/GeneralCombat/Blueprints/Widgets/Combat/Indicators/WB_LockTargetIndicator.WB_LockTargetIndicator_C"))
      (bind _output_get_2 (Variables|Focus|SetLock%20On%20Indicator%20Widget _returnvalue_2))
      (Default|Initialize _output_get_2 (Variables|Default|GetBPC_CombatUnit))
      (Widget|SetRenderOpacity (Variables|Focus|GetLock%20On%20Indicator%20Widget) 0.0)
      (UserInterface|SetWidget (Variables|Default|GetWidget_LockOnIndicator) (Variables|Focus|GetLock%20On%20Indicator%20Widget))
      (Transformation|AttachComponentToComponent (Variables|Default|GetWidget_LockOnIndicator) (Variables|Character|GetMesh) "CenterMass" "SnapToTarget" "KeepWorld" "KeepWorld" true))))

(fn OnCombatInitiated
  (if (not (Variables|Focus|GetFocused))
    (CallFunction|SetFocusActive true)
    (bind _returnvalue (Utilities|Time|SetTimerbyEvent (EventDispatchers|CreateEvent :!event OnUnfocused) 5.0))
    (Variables|Focus|SetHide%20Healthbar%20Display%20Timer _returnvalue)))

(fn OnStatUpdated
  (params (Stat :type S%20Combat%20Resource%20Structure%20%28by%20ref%29) (Initigator :type Actor%20Object%20Reference)))

(fn GetCenterMassLocation
  (return (Transformation|GetSocketLocation (Variables|Character|GetMesh) "CenterMass")))

(fn GetLockonLocation
  (return (Transformation|GetSocketLocation (Variables|Character|GetMesh) "LockOn")))