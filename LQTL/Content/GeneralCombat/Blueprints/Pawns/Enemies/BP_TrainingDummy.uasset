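; BP_TrainingDummy is an enemy pawn that serves as a training dummy, with a soaked value shown on its health bar.
; Each capsule overlap raises the clamped soaked value, updates the widget and initiates combat.
; On death from BPCCombatUnit, it unfocuses, ragdolls, raises a combat flag counter and swaps in a dynamic material.
; After a short delay, a timeline drives that material's dissolve parameter, then the actor is destroyed.
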(event OnComponentBeginOverlap(CapsuleComponent)
  (params (OverlappedComponent :type Primitive%20Component%20Object%20Reference) (OtherActor :type Actor%20Object%20Reference) (OtherComp :type Primitive%20Component%20Object%20Reference) (OtherBodyIndex :type Integer) (bFromSweep :type Boolean) (SweepResult :type Hit%20Result%20Structure%20%28by%20ref%29))
  (bind _output_get (Variables|Default|SetSoaked%20Value (Math|Float|Clamp(Float) (+ (Variables|Default|GetSoaked%20Value) 5e+01) 0.0 (Variables|Default|GetMax%20Soaked%20Value))))
  (Default|SetSoakedValue (Variables|Default|GetHealth%20Bar%20Widget) _output_get)
  (CallFunction|OnCombatInitiated))

(event EventBeginPlay
  (|CallParentFunction)
  (Default|SetSoakedValue (Variables|Default|GetHealth%20Bar%20Widget) (Variables|Default|GetSoaked%20Value))
  ;[0.4167 0.04774 0.06603] Event binding
  (EventDispatchers|BindEventtoOnDeath (Variables|Default|GetBPC_CombatUnit) (EventDispatchers|CreateEvent :!event Custom|Event%20On%20Death)))

(event Custom|Event%20On%20Death
  (params (Initigator :type Actor%20Object%20Reference))
  (bind _mesh (Variables|Character|GetMesh))
  (Utilities|FlowControl|Sequence
    (:then_0
      (CallFunction|OnUnfocused)
      (Physics|SetSimulatePhysics (Variables|Character|GetMesh) true)
      (Collision|SetCollisionProfileName (Variables|Character|GetMesh) "Ragdoll" true :!class /Script/Engine.PrimitiveComponent)
      (Default|IncreaseCombatFlagsCounter (Variables|Default|GetBPC_CombatUnit) (|BitmaskLiteral 2))
      (bind _returnvalue (Rendering|Material|CreateDynamicMaterialInstance _mesh 0 (Rendering|Material|GetMaterial _mesh 0) "None" :!class /Script/Engine.PrimitiveComponent))
      (bind _output_get (Variables|Default|SetDissolve%20Material _returnvalue))
      (Rendering|Material|SetMaterial (Variables|Character|GetMesh) 0 _output_get))
    (:then_1
      (Utilities|FlowControl|Delay 2.0)
      (bind _alpha (Timeline|Dissolve%20Timeline PlayFromStart)
        (:Update
          (Rendering|Material|SetScalarParameterValue (Variables|Default|GetDissolve%20Material) "Dissolve" _alpha :!class /Script/Engine.MaterialInstanceDynamic))
        (:Finished
          (Rendering|SetCastShadow (Variables|Character|GetMesh) false)
          (Actor|DestroyActor))))))

(fn ConstructionScript)