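; Looping FX demo actor that fires repeated volleys of spear projectiles, starting on BeginPlay.
; Each cycle traces against static world objects along a fixed world direction from SpawnLocation to find a target.
; A delayed loop spawns ten BP_Projectile_Spear_01 actors facing the camera's rotation, each given the hit point or trace end as TargetLocation.
; A retriggerable delay, refreshed by every spawn, restarts the cycle after the last one.
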(event Custom|Throw
  (bind _spawn_location (Variables|Default|GetSpawn%20Location))
  (bind _returnvalue (Transformation|GetWorldLocation _spawn_location))
  ;[1 1 1] Shot
  (bind _outhit (Collision|LineTraceForObjects _returnvalue (+ _returnvalue (* (Variables|Default|GetRange) (Math|Vector|GetForwardVector "0.000000,0.000000,1.000000"))) (Utilities|Array|MakeArray "ObjectTypeQuery1") false 0 "None" :!label _label))
  (Utilities|ForLoopwithDelay 0 9 0.1
    (:Loop%20Body
      (bind _returnvalue_2 (Game|SpawnActorfromClass "/Game/Common/FX_Sources/SourcePackage/ElementPrjtile_FX/Characters/Blueprints/BP_Projectile_Spear_01.BP_Projectile_Spear_01_C" (Math|Transform|MakeTransform (Transformation|GetWorldLocation (Variables|Default|GetSpawn%20Location)) (Camera|GetCameraRotation (Game|GetPlayerCameraManager 0)) "1.000000,1.000000,1.000000") "AdjustIfPossibleButAlwaysSpawn" "OverrideRootScale" 0 0))
      (Variables|/Game/Common/FX_Sources/SourcePackage/ElementPrjtile_FX/Characters/Blueprints/BP_Projectile_Spear_01.BP_Projectile_Spear_01_C|SetTarget%20Location _returnvalue_2 (Math|Vector|SelectVector (.Location (Collision|BreakHitResult _outhit)) (.TraceEnd (Collision|BreakHitResult _outhit)) (.bBlockingHit (Collision|BreakHitResult _outhit))))
      (Utilities|FlowControl|RetriggerableDelay 2.0)
      (goto _label))))

(event EventBeginPlay
  (bind _spawn_location (Variables|Default|GetSpawn%20Location))
  (bind _returnvalue (Transformation|GetWorldLocation _spawn_location))
  ;[1 1 1] Shot
  (bind _outhit (Collision|LineTraceForObjects _returnvalue (+ _returnvalue (* (Variables|Default|GetRange) (Math|Vector|GetForwardVector "0.000000,0.000000,1.000000"))) (Utilities|Array|MakeArray "ObjectTypeQuery1") false 0 "None" :!label _label))
  (Utilities|ForLoopwithDelay 0 9 0.1
    (:Loop%20Body
      (bind _returnvalue_2 (Game|SpawnActorfromClass "/Game/Common/FX_Sources/SourcePackage/ElementPrjtile_FX/Characters/Blueprints/BP_Projectile_Spear_01.BP_Projectile_Spear_01_C" (Math|Transform|MakeTransform (Transformation|GetWorldLocation (Variables|Default|GetSpawn%20Location)) (Camera|GetCameraRotation (Game|GetPlayerCameraManager 0)) "1.000000,1.000000,1.000000") "AdjustIfPossibleButAlwaysSpawn" "OverrideRootScale" 0 0))
      (Variables|/Game/Common/FX_Sources/SourcePackage/ElementPrjtile_FX/Characters/Blueprints/BP_Projectile_Spear_01.BP_Projectile_Spear_01_C|SetTarget%20Location _returnvalue_2 (Math|Vector|SelectVector (.Location (Collision|BreakHitResult _outhit)) (.TraceEnd (Collision|BreakHitResult _outhit)) (.bBlockingHit (Collision|BreakHitResult _outhit))))
      (Utilities|FlowControl|RetriggerableDelay 2.0)
      (goto _label))))

(fn ConstructionScript)