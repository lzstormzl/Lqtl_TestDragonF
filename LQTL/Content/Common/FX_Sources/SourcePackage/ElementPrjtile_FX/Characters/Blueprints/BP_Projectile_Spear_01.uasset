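; Spear projectile actor that flies a randomized curved path to TargetLocation with a Niagara effect.
; BeginPlay picks a random point along the line to the target and offsets it by a random radius and angle to form a control point.
; Tick slides that point toward the target while the actor chases it with a swept move, facing its travel direction.
; On collision or arrival it spawns the bullet-hit effect and destroys itself.
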(event OnComponentHit(SphereCollider)
  (params (HitComponent :type Primitive%20Component%20Object%20Reference) (OtherActor :type Actor%20Object%20Reference) (OtherComp :type Primitive%20Component%20Object%20Reference) (NormalImpulse :type Vector :default "0, 0, 0") (Hit :type Hit%20Result%20Structure%20%28by%20ref%29))
  (bind _sphere (Variables|Default|GetSphere))
  (Components|DestroyComponent (Variables|Default|GetSphere%20Collider))
  (Niagara|SpawnSystematLocation "/Game/Common/FX_Sources/SourcePackage/ElementPrjtile_FX/Effect/NiagaraSystems/MagicTrailBullet/NS_BulletHit_01.NS_BulletHit_01" (Transformation|GetWorldLocation _sphere) (Transformation|GetWorldRotation _sphere))
  (Components|DestroyComponent (Variables|Default|GetNewNiagaraSystem))
  (Actor|DestroyActor))

(event EventBeginPlay
  (bind _returnvalue (Transformation|GetActorLocation))
  (bind _sphere (Variables|Default|GetSphere))
  (Utilities|FlowControl|Delay 0.0)
  (CallFunction|MidPointCalculator)
  (CallFunction|CurveControlPoint)
  (Components|Activation|Activate (Variables|Default|GetNewNiagaraSystem) false)
  (Utilities|FlowControl|Gate true) ; enters at Open
)

(event EventTick
  (params (DeltaSeconds :type Float%20%28single-precision%29))
  (bind _returnvalue (Transformation|GetActorLocation))
  (bind _sphere (Variables|Default|GetSphere))
  (Utilities|FlowControl|Gate true
    (:Exit
      (if (Utilities|Operators|NotEqual(!=) (Transformation|GetActorLocation) (Variables|Default|GetTarget%20Location) 0.0)
        (Variables|Default|SetCurved%20Point (Math|Interpolation|VInterptoConstant (Variables|Default|GetCurved%20Point) (Variables|Default|GetTarget%20Location) (Utilities|Time|GetWorldDeltaSeconds) (Variables|Default|GetProjectile%20Speed)))
        (Transformation|SetActorLocation (Math|Interpolation|VInterptoConstant _returnvalue (Variables|Default|GetCurved%20Point) (Utilities|Time|GetWorldDeltaSeconds) (Variables|Default|GetProjectile%20Speed)) true false)
        (Transformation|SetActorRotation (Math|Rotator|FindLookatRotation _returnvalue (Math|Interpolation|VInterptoConstant _returnvalue (Variables|Default|GetCurved%20Point) (Utilities|Time|GetWorldDeltaSeconds) (Variables|Default|GetProjectile%20Speed))))
        (else
          (Components|DestroyComponent (Variables|Default|GetSphere%20Collider))
          (Niagara|SpawnSystematLocation "/Game/Common/FX_Sources/SourcePackage/ElementPrjtile_FX/Effect/NiagaraSystems/MagicTrailBullet/NS_BulletHit_01.NS_BulletHit_01" (Transformation|GetWorldLocation _sphere) (Transformation|GetWorldRotation _sphere))
          (Components|DestroyComponent (Variables|Default|GetNewNiagaraSystem))
          (Actor|DestroyActor))))))

(fn ConstructionScript)

(fn MidPointCalculator
  (Variables|Default|SetMidPoint (+ (* (- (Variables|Default|GetTarget%20Location) (Transformation|GetActorLocation)) (Math|Random|RandomFloatinRange (Variables|Default|GetMin%20Curve%20Point%20Distance) (Variables|Default|GetMax%20Curve%20Point%20Distance))) (Transformation|GetActorLocation))))

(fn CurveControlPoint
  (bind _midpoint (Variables|Default|GetMidPoint))
  (bind _target_location (Variables|Default|GetTarget%20Location))
  (bind _returnvalue (Math|Rotator|FindLookatRotation _midpoint _target_location))
  (bind (_x _y) (Math|Rotator|BreakRotIntoAxes _returnvalue))
  (Variables|Default|SetCurved%20Point (+ (Variables|Default|GetMidPoint) (Math|Vector|RotateVectorAroundAxis (* (Math|Random|RandomFloatinRange (Variables|Default|GetMin%20Curve%20Radius) (Variables|Default|GetMax%20Curve%20Radius)) _y) (Math|Random|RandomFloatinRange (Variables|Default|GetMin%20Angle) (Variables|Default|GetMax%20Angle)) _x))))