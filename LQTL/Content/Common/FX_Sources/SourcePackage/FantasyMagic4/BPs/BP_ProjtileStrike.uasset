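; Lightning projectile effect actor that homes in on a BP_ProjectileTarget actor and bursts on arrival.
; BeginPlay gathers the targets, and Tick moves the root at constant speed toward a point above the first one's mesh.
; On reaching that point it deactivates its Niagara effect, waits briefly, spawns a scaled-up lightning impact system and destroys itself.
; Movement has no sweep or collision test; arrival is detected purely by position comparison.
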(event Custom|Impact
  (Niagara|SpawnSystematLocation "/Game/Common/FX_Sources/SourcePackage/FantasyMagic4/PS/FX_LightningProjImpact.FX_LightningProjImpact" (Transformation|GetWorldLocation (Variables|Default|GetNiagara)) "0, 0, 0" "2.000000,2.000000,2.000000"))

(event EventBeginPlay
  (bind _outactors (Actor|GetAllActorsOfClass "/Game/Common/FX_Sources/SourcePackage/FantasyMagic4/BPs/BP_ProjectileTarget.BP_ProjectileTarget_C")))

(event Collision|EventActorBeginOverlap
  (params (OtherActor :type Actor%20Object%20Reference)))

(event EventTick
  (params (DeltaSeconds :type Float%20%28single-precision%29))
  (bind _defaultsceneroot (Variables|Default|GetDefaultSceneRoot))
  (bind _returnvalue (Transformation|GetWorldLocation _defaultsceneroot))
  (Transformation|SetWorldLocation _defaultsceneroot (Math|Interpolation|VInterptoConstant _returnvalue (+ (Transformation|GetWorldLocation (Variables|/Game/Common/FX_Sources/SourcePackage/FantasyMagic4/BPs/BP_ProjectileTarget.BP_ProjectileTarget_C|GetStaticMesh (Utilities|Array|Get(acopy) (stale EventBeginPlay _outactors)))) "0, 0,150.000000") (Math|Float|Fraction DeltaSeconds) 1e+03) false false)
  (if (Math|Vector|Equal(Vector) _returnvalue (+ (Transformation|GetWorldLocation (Variables|/Game/Common/FX_Sources/SourcePackage/FantasyMagic4/BPs/BP_ProjectileTarget.BP_ProjectileTarget_C|GetStaticMesh (Utilities|Array|Get(acopy) (stale EventBeginPlay _outactors)))) "0, 0,150.000000") 0.0001)
    (Components|Activation|Deactivate (Variables|Default|GetNiagara))
    (Utilities|FlowControl|Delay 0.2)
    (Utilities|FlowControl|Sequence
      (:then_0
        (CallFunction|Impact))
      (:then_1
        (Actor|DestroyActor)))))

(fn ConstructionScript)