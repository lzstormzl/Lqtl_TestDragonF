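; Demo button Blueprint with two overlap-triggered pads that reset or hide a referenced actor.
; Construction caches the actor's class and transform and creates dynamic materials for button feedback.
; The reset pad flip-flops on overlap begin and end, respawning the actor by replacing it.
; The hide pad's timeline, also played on BeginPlay, animates the press, then alternates hiding with showing and respawning.
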(event OnComponentBeginOverlap(Triggercollisionhide)
  (params (OverlappedComponent :type Primitive%20Component%20Object%20Reference) (OtherActor :type Actor%20Object%20Reference) (OtherComp :type Primitive%20Component%20Object%20Reference) (OtherBodyIndex :type Integer) (bFromSweep :type Boolean) (SweepResult :type Hit%20Result%20Structure%20%28by%20ref%29))
  (bind _button_hide_material (Variables|Default|GetButton%20Hide%20material))
  (bind (_direction _press _colour) (Timeline|Timeline PlayFromStart)
    (:Update
      (Transformation|SetRelativeScale3D (Variables|Default|GetButton%20Hide%20Floor) (Math|Conversions|ToVector(Float) _press))
      (Rendering|Material|SetVectorParameterValue (Variables|Default|GetButton%20Hide%20material) "Colour" _colour :!class /Script/Engine.MaterialInstanceDynamic))
    (:Finished
      (Utilities|FlowControl|FlipFlop
        (:A
          (Rendering|SetActorHiddenInGame (Variables|Default|GetActor%20to%20spawn) true)
          (Rendering|Material|SetVectorParameterValue _button_hide_material "Colour" "(R=1.000000,G=0.000000,B=0.000000,A=1.000000)" :!class /Script/Engine.MaterialInstanceDynamic))
        (:B
          (Rendering|SetActorHiddenInGame (Variables|Default|GetActor%20to%20spawn) false)
          (Rendering|Material|SetVectorParameterValue _button_hide_material "Colour" "(R=0.000000,G=1.000000,B=0.000000,A=1.000000)" :!class /Script/Engine.MaterialInstanceDynamic)
          (bind _returnvalue (Game|SpawnActorfromClass (Variables|Default|Getclass%20target) (Variables|Default|Gettransf%20target) "Undefined" "SelectDefaultAtRuntime" (Variables|Default|GetActor%20to%20spawn) 0))
          (Actor|DestroyActor (Variables|Default|GetActor%20to%20spawn))
          (Variables|Default|SetActor%20to%20spawn _returnvalue))))))

(event OnComponentBeginOverlap(Triggercollisionreset)
  (params (OverlappedComponent :type Primitive%20Component%20Object%20Reference) (OtherActor :type Actor%20Object%20Reference) (OtherComp :type Primitive%20Component%20Object%20Reference) (OtherBodyIndex :type Integer) (bFromSweep :type Boolean) (SweepResult :type Hit%20Result%20Structure%20%28by%20ref%29))
  (bind _button_reset_material (Variables|Default|GetButton%20Reset%20material))
  (Utilities|FlowControl|FlipFlop
    (:A
      (Rendering|Material|SetScalarParameterValue _button_reset_material "State" 1.0 :!class /Script/Engine.MaterialInstanceDynamic) ; Change a scalar value in the button material that turns it green
      (Rendering|Material|SetVectorParameterValue (Variables|Default|GetButton%20Hide%20material) "Colour" "(R=0.000000,G=1.000000,B=0.000000,A=1.000000)" :!class /Script/Engine.MaterialInstanceDynamic)
      (bind _returnvalue (Game|SpawnActorfromClass (Variables|Default|Getclass%20target) (Variables|Default|Gettransf%20target) "Undefined" "SelectDefaultAtRuntime" (Variables|Default|GetActor%20to%20spawn) 0))
      (Actor|DestroyActor (Variables|Default|GetActor%20to%20spawn))
      (Variables|Default|SetActor%20to%20spawn _returnvalue))
    (:B
      (Rendering|Material|SetScalarParameterValue _button_reset_material "State" 0.0 :!class /Script/Engine.MaterialInstanceDynamic))))

(event OnComponentEndOverlap(Triggercollisionreset)
  (params (OverlappedComponent :type Primitive%20Component%20Object%20Reference) (OtherActor :type Actor%20Object%20Reference) (OtherComp :type Primitive%20Component%20Object%20Reference) (OtherBodyIndex :type Integer))
  (bind _button_reset_material (Variables|Default|GetButton%20Reset%20material))
  (Utilities|FlowControl|FlipFlop
    (:A
      (Rendering|Material|SetScalarParameterValue _button_reset_material "State" 1.0 :!class /Script/Engine.MaterialInstanceDynamic) ; Change a scalar value in the button material that turns it green
      (Rendering|Material|SetVectorParameterValue (Variables|Default|GetButton%20Hide%20material) "Colour" "(R=0.000000,G=1.000000,B=0.000000,A=1.000000)" :!class /Script/Engine.MaterialInstanceDynamic)
      (bind _returnvalue (Game|SpawnActorfromClass (Variables|Default|Getclass%20target) (Variables|Default|Gettransf%20target) "Undefined" "SelectDefaultAtRuntime" (Variables|Default|GetActor%20to%20spawn) 0))
      (Actor|DestroyActor (Variables|Default|GetActor%20to%20spawn))
      (Variables|Default|SetActor%20to%20spawn _returnvalue))
    (:B
      (Rendering|Material|SetScalarParameterValue _button_reset_material "State" 0.0 :!class /Script/Engine.MaterialInstanceDynamic))))

(event EventBeginPlay
  (bind _button_hide_material (Variables|Default|GetButton%20Hide%20material))
  (bind (_direction _press _colour) (Timeline|Timeline PlayFromStart)
    (:Update
      (Transformation|SetRelativeScale3D (Variables|Default|GetButton%20Hide%20Floor) (Math|Conversions|ToVector(Float) _press))
      (Rendering|Material|SetVectorParameterValue (Variables|Default|GetButton%20Hide%20material) "Colour" _colour :!class /Script/Engine.MaterialInstanceDynamic))
    (:Finished
      (Utilities|FlowControl|FlipFlop
        (:A
          (Rendering|SetActorHiddenInGame (Variables|Default|GetActor%20to%20spawn) true)
          (Rendering|Material|SetVectorParameterValue _button_hide_material "Colour" "(R=1.000000,G=0.000000,B=0.000000,A=1.000000)" :!class /Script/Engine.MaterialInstanceDynamic))
        (:B
          (Rendering|SetActorHiddenInGame (Variables|Default|GetActor%20to%20spawn) false)
          (Rendering|Material|SetVectorParameterValue _button_hide_material "Colour" "(R=0.000000,G=1.000000,B=0.000000,A=1.000000)" :!class /Script/Engine.MaterialInstanceDynamic)
          (bind _returnvalue (Game|SpawnActorfromClass (Variables|Default|Getclass%20target) (Variables|Default|Gettransf%20target) "Undefined" "SelectDefaultAtRuntime" (Variables|Default|GetActor%20to%20spawn) 0))
          (Actor|DestroyActor (Variables|Default|GetActor%20to%20spawn))
          (Variables|Default|SetActor%20to%20spawn _returnvalue))))))

(fn ConstructionScript
  (bind _actor_to_spawn (Variables|Default|GetActor%20to%20spawn))
  (Utilities|FlowControl|Sequence
    (:then_0
      (bind _returnvalue (Rendering|Material|CreateDynamicMaterialInstance (Variables|Default|GetButton%20Reset) 1 0 "None" :!class /Script/Engine.PrimitiveComponent))
      (Variables|Default|SetButton%20Reset%20material _returnvalue))
    (:then_1
      (bind _returnvalue_2 (Rendering|Material|CreateDynamicMaterialInstance (Variables|Default|GetButton%20Hide%20Floor) 0 0 "None" :!class /Script/Engine.PrimitiveComponent))
      (bind _returnvalue_3 (Rendering|Material|CreateDynamicMaterialInstance (Variables|Default|GetButton%20Hide%20Top) 0 _returnvalue_2 "None" :!class /Script/Engine.PrimitiveComponent))
      (bind _output_get (Variables|Default|SetButton%20Hide%20material _returnvalue_3))
      (Rendering|Material|SetVectorParameterValue _output_get "Colour" "(R=0.000000,G=1.000000,B=0.000000,A=1.000000)" :!class /Script/Engine.MaterialInstanceDynamic))
    (:then_2
      (Variables|Default|Setclass%20target (Utilities|GetClass _actor_to_spawn))
      (Variables|Default|Settransf%20target (Transformation|GetActorTransform _actor_to_spawn)))))