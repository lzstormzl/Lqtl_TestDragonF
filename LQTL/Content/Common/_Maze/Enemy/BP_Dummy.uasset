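; BP_Dummy is a dummy enemy in the Maze folder that plays hit reactions.
; HitReact plays one of two randomly chosen get-hit montages on its mesh.
; A TakingDamaged flag and a short delay gate the event, so repeated hits are ignored until the flag resets.
; It has no other active logic, and no health or damage values are handled here.
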(event Custom|HitReact
  ;[1 1 1 1 90] Play Hit-React
  (if (not (Variables|Default|GetTakingDamaged?))
    (Variables|Default|SetTakingDamaged? true)
    (Animation|Montage|PlayMontage (Variables|Character|GetMesh) (Utilities|Select :Index (Math|Random|RandomIntegerinRange 0 1) :Option%200 (Variables|Montage_Child|GetGetHit_Opt0) :Option%201 (Variables|Montage_Child|GetGetHit_Opt1))
      (:then
        (Utilities|FlowControl|Delay 0.5)
        (Variables|Default|SetTakingDamaged? false)))))

(event EventBeginPlay)

(event Collision|EventActorBeginOverlap
  (params (OtherActor :type Actor%20Object%20Reference)))

(event EventTick
  (params (DeltaSeconds :type Float%20%28single-precision%29)))

(fn ConstructionScript)