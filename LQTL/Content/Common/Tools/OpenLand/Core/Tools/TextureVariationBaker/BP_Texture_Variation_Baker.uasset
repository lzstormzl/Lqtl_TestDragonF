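; Editor tool Blueprint that bakes a noise texture for texture variation into a static Texture2D asset.
; Update Render Target sets scale, band count and random seed on a dynamic instance of M_Texture_Variation_Baker and draws it into RT_TV_Baked_Noise.
; Bake Texture refreshes that render target, then saves it as a mipmap-free texture at the configured location and name, using the chosen compression.
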(event EventBeginPlay)

(event Collision|EventActorBeginOverlap
  (params (OtherActor :type Actor%20Object%20Reference)))

(event EventTick
  (params (DeltaSeconds :type Float%20%28single-precision%29)))

(fn ConstructionScript)

(fn UpdateRenderTarget
  (bind _returnvalue (Rendering|Material|CreateDynamicMaterialInstance "/Game/Common/Tools/OpenLand/Core/Tools/TextureVariationBaker/M_Texture_Variation_Baker.M_Texture_Variation_Baker" "None" "None" :!class /Script/Engine.KismetMaterialLibrary))
  (Rendering|Material|SetScalarParameterValue _returnvalue "Variation Scale" (Variables|1.Variations|GetVariation%20Scale) :!class /Script/Engine.MaterialInstanceDynamic)
  (Rendering|Material|SetScalarParameterValue _returnvalue "Variation Bands" (Math|Conversions|ToFloat(Integer) (Variables|1.Variations|GetVariation%20Bands)) :!class /Script/Engine.MaterialInstanceDynamic)
  (Rendering|Material|SetScalarParameterValue _returnvalue "Random Seed" (Variables|1.Variations|GetRandom%20Seed) :!class /Script/Engine.MaterialInstanceDynamic)
  (Rendering|DrawMaterialtoRenderTarget "/Game/Common/Tools/OpenLand/Core/Materials/Functions/TextureVariations/RT_TV_Baked_Noise.RT_TV_Baked_Noise" _returnvalue))

(fn BakeTexture
  (1.Variations|UpdateRenderTarget)
  (Class|KismetRenderingLibrary|RenderTargetCreateStaticTexture2DEditorOnly "/Game/Common/Tools/OpenLand/Core/Materials/Functions/TextureVariations/RT_TV_Baked_Noise.RT_TV_Baked_Noise" (Utilities|String|ToString(Text) (Utilities|Text|FormatText "{Location}/{Name}" (Variables|2.Baking|GetTexture%20Location) (Variables|2.Baking|GetTexture%20Name))) (Variables|2.Baking|GetCompression%20Settings) "TMGS_NoMipmaps"))