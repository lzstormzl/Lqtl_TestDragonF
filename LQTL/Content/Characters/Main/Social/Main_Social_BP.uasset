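; Player character for the social mode, handling NPC interaction, social stats, companions and an overhead text tooltip.
; Overlapping NPC-tagged actors feed the interact widget, and the Interact input messages the current InteractNPC.
; Stats initialize from a data table, support clamped changes and condition checks, and persist with the companion list through GameInstance save data.
; Companions spawn or despawn with stat bonuses, while hotkeys open menus, advance calendar phases, toggle flying and possess BP_TieuQuy.
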(event OnComponentBeginOverlap(InteractCheck)
  (params (OverlappedComponent :type Primitive%20Component%20Object%20Reference) (OtherActor :type Actor%20Object%20Reference) (OtherComp :type Primitive%20Component%20Object%20Reference) (OtherBodyIndex :type Integer) (bFromSweep :type Boolean) (SweepResult :type Hit%20Result%20Structure%20%28by%20ref%29))
  (if (and (Actor|ActorHasTag OtherActor "NPC") (Variables|Default|GetIsPlayerControlling?))
    (Variables|Widgets|GetInteractSequenceWidget
      (:then
        _)
      (:else
        (bind _returnvalue (UserInterface|CreateWidget "/Game/GeneralSocial/2_GameSystems/3_InteractSystem/WBP_InteractSequence.WBP_InteractSequence_C"))
        (Variables|Widgets|SetInteractSequenceWidget _returnvalue)))
    (Default|UpdateInteractWidget (Variables|Widgets|GetInteractSequenceWidget) OtherActor)))

(event OnComponentEndOverlap(InteractCheck)
  (params (OverlappedComponent :type Primitive%20Component%20Object%20Reference) (OtherActor :type Actor%20Object%20Reference) (OtherComp :type Primitive%20Component%20Object%20Reference) (OtherBodyIndex :type Integer))
  (if (and (Actor|ActorHasTag OtherActor "NPC") (Variables|Default|GetIsPlayerControlling?))
    (bind _interactsequencewidget (Variables|Widgets|GetInteractSequenceWidget)
      (:then
        (Default|RemoveInteract _interactsequencewidget OtherActor))
      (:else))))

(event Custom|SetIsInteracting_1
  (params (IsInteracting :type Boolean))
  (Variables|Default|SetIsInteracting IsInteracting))

(event Input|EnhancedActionEvents|EnhancedInputActionIA_Interact
  (params (ActionValue :type Boolean) (ElapsedSeconds :type Float%20%28double-precision%29) (TriggeredSeconds :type Float%20%28double-precision%29) (InputAction :type Input%20Action%20Object%20Reference :default "/Game/GeneralSocial/1_Social/5_Input/Actions/IA_Interact.IA_Interact"))
  (:Started
    (Utilities|FlowControl|DelayUntilNextTick)
    (if (not (Variables|Default|GetIsInteracting))
      (bind _interactnpc (Variables|Default|GetInteractNPC)
        (:then
          (Class|BPIInteraction|Interact(Message) _interactnpc))
        (:else)))))

(event Input|EnhancedActionEvents|EnhancedInputActionIA_Jump
  (params (ActionValue :type Boolean) (ElapsedSeconds :type Float%20%28double-precision%29) (TriggeredSeconds :type Float%20%28double-precision%29) (InputAction :type Input%20Action%20Object%20Reference :default "/Game/GeneralSocial/1_Social/5_Input/Actions/IA_Jump.IA_Jump"))
  (bind _returnvalue (Game|GetPlayerCharacter 0))
  (bind _returnvalue_2 (Transformation|GetActorForwardVector _returnvalue))
  (bind (_x _y) (Math|Vector|BreakVector _returnvalue_2))
  (Pawn|Input|AddMovementInput (Game|GetPlayerCharacter 0) (Math|Vector|MakeVector _x _y 1e+02) (Math|Conversions|ToFloat(Boolean) ActionValue) false))

(event EventDisablePlayerTooltip
  (Rendering|SetVisibility (Variables|Default|GetWidget) false false))

(event EventShowPlayerTooltip
  (params (Text :type Text))
  (bind _widget (Variables|Default|GetWidget))
  (Rendering|SetVisibility _widget true false)
  (bind _asw_text_in_head (Utilities|Casting|CastToW_TextInHead (UserInterface|GetWidget _widget)))
  (Variables|/Script/UMG.TextBlock|SetText (Variables|/Game/GeneralSocial/1_Social/3_Characters/1_Player/W_TextInHead.W_TextInHead_C|GetTextBlock_24 _asw_text_in_head) Text))

(event EventBeginPlay
  (Utilities|FlowControl|Delay 0.3)
  (bind _asthuy_tinh_social_game_mode (Utilities|Casting|CastToThuyTinh_Social_GameMode (Game|GetGameMode)))
  (Variables|Default|SetThuy%20Tinh%20Social%20Game%20Mode _asthuy_tinh_social_game_mode)
  (Rendering|SetVisibility (Variables|Default|GetWidget) false false)
  (Save/Load|Load|LoadSocialPlayerData))

(event Input|KeyboardEvents|DebugKeyR
  (params (Key :type Key%20Structure) (ActionValue :type Input%20Action%20Value%20Structure))
  (:Pressed
    (bind _returnvalue (Actor|GetActorOfClass "/Game/GeneralSocial/1_Social/3_Characters/1_Player/BP_TieuQuy.BP_TieuQuy_C"))
    (Utilities|IsValid _returnvalue
      (:Is%20Valid
        (Pawn|Possess (Game|GetPlayerController 0) _returnvalue)
        (Variables|/Game/GeneralSocial/1_Social/3_Characters/1_Player/BP_TieuQuy.BP_TieuQuy_C|SetIsPlayerControlling? _returnvalue true))
      (:Is%20Not%20Valid
        (bind _returnvalue_2 (Game|SpawnActorfromClass "/Game/GeneralSocial/1_Social/3_Characters/1_Player/BP_TieuQuy.BP_TieuQuy_C" (Math|Transform|MakeTransform (Transformation|GetActorLocation (CallFunction|GetPlayerCharacterSocial)) "0, 0, 0" "1.000000,1.000000,1.000000") "Undefined" "MultiplyWithRoot" 0 0))
        (Variables|/Game/GeneralSocial/1_Social/3_Characters/1_Player/BP_TieuQuy.BP_TieuQuy_C|SetIsPlayerControlling? _returnvalue_2 true)
        (Pawn|Possess (Game|GetPlayerController 0) _returnvalue_2)))
    (Variables|/Game/GeneralSocial/1_Social/ThuyTinh_Social_GameMode.ThuyTinh_Social_GameMode_C|SetCharacterPlayerControlling (CallFunction|GetSocialGameMode) "NewEnumerator1")
    (Variables|Default|SetIsPlayerControlling? false)
    (bind _interactsequencewidget (Variables|Widgets|GetInteractSequenceWidget)
      (:then
        (Default|TurnOffInteract _interactsequencewidget))
      (:else))))

(event Input|KeyboardEvents|DebugKeyZ
  (params (Key :type Key%20Structure) (ActionValue :type Input%20Action%20Value%20Structure))
  (:Pressed
    (bind _returnvalue (UserInterface|CreateWidget "/Game/GeneralSocial/1_Social/Minigame-Resources/Cooking/W_Cooking.W_Cooking_C"))
    (UserInterface|Viewport|AddtoViewport _returnvalue 0)))

(event Input|KeyboardEvents|DebugKeyX
  (params (Key :type Key%20Structure) (ActionValue :type Input%20Action%20Value%20Structure))
  (bind _charactermovement (Variables|Character|GetCharacterMovement))
  (:Pressed
    (Utilities|FlowControl|FlipFlop
      (:A
        (Pawn|Components|CharacterMovement|SetMovementMode _charactermovement "MOVE_Flying" 0))
      (:B
        (Pawn|Components|CharacterMovement|SetMovementMode _charactermovement "MOVE_Walking" 0)))))

(event Input|KeyboardEvents|V
  (params (Key :type Key%20Structure))
  (bind _returnvalue (Game|GetPlayerController 0))
  (:Pressed
    (Variables|Widgets|GetCompanionSelectWidget
      (:then
        (UserInterface|Viewport|AddtoViewport (Variables|Widgets|GetCompanionSelectWidget) 0))
      (:else
        (bind _returnvalue_2 (UserInterface|CreateWidget "/Game/GeneralSocial/2_GameSystems/9_Companion/W_CompanionSelecet.W_CompanionSelecet_C"))
        (Variables|Widgets|SetCompanionSelectWidget _returnvalue_2)
        (UserInterface|Viewport|AddtoViewport (Variables|Widgets|GetCompanionSelectWidget) 0)))
    (Input|SetInputModeUIOnly _returnvalue (Variables|Widgets|GetCompanionSelectWidget) "DoNotLock" false)
    (Variables|/Script/Engine.PlayerController|SetbShowMouseCursor _returnvalue true)))

(event Input|KeyboardEvents|M
  (params (Key :type Key%20Structure))
  (bind _returnvalue (Game|GetPlayerController 0))
  (:Pressed
    (Variables|Widgets|GetStatsWidget
      (:then
        (UserInterface|Viewport|AddtoViewport (Variables|Widgets|GetStatsWidget) 0))
      (:else
        (bind _returnvalue_2 (UserInterface|CreateWidget "/Game/GeneralSocial/1_Social/WBP_StatsActionTest.WBP_StatsActionTest_C"))
        (bind _output_get (Variables|Widgets|SetStatsWidget _returnvalue_2))
        (UserInterface|Viewport|AddtoViewport _output_get 0)))
    (Input|SetInputModeUIOnly _returnvalue _returnvalue_2 "DoNotLock" false)
    (Variables|/Script/Engine.PlayerController|SetbShowMouseCursor _returnvalue true)))

(event Input|KeyboardEvents|L
  (params (Key :type Key%20Structure))
  (:Pressed
    (Default|StartMorningClassroom (CallFunction|GetCalendarManager self))))

(event Input|KeyboardEvents|T
  (params (Key :type Key%20Structure))
  (bind _returnvalue (Game|GetPlayerController 0))
  (bind _schedulemanager (CallFunction|GetScheduleManager))
  (bind _schedulewidget (Variables|/Game/GeneralSocial/2_GameSystems/ScheduleNActionSystem/BP_ScheduleManager.BP_ScheduleManager_C|GetScheduleWidget _schedulemanager))
  (:Pressed
    (UserInterface|Viewport|AddtoViewport _schedulewidget 0)
    (Variables|/Script/Engine.PlayerController|SetbShowMouseCursor _returnvalue true)
    (Input|SetInputModeUIOnly _returnvalue _schedulewidget "DoNotLock" false)))

(event Input|KeyboardEvents|1
  (params (Key :type Key%20Structure))
  (:Pressed
    (Default|AdvancedPhasewithTransition (CallFunction|GetCalendarManager self))))

(event Input|KeyboardEvents|DebugKeyI
  (params (Key :type Key%20Structure :default "None") (ActionValue :type Input%20Action%20Value%20Structure))
  (bind _thuy_tinh_social_game_mode (Variables|Default|GetThuy%20Tinh%20Social%20Game%20Mode))
  (bind _calendarmanager (Variables|/Game/GeneralSocial/1_Social/ThuyTinh_Social_GameMode.ThuyTinh_Social_GameMode_C|GetCalendarManager _thuy_tinh_social_game_mode))
  (bind _schedule_widget (Default|GetScheduleWidget _calendarmanager))
  (:Pressed
    (Utilities|FlowControl|FlipFlop
      (:A
        (UserInterface|Viewport|AddtoViewport _schedule_widget 0))
      (:B
        (Widget|RemovefromParent _schedule_widget)))))

(event Input|KeyboardEvents|DebugKeyX
  (params (Key :type Key%20Structure :default "None") (ActionValue :type Input%20Action%20Value%20Structure))
  (:Pressed
    (Default|StartNextPhase (CallFunction|GetSocialGameMode self))))

(event Input|KeyboardEvents|DebugKeyQ
  (params (Key :type Key%20Structure :default "None") (ActionValue :type Input%20Action%20Value%20Structure))
  (bind _thuy_tinh_social_game_mode (Variables|Default|GetThuy%20Tinh%20Social%20Game%20Mode))
  (bind _questjournal (Variables|/Game/GeneralSocial/1_Social/ThuyTinh_Social_GameMode.ThuyTinh_Social_GameMode_C|GetQuestJournal _thuy_tinh_social_game_mode))
  ;[0 0 0] Bật quest journal
  (:Pressed
    (Utilities|FlowControl|FlipFlop
      (:A
        (UserInterface|Viewport|AddtoViewport _questjournal 0))
      (:B
        (Widget|RemovefromParent _questjournal)))))

(fn ConstructionScript
  (Initialize|InitializePlayerStats))

(fn TraceInteract
  (params (Range :type Float%20%28single-precision%29))
  (bind _returnvalue (Transformation|GetActorLocation))
  (bind _outhit (Collision|LineTraceForObjects _returnvalue (+ _returnvalue (* (Transformation|GetActorForwardVector) Range)) (Utilities|Array|MakeArray "ObjectTypeQuery3" "ObjectTypeQuery2") false 0 "ForOneFrame"))
  (if (Utilities|DoesObjectImplementInterface (.HitActor (Collision|BreakHitResult _outhit)) "/Game/GeneralSocial/2_GameSystems/3_InteractSystem/BPI_Interaction.BPI_Interaction_C")
    (Class|BPIInteraction|Interact(Message) (.HitActor (Collision|BreakHitResult _outhit)))))

(fn SaveSocialPlayerData
  (bind _gamedata (Class|BPISaveGame|GetSaveGameData(Message) (Game|GetGameInstance)))
  (Variables|/Game/GeneralSocial/2_GameSystems/4_SaveLoadSystem/BP_SaveGame.BP_SaveGame_C|SetPlayerSocialDataSave _gamedata (Utilities|Struct|MakePlayerSocialSaveData (Variables|Stats|GetPlayerSocialStats) (Variables|Default|GetCompanionFollow))))

(fn LoadSocialPlayerData
  (bind _gamedata (Class|BPISaveGame|GetSaveGameData(Message) (Game|GetGameInstance)))
  (Utilities|IsValid _gamedata
    (:Is%20Valid
      (Utilities|FlowControl|Sequence
        (:then_0
          (if (Utilities|Map|IsNotEmpty (.playerstats (Variables|/Game/GeneralSocial/2_GameSystems/4_SaveLoadSystem/BP_SaveGame.BP_SaveGame_C|GetPlayerSocialDataSave _gamedata)))
            (Variables|Stats|SetPlayerSocialStats (.playerstats (Variables|/Game/GeneralSocial/2_GameSystems/4_SaveLoadSystem/BP_SaveGame.BP_SaveGame_C|GetPlayerSocialDataSave _gamedata)))))
        (:then_1
          (Variables|Default|SetCompanionFollow (.companionsfollow (Variables|/Game/GeneralSocial/2_GameSystems/4_SaveLoadSystem/BP_SaveGame.BP_SaveGame_C|GetPlayerSocialDataSave _gamedata))))))))

(fn InitializePlayerStats
  (bind _outrownames (DataTable|GetDataTableRowNames "/Game/GeneralSocial/Config/DataTableConfig/Player/social_stats_definition_DT.social_stats_definition_DT"))
  (for _array_element _outrownames
    (bind _returnvalue (Utilities|GetDataTableRow "/Game/GeneralSocial/Config/DataTableConfig/Player/social_stats_definition_DT.social_stats_definition_DT" _array_element)
      (:then
        (Utilities|Map|Add (Variables|Stats|GetPlayerSocialStats) _array_element (Utilities|Struct|MakePlayerStatStruct (.DisplayName (Utilities|Struct|Breaksocial_stats_definition_struct _returnvalue)) 0 (.MinValue (Utilities|Struct|Breaksocial_stats_definition_struct _returnvalue)) (.MaxValue (Utilities|Struct|Breaksocial_stats_definition_struct _returnvalue))))))))

(fn PlusPlayerStat
  (params (StatKeyName :type Name%20%28by%20ref%29) (Amount :type Integer))
  (bind _playersocialstats (Variables|Stats|GetPlayerSocialStats))
  (bind _value (Utilities|Map|Find _playersocialstats StatKeyName))
  (LocalVariables|SetDisplayName (.displayname _value))
  (LocalVariables|SetValue (.value _value))
  (LocalVariables|SetMinValue (.minvalue _value))
  (LocalVariables|SetMaxValue (.maxvalue _value))
  (if (> (+ (LocalVariables|GetValue) Amount) (LocalVariables|GetMaxValue))
    (Utilities|Map|Add (Variables|Stats|GetPlayerSocialStats) StatKeyName (Utilities|Struct|MakePlayerStatStruct (LocalVariables|GetDisplayName) (LocalVariables|GetMaxValue) (LocalVariables|GetMinValue) (LocalVariables|GetMaxValue)))
    (elif (< (+ (LocalVariables|GetValue) Amount) (LocalVariables|GetMinValue))
      (Utilities|Map|Add (Variables|Stats|GetPlayerSocialStats) StatKeyName (Utilities|Struct|MakePlayerStatStruct (LocalVariables|GetDisplayName) (LocalVariables|GetMinValue) (LocalVariables|GetMinValue) (LocalVariables|GetMaxValue)))
      (else
        (Utilities|Map|Add (Variables|Stats|GetPlayerSocialStats) StatKeyName (Utilities|Struct|MakePlayerStatStruct (LocalVariables|GetDisplayName) (+ (LocalVariables|GetValue) Amount) (LocalVariables|GetMinValue) (LocalVariables|GetMaxValue)))))))

(fn SetPlayerStat
  (params (StatID :type Name) (Amount :type Integer))
  (bind _playersocialstats (Variables|Stats|GetPlayerSocialStats))
  (bind _value (Utilities|Map|Find _playersocialstats StatID))
  (Utilities|Map|Add _playersocialstats StatID (Utilities|Struct|MakePlayerStatStruct (.displayname _value) Amount (.minvalue _value) (.maxvalue _value))))

(fn RecoveryPlayerActionPoint
  (bind _playersocialstats (Variables|Stats|GetPlayerSocialStats))
  (bind _value (Utilities|Map|Find _playersocialstats "Energy"))
  (Utilities|Map|Add _playersocialstats "Energy" (Utilities|Struct|MakePlayerStatStruct (.displayname _value) (.maxvalue _value) (.minvalue _value) (.maxvalue _value))))

(fn GetSocialPlayerStat
  (params (StatID :type Name))
  (return (.Value (Utilities|Map|Find (Variables|Stats|GetPlayerSocialStats) StatID))))

(fn CheckPlayerStatsArray
  (params (PlayerStats :type Array%20of%20F%20Check%20Player%20Stat%20Structures))
  (for _array_element PlayerStats
    (bind _returnvalue (CallFunction|CheckPlayerStats (.StatID (Utilities|Struct|BreakF_CheckPlayerStat _array_element)) (.> (Utilities|Struct|BreakF_CheckPlayerStat _array_element)) (.None (Utilities|Struct|BreakF_CheckPlayerStat _array_element)) (.< (Utilities|Struct|BreakF_CheckPlayerStat _array_element)) (.Amount (Utilities|Struct|BreakF_CheckPlayerStat _array_element))))
    (if (not _returnvalue)
      (return false)))
  (return true))

(fn CheckPlayerStats
  (params (StatKeyName :type Name :default "None") (> :type Boolean) (= :type Boolean) (< :type Boolean) (Amount :type Integer))
  (if (Math|Boolean|ANDBoolean (not >) (not =) (not <))
    (return true)
    (elif (and > =)
      (return (>= (Utilities|Struct|BreakPlayerStatStruct (.Value (Utilities|Map|Find (Variables|Stats|GetPlayerSocialStats) StatKeyName))) Amount))
      (elif (and < =)
        (return (<= (Utilities|Struct|BreakPlayerStatStruct (.Value (Utilities|Map|Find (Variables|Stats|GetPlayerSocialStats) StatKeyName))) Amount))
        (elif >
          (return (> (Utilities|Struct|BreakPlayerStatStruct (.Value (Utilities|Map|Find (Variables|Stats|GetPlayerSocialStats) StatKeyName))) Amount))
          (elif =
            (return (== (Utilities|Struct|BreakPlayerStatStruct (.Value (Utilities|Map|Find (Variables|Stats|GetPlayerSocialStats) StatKeyName))) Amount))
            (elif <
              (return (< (Utilities|Struct|BreakPlayerStatStruct (.Value (Utilities|Map|Find (Variables|Stats|GetPlayerSocialStats) StatKeyName))) Amount))
              (else
                (return false)))))))))

(event Custom|SpawnCompanion
  (params (CompanionClass :type BP%20Companion%20Base%20Class%20Reference))
  (bind _returnvalue (Game|GetPlayerCharacter 0))
  ;[0.08204 0.1788 1] Spawn Companion
  ;;[0 0 0] Kiểm tra component có đang tồn tại trên thế giới không?
  (bind _returnvalue_2 (Actor|GetActorOfClass CompanionClass))
  (Utilities|IsValid _returnvalue_2
    (:Is%20Valid
      ;;[0 0 0] Nếu có thì set vị trí companion đấy tới chỗ người chơi và trao controller cho nó. Bỏ nó vào list những companion đang sử dụng
      (Transformation|SetActorLocationAndRotation _returnvalue_2 (Transformation|GetActorLocation _returnvalue) (Transformation|GetActorRotation _returnvalue))
      (Pawn|SpawnDefaultController _returnvalue_2)
      (Utilities|Array|AddUnique (Variables|Default|GetCompanionFollow) CompanionClass)
      (Default|PlusCompanionStat _returnvalue_2))
    (:Is%20Not%20Valid
      ;;[0 0 0] Nếu không thì spawn Companion ra chỗ vị trí của người chơi, trao controller và thêm vào list những component đang sử dụng
      (bind _returnvalue_3 (Game|SpawnActorfromClass CompanionClass (Transformation|GetActorTransform (Game|GetPlayerCharacter 0)) "AdjustIfPossibleButAlwaysSpawn" "MultiplyWithRoot" 0 "None" "" 0 0 0 0))
      (Pawn|SpawnDefaultController _returnvalue_3)
      (Utilities|Array|AddUnique (Variables|Default|GetCompanionFollow) CompanionClass)
      (Default|PlusCompanionStat _returnvalue_3))))

(event Custom|DespawnCompanion
  (params (Companion :type BP%20Companion%20Base%20Class%20Reference) (TeleToNextMap :type Boolean))
  (if (Utilities|Array|ContainsItem (Variables|Default|GetCompanionFollow) Companion)
    (if TeleToNextMap
      _
      (else
        (Utilities|Array|RemoveItem (Variables|Default|GetCompanionFollow) Companion)))
    (bind _returnvalue (Actor|GetActorOfClass Companion))
    (Utilities|IsValid _returnvalue
      (:Is%20Valid
        (Default|MinusCompanionStat _returnvalue)
        (Actor|DestroyActor _returnvalue)))
    (else
      (Development|PrintString "Không despawn được vì không tìm thấy Actor trong list Companion Follow"))))

(event EventPlusPlayerStats
  (params (StatKey :type Name :default "None") (Amount :type Integer))
  (CallFunction|PlusPlayerStat StatKey Amount))

(fn GetName
  (return ""))

(fn GetThuyTinhSocialStats
  (params (StatKey :type Name :default "None"))
  (bind _playersocialstats (Variables|Stats|GetPlayerSocialStats))
  (bind (_value _returnvalue) (Utilities|Map|Find _playersocialstats StatKey))
  (if _returnvalue
    (return _value)
    (else
      (return ""))))