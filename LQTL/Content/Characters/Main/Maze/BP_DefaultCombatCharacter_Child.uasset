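; Player combat character child that adds hold-to-charge summoning of "Thủy Tướng" legion companions, plus command and assault inputs.
; The equipped weapon picks the Shark or Swordfish class for ThuytuongPool, and a data table caps the count.
; Charge time and SpiritOrb set the number summoned at mesh sockets; holding again unsummons them.
; DoOnce-gated montages, Niagara tiers and material-collection glow show charge, while TeleportAssault rings summons around the locked target.
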(event Custom|On%20switch%20weapon%20to%20legion
  (params (Equipment :type BP%20Equipment%20Base%20Object%20Reference))
  (bind _self self)
  (bind _thuytuong_pool (Variables|Default|GetThuytuong_pool))
  (if (.Result (Default|GetEquippedEquipment (Variables|Default|GetEquipment%20Handler)))
    (switch int (Default|GetEquippedIndex (Variables|/Game/GeneralCombat/Blueprints/Pawns/BP_DefaultCombatCharacter.BP_DefaultCombatCharacter_C|GetEquipment%20Handler (.Out%20Character (CallFunction|GetPlayerCombatCharacter))))
      (:0
        (Default|Iniatialize _thuytuong_pool "/Game/Characters/Allies/Legions/Shark/Shark_BP.Shark_BP_C" _self))
      (:1
        (Default|Iniatialize _thuytuong_pool "/Game/Characters/Allies/Legions/Swordfish/Swordfish_BP.Swordfish_BP_C" _self)))
    (else
      (Default|Iniatialize _thuytuong_pool 0 _self))))

(event Custom|Spawn%20Fx
  ;[0.6181 0.855 1] Sync Action Thạch Sanh Hardcode
  (Game|SpawnActorfromClass "/Game/GeneralCombat/Blueprints/Widgets/Combat/AllComponentsTempFromTienForHardCode/BP_FxSkill.BP_FxSkill_C" (Math|Transform|MakeTransform (+ (* (Transformation|GetActorForwardVector) 3e+02) (Transformation|GetActorLocation)) "0, 0, 0" "1.000000,1.000000,1.000000") "Undefined" "MultiplyWithRoot" 0 0))

(event Input|EnhancedActionEvents|EnhancedInputActionIA_LegionCommand
  (params (ActionValue :type Boolean) (ElapsedSeconds :type Float%20%28double-precision%29) (TriggeredSeconds :type Float%20%28double-precision%29) (InputAction :type Input%20Action%20Object%20Reference :default "/Game/GeneralCombat/Data/Input/Gameplay/IA_LegionCommand.IA_LegionCommand"))
  ;[1 1 1] Command
  (Development|PrintString "Command Summon")
  (Default|CallOnCommand (Default|GetLockonActor (Variables|Default|GetAdvanced%20Camera%20Handler))))

(event Input|EnhancedActionEvents|EnhancedInputActionIA_LegionAssault
  (params (ActionValue :type Boolean) (ElapsedSeconds :type Float%20%28double-precision%29) (TriggeredSeconds :type Float%20%28double-precision%29) (InputAction :type Input%20Action%20Object%20Reference :default "/Game/GeneralCombat/Data/Input/Gameplay/IA_LegionAssault.IA_LegionAssault"))
  (bind _advanced_camera_handler (Variables|Default|GetAdvanced%20Camera%20Handler))
  (bind _actor (Default|GetLockonActor _advanced_camera_handler))
  ;[1 1 1] Assault
  (Development|PrintString "Assault Summon")
  (Utilities|IsValid _actor
    (:Is%20Valid
      (Default|CallOnAssault _actor))
    (:Is%20Not%20Valid
      (Default|CallOnAssault))))

(event EventBeginPlay
  (|CallParentFunction)
  (EventDispatchers|BindEventtoOnEquippedEquipmentChanged (Variables|Default|GetEquipment%20Handler) (delegate Custom|On%20switch%20weapon%20to%20legion)))

(event EventReturnAttackTokenRange
  (params (Amount%20Range :type Integer))
  (Default|ReturnAttackTokenRange (Variables|Default|GetBPC_DamageSystem) Amount%20Range))

(event EventReturnAttackTokenMelee
  (params (Amount%20Melee :type Integer))
  (Default|ReturnAttackTokenMelee (Variables|Default|GetBPC_DamageSystem) Amount%20Melee))

(event Input|KeyboardEvents|3
  (params (Key :type Key%20Structure))
  ;[0.6181 0.855 1] Sync Action Thạch Sanh Hardcode
  (:Pressed
    (bind _notifyname (Animation|Montage|PlayMontage (Variables|Character|GetMesh) "/Game/GeneralCombat/Blueprints/Widgets/Combat/AllComponentsTempFromTienForHardCode/AM_Shark_Combo_Light_01.AM_Shark_Combo_Light_01")
      (:OnNotifyBegin
        (switch name _notifyname)))))

(event Input|KeyboardEvents|2
  (params (Key :type Key%20Structure))
  ;[0.6181 0.855 1] Sync Action Thạch Sanh Hardcode
  (:Pressed
    (Default|AddBuff (Variables|Default|GetBPC_BuffComponent) "Stoneskin")))

(fn ConstructionScript
  (|CallParentFunction))

(fn TeleportSummon
  (params (Number%20Summons :type Integer))
  (bind _returnvalue (Transformation|GetActorLocation))
  (for (_array_element _array_index) (Variables|Summon|GetThuy%20tuong%20summoning)
    (switch int _array_index
      (:0
        (LocalVariables|SetSocket%20name "Legion_spawn_C_socket"))
      (:1
        (LocalVariables|SetSocket%20name "Legion_spawn_CR_socket"))
      (:2
        (LocalVariables|SetSocket%20name "Legion_spawn_CL_socket"))
      (:3
        (LocalVariables|SetSocket%20name "Legion_spawn_R_socket"))
      (:4
        (LocalVariables|SetSocket%20name "Legion_spawn_L_socket")))
    (LocalVariables|SetSummon%20location (CallFunction|GetSocketLocationatOffset (Variables|Character|GetMesh) (LocalVariables|GetSocket%20name) "0, 0, 0"))
    (Utilities|IsValid _array_element
      (:Is%20Valid
        (Transformation|SetActorLocation _returnvalue false false)
        (Transformation|SetActorLocationAndRotation (LocalVariables|GetSummon%20location) (Math|Rotator|FindLookatRotation _returnvalue (LocalVariables|GetSummon%20location)))))))

(fn Summon
  (params (Number%20Summons :type Integer))
  (if (>= Number%20Summons 0)
    (for _index (range 0 (- Number%20Summons 1))
      (bind _legion_actor (Default|SummonLegion (Variables|Default|GetThuytuong_pool) _index))
      (Utilities|Array|AddUnique (Variables|Summon|GetThuy%20tuong%20summoning) _legion_actor)
      (Default|CallOnSummon (Default|GetLockonActor (Variables|Default|GetAdvanced%20Camera%20Handler))))
    (Summon|TeleportSummon (- Number%20Summons 1))))

(fn Unsummon
  (bind _thuy_tuong_summoning (Variables|Summon|GetThuy%20tuong%20summoning))
  (for _array_element _thuy_tuong_summoning
    (Utilities|IsValid _array_element
      (:Is%20Valid
        (Default|ReturnLegion (Variables|Default|GetThuytuong_pool) _array_element))))
  (Utilities|Array|Clear _thuy_tuong_summoning)
  (Variables|Summon|SetTurnSummon? false))

(fn TeleportAssault
  (params (Actor%20LockOn :type Actor%20Object%20Reference))
  (bind _thuy_tuong_summoning (Variables|Summon|GetThuy%20tuong%20summoning))
  (bind _returnvalue (Transformation|GetActorLocation Actor%20LockOn))
  (for (_array_element _array_index) _thuy_tuong_summoning
    (Components|Movement|StopMovementImmediately (Variables|/Script/Engine.Character|GetCharacterMovement _array_element))
    (Animation|StopAnimMontage _array_element (Animation|GetCurrentMontage _array_element :!class /Script/Engine.Character))
    (Collision|SetActorEnableCollision _array_element false)
    (Rendering|SetActorHiddenInGame _array_element true)
    (Transformation|SetActorLocation _array_element _returnvalue false true)
    (Transformation|SetActorLocationAndRotation _array_element (+ _returnvalue (Math|Vector|MakeVector (* (Math|Trig|Cos(Radians) (Math|Trig|DegreesToRadians (Math|Conversions|ToFloat(Integer) (* (/ 360 (Utilities|Array|Length _thuy_tuong_summoning)) _array_index)))) (Variables|Summon|GetAssaultRadius)) (* (Math|Trig|Sin(Radians) (Math|Trig|DegreesToRadians (Math|Conversions|ToFloat(Integer) (* (/ 360 (Utilities|Array|Length _thuy_tuong_summoning)) _array_index)))) (Variables|Summon|GetAssaultRadius)) 0.0)) (Math|Rotator|FindLookatRotation (+ _returnvalue (Math|Vector|MakeVector (* (Math|Trig|Cos(Radians) (Math|Trig|DegreesToRadians (Math|Conversions|ToFloat(Integer) (* (/ 360 (Utilities|Array|Length _thuy_tuong_summoning)) _array_index)))) (Variables|Summon|GetAssaultRadius)) (* (Math|Trig|Sin(Radians) (Math|Trig|DegreesToRadians (Math|Conversions|ToFloat(Integer) (* (/ 360 (Utilities|Array|Length _thuy_tuong_summoning)) _array_index)))) (Variables|Summon|GetAssaultRadius)) 0.0)) _returnvalue) true)
    (Collision|SetActorEnableCollision _array_element true)
    (Rendering|SetActorHiddenInGame _array_element false)))

(fn FTinhsoSummon
  (params (SummonChargeTime :type Float%20%28double-precision%29))
  (bind _time_per_summon (Variables|Summon|GetTime%20per%20summon))
  (bind _returnvalue (/ 1.0 _time_per_summon))
  (bind _returnvalue_2 (* SummonChargeTime _returnvalue))
  (bind _returnvalue_3 (Math|Float|Floor _returnvalue_2))
  (if (< _returnvalue_3 1)
    (return -1)
    (else
      (return (Math|Integer|Clamp(Integer) _returnvalue_3 0 (Variables|Summon|GetNumber%20max%20summons))))))

(fn CheckWeaponPlayer
  (return (Default|GetEquippedIndex (Variables|/Game/GeneralCombat/Blueprints/Pawns/BP_DefaultCombatCharacter.BP_DefaultCombatCharacter_C|GetEquipment%20Handler (.Out%20Character (CallFunction|GetPlayerCombatCharacter))))))

(fn SummonLevel
  (params (A :type Float%20%28double-precision%29) (A2 :type Float%20%28double-precision%29))
  (if (and (>= A2 1.0) (< A 2.0))
    _))

(fn LevelFunction
  (params (TimePerSummon :type Float%20%28double-precision%29) (Sum_Time :type Float%20%28double-precision%29))
  (return (Math|Integer|Clamp(Integer) (Math|Float|Floor (* Sum_Time (/ 1.0 TimePerSummon))) 0 (Variables|Summon|GetNumber%20max%20summons))))

(fn SoLuongSummonRealF
  (params (SummonChargeTime :type Float%20%28double-precision%29))
  (if (< (Utilities|Struct|BreakS_CombatResource (Default|GetCurrentStat (Variables|Default|GetCombat%20Unit))) (* (Summon|FTinhsoSummon SummonChargeTime) 100))
    (bind _output_get (Variables|Summon|SetSummonW_Level (Math|Float|Truncate (/ (Utilities|Struct|BreakS_CombatResource (Default|GetCurrentStat (Variables|Default|GetCombat%20Unit))) 1e+02))))
    (return _output_get)
    (else
      (bind _output_get_2 (Variables|Summon|SetSummonW_Level (Summon|FTinhsoSummon SummonChargeTime)))
      (return _output_get_2))))

(event Custom|EndSummonFx)

(event Custom|TimmingSummon
  (Utilities|FlowControl|Sequence
    (:then_0
      (CallFunction|EndSummonFx))
    (:then_1
      (if (< (Utilities|Struct|BreakS_CombatResource (Default|GetCurrentStat (Variables|Default|GetCombat%20Unit))) (* (Summon|FTinhsoSummon (Variables|Summon|GetSummonChargeTime)) 100))
        (CallFunction|KhiKDuSpiritOrb)
        (else
          (CallFunction|KhiDuSpiritOrbCE))))))

(event Custom|Khi_K_Du_SpiritOrb
  (Summon|Summon (Math|Float|Truncate (/ (Utilities|Struct|BreakS_CombatResource (Default|GetCurrentStat (Variables|Default|GetCombat%20Unit))) 1e+02)))
  (Variables|Summon|SetTurnSummon? false)
  (Default|AddCurrentStat (Variables|Default|GetCombat%20Unit) (Utilities|Struct|MakeS_CombatResource (Math|Conversions|ToFloat(Integer) (* (Math|Float|Truncate (/ (Utilities|Struct|BreakS_CombatResource (Default|GetCurrentStat (Variables|Default|GetCombat%20Unit))) 1e+02)) -100))) self))

(event Custom|Xoa_Fx_LoopSummon
  (Components|Activation|Deactivate (Variables|Summon|GetFX_Summon_Comp)))

(event Custom|Upgrade_Weapon_Summon_CE
  (switch int (Summon|SoLuongSummonRealF (Variables|Summon|GetSummonChargeTime))
    (:1
      (Utilities|FlowControl|DoOnce false
        (:Completed
          (CallFunction|WeaponSummonFxLvl1CE))))
    (:3
      (Utilities|FlowControl|DoOnce false
        (:Completed
          (CallFunction|WeaponSummonFxLvl3CE))))
    (:5
      (Utilities|FlowControl|DoOnce false
        (:Completed
          (CallFunction|WeaponSummonFxLvl5CE))))))

(event Custom|IASummon_Cancel
  (if (not (== (CallFunction|CheckWeaponPlayer) 2))
    (Development|PrintString "Giữ hơn 1 Giây để Summon" true true "(R=0.000000,G=0.660000,B=1.000000,A=1.000000)" 5.0)))

(event Custom|Reset_Weapon_Fx_CE
  (Utilities|FlowControl|Sequence
    (:then_0
      (Utilities|FlowControl|DoOnce false) ; enters at Reset
    )
    (:then_1
      (Utilities|FlowControl|DoOnce false) ; enters at Reset
    )
    (:then_2
      (Utilities|FlowControl|DoOnce false) ; enters at Reset
    )))

(event Custom|Reset_Weapon_Glow_CE
  (Utilities|FlowControl|Delay 1.0)
  (bind _weaponglow (Timeline|Timeline_6 ReverseFromEnd)
    (:Update
      (Rendering|Material|SetScalarParameterValue "/Game/Characters/Main/Maze/Anim/_ComboBasicW/MPC_Weapon.MPC_Weapon" "Glow" _weaponglow :!class /Script/Engine.KismetMaterialLibrary))))

(event Custom|Reset_Anim_Loop_Summon
  (Utilities|FlowControl|DoOnce false) ; enters at Reset
)

(event Custom|Reset_FxLoop_Summon
  (Utilities|FlowControl|DoOnce false) ; enters at Reset
)

(event Custom|Weapon_SummonFx_lvl5_CE
  (Utilities|FlowControl|Sequence
    (:then_0
      (bind _weaponglow (Timeline|Weapon_Glow_Lvl5 PlayFromStart)
        (:Update
          (Rendering|Material|SetScalarParameterValue "/Game/Characters/Main/Maze/Anim/_ComboBasicW/MPC_Weapon.MPC_Weapon" "Glow" _weaponglow :!class /Script/Engine.KismetMaterialLibrary))))
    (:then_1
      (bind _returnvalue (Niagara|SpawnSystemAttached "/Game/Characters/Main/Maze/Fx/SummonThuyTuong/WeaponFx/NS_SummonWeaponFx_CaKiem_5.NS_SummonWeaponFx_CaKiem_5" (Variables|Character|GetMesh) "weapon_rSocket" "0, 0, 0" "0, 0, 0" "KeepRelativeOffset" false))
      (Utilities|Array|AddUnique (Variables|Summon|GetFX_Summon_Comp) _returnvalue))))

(event Custom|Weapon_SummonFx_lvl1_CE
  (Utilities|FlowControl|Sequence
    (:then_0
      (bind _weaponglow (Timeline|Weapon_Glow_Lvl1 PlayFromStart)
        (:Update
          (Rendering|Material|SetScalarParameterValue "/Game/Characters/Main/Maze/Anim/_ComboBasicW/MPC_Weapon.MPC_Weapon" "Glow" _weaponglow :!class /Script/Engine.KismetMaterialLibrary))))
    (:then_1
      (bind _returnvalue (Niagara|SpawnSystemAttached "/Game/Characters/Main/Maze/Fx/SummonThuyTuong/WeaponFx/NS_SummonWeaponFx_CaKiem_1.NS_SummonWeaponFx_CaKiem_1" (Variables|Character|GetMesh) "weapon_rSocket" "0, 0, 0" "0, 0, 0" "KeepRelativeOffset" false))
      (Utilities|Array|AddUnique (Variables|Summon|GetFX_Summon_Comp) _returnvalue))))

(event Custom|SummonTT_Trigger
  (params (SummonChargeTime :type Float%20%28double-precision%29))
  ;[1 1 1] Trigger_Loop
  (if (== (CallFunction|CheckWeaponPlayer) 2)
    (Development|PrintString "Vũ Khí không có Thủy Tướng" true true "(R=1.000000,G=0.021536,B=0.000000,A=1.000000)" 2.0 "1")
    (else
      (Variables|Summon|SetSummonChargeTime SummonChargeTime)
      (if (> (Utilities|Array|Length (Variables|Summon|GetThuy%20tuong%20summoning)) 0)
        (CallFunction|TurnUnsummonCE)
        (else
          (CallFunction|TurnSummonCE))))))

(event Custom|Weapon_SummonFx_lvl3_CE
  (Utilities|FlowControl|Sequence
    (:then_0
      (bind _weaponglow (Timeline|Weapon_Glow_Lvl3 PlayFromStart)
        (:Update
          (Rendering|Material|SetScalarParameterValue "/Game/Characters/Main/Maze/Anim/_ComboBasicW/MPC_Weapon.MPC_Weapon" "Glow" _weaponglow :!class /Script/Engine.KismetMaterialLibrary))))
    (:then_1
      (bind _returnvalue (Niagara|SpawnSystemAttached "/Game/Characters/Main/Maze/Fx/SummonThuyTuong/WeaponFx/NS_SummonWeaponFx_CaKiem_3.NS_SummonWeaponFx_CaKiem_3" (Variables|Character|GetMesh) "weapon_rSocket" "0, 0, 0" "0, 0, 0" "KeepRelativeOffset" false))
      (Utilities|Array|AddUnique (Variables|Summon|GetFX_Summon_Comp) _returnvalue))))

(event Custom|AN_Unsummon_CE
  (Summon|Unsummon))

(event Custom|Reset_Anim_Unsummon
  (Utilities|FlowControl|DoOnce false) ; enters at Reset
)

(event Custom|SummonTT_Start
  (if (== (CallFunction|CheckWeaponPlayer) 2)
    (Development|PrintString "Vũ Khí không có Thủy Tướng" true true "(R=1.000000,G=0.021536,B=0.000000,A=1.000000)" 2.0 "1")
    (else
      (Variables|Summon|SetSummonChargeTime 0.0)
      (if (== (Utilities|Array|Length (Variables|Summon|GetThuy%20tuong%20summoning)) 0)
        (Utilities|FlowControl|Sequence
          (:then_0
            (Animation|Montage|PlayMontage (Variables|Character|GetMesh) "/Game/Characters/Main/Maze/Anim/SummonTT/Summon_Ver2/Summon_Start_Montage.Summon_Start_Montage"))
          (:then_1
            (Variables|Summon|SetTurnSummon? true)))
        (else
          (Development|PrintString "Giữ để Unsummon Thủy Tướng" true true "(R=1.000000,G=0.021536,B=0.000000,A=1.000000)" 2.0 "1"))))))

(event Custom|SummonTT_CompleteHold
  (if (and (== (Utilities|Array|Length (Variables|Summon|GetThuy%20tuong%20summoning)) 0) (Variables|Summon|GetTurnSummon?))
    (CallFunction|XoaFxLoopSummon)
    (switch int (CallFunction|CheckWeaponPlayer)
      (:0
        (bind _returnvalue (Utilities|GetDataTableRow "/Game/GeneralCombat/Data/DataTables/AIUnit/DT_LegionInfoData.DT_LegionInfoData" "SpearFish")
          (:then
            (Variables|Summon|SetNumber%20max%20summons (Utilities|Struct|BreakS_LegionData _returnvalue)))))
      (:1
        (bind _returnvalue_2 (Utilities|GetDataTableRow "/Game/GeneralCombat/Data/DataTables/AIUnit/DT_LegionInfoData.DT_LegionInfoData" "Shark")
          (:then
            (Variables|Summon|SetNumber%20max%20summons (Utilities|Struct|BreakS_LegionData _returnvalue_2))))))
    (if (not (Variables|Summon|GetbIsStopSummon))
      (Utilities|FlowControl|Sequence
        (:then_0
          (Animation|Montage|PlayMontage (Variables|Character|GetMesh) "/Game/Characters/Main/Maze/Anim/SummonTT/Summon_Ver2/Summon_End_Montage.Summon_End_Montage"))))))

(event Custom|Fx_LoopSummon
  (Utilities|FlowControl|DoOnce false
    (:Completed
      (Utilities|FlowControl|Sequence
        (:then_0
          (Camera|PlayWorldCameraShake "/Game/Developers/Hiep/_MazeLong/EnemyTest/ImposterBeast/MoveSet/Atk/_BluePrintClass/CameraShake/IB_LightLongShake.IB_LightLongShake_C" "0, 0, 0" 5.0 2e+01))
        (:then_1
          (bind _returnvalue (Niagara|SpawnSystemAttached "/Game/Characters/Main/Maze/Fx/SummonThuyTuong/Tu/NS_TTTu2.NS_TTTu2" (Variables|Character|GetMesh) "weapon_rSocket" "0, 0, 0" "0, 0, 0" "KeepRelativeOffset" false))
          (Utilities|Array|AddUnique (Variables|Summon|GetFX_Summon_Comp) _returnvalue))))))

(event Custom|TurnSummon_CE
  (if (Variables|Summon|GetTurnSummon?)
    (Utilities|FlowControl|Sequence
      (:then_0
        (Utilities|FlowControl|DoOnce false
          (:Completed
            (Animation|Montage|PlayMontage (Variables|Character|GetMesh) "/Game/Characters/Main/Maze/Anim/SummonTT/Summon_Ver2/Summon_Loop_Montage.Summon_Loop_Montage"))))
      (:then_1
        (CallFunction|UpgradeWeaponSummonCE)))))

(event Custom|ResetSummon
  (CallFunction|ResetFxLoopSummon)
  (CallFunction|ResetAnimLoopSummon)
  (CallFunction|ResetWeaponGlowCE)
  (CallFunction|ResetWeaponFxCE)
  (CallFunction|ResetAnimUnsummon))

(event Custom|Turn_Unsummon_CE
  (Utilities|FlowControl|DoOnce false
    (:Completed
      (Animation|Montage|PlayMontage (Variables|Character|GetMesh) "/Game/Characters/Main/Maze/Anim/SummonTT/Summon_Ver2/Unsummon_Montage.Unsummon_Montage"))))

(event Custom|Khi_Du_SpiritOrb_CE
  (Default|AddCurrentStat (Variables|Default|GetCombat%20Unit) (Utilities|Struct|MakeS_CombatResource (Math|Conversions|ToFloat(Integer) (* (Math|Integer|Clamp(Integer) (Summon|FTinhsoSummon (Variables|Summon|GetSummonChargeTime)) 0 5) -100))) self)
  (Summon|Summon (Summon|FTinhsoSummon (Variables|Summon|GetSummonChargeTime)))
  (Variables|Summon|SetTurnSummon? false))

(event Input|EnhancedActionEvents|EnhancedInputActionIA_Dodge
  (params (ActionValue :type Boolean) (ElapsedSeconds :type Float%20%28double-precision%29) (TriggeredSeconds :type Float%20%28double-precision%29) (InputAction :type Input%20Action%20Object%20Reference :default "/Game/GeneralCombat/Data/Input/Gameplay/IA_Dodge.IA_Dodge"))
  ;[1 1 1] Cancel Summon
  (Variables|Summon|SetSummonChargeTime 0.0)
  (Variables|Summon|SetTurnSummon? false)
  (Variables|Summon|SetbIsStopSummon true)
  (Utilities|FlowControl|Delay 3.0)
  (Variables|Summon|SetbIsStopSummon false))

(event Input|EnhancedActionEvents|EnhancedInputActionIA_Summon
  (params (ActionValue :type Boolean) (ElapsedSeconds :type Float%20%28double-precision%29) (TriggeredSeconds :type Float%20%28double-precision%29) (InputAction :type Input%20Action%20Object%20Reference :default "/Game/Characters/Allies/IA_Summon.IA_Summon"))
  ;[0.2083 0.2083 0.2083] Hold 1s mới chạy vào Triggered
  (:Triggered
    (CallFunction|SummonTTTrigger TriggeredSeconds)
    (if (Variables|Summon|GetTurnSummon?)
      (Development|PrintString (Utilities|String|ToString(Float) TriggeredSeconds))))
  (:Started
    (CallFunction|SummonTTStart))
  (:Canceled
    ;[1 1 1] Giữ k đủ 1 s
    (CallFunction|IASummonCancel))
  (:Completed
    (CallFunction|SummonTTCompleteHold)
    (CallFunction|ResetSummon)))

(fn GetTeamNumber
  (return 0))

(fn ReserveAttackTokenMelee
  (params (Amount%20Melee :type Integer))
  (return false))

(fn ReserveAttackTokenRange
  (params (Amount%20Range :type Integer))
  (return false))