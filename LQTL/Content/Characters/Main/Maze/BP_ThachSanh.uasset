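; BP_ThachSanh is a short-lived Thach Sanh character that performs blessing animations for slots 3 and 4.
; Slot 3 plays a floating bow montage when the player's camera handler has a valid lock-on target, otherwise a standing bow montage.
; Slot 4 plays a slowed long Tiba montage, and every montage destroys the actor on completion.
; An unconnected rotation toward the lock-on target never runs.
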(event Custom|BlesTS_Slot4
  (Animation|Montage|PlayMontage (Variables|Character|GetMesh) "/Game/Characters/Main/Maze/Form/Blessing/ThachSanh/Anim_Model/Blessing_TS_Tiba_Long_Montage.Blessing_TS_Tiba_Long_Montage" 0.75
    (:OnCompleted
      (Actor|DestroyActor))))

(event Custom|BlesTS_Slot3
  (if (Utilities|IsValid (Variables|/Game/GeneralCombat/Blueprints/Components/BPC_AdvancedCameraHandler.BPC_AdvancedCameraHandler_C|GetLock%20On%20Target (Variables|/Game/GeneralCombat/Blueprints/Pawns/BP_DefaultCombatCharacter.BP_DefaultCombatCharacter_C|GetAdvanced%20Camera%20Handler (.Out%20Character (CallFunction|GetPlayerCombatCharacter)))))
    (Animation|Montage|PlayMontage (Variables|Character|GetMesh) "/Game/Characters/Main/Maze/Form/Blessing/ThachSanh/Anim_Model/Blessing_TS_BowFloat_Montage.Blessing_TS_BowFloat_Montage"
      (:OnCompleted
        (Actor|DestroyActor)))
    (else
      (Animation|Montage|PlayMontage (Variables|Character|GetMesh) "/Game/Characters/Main/Maze/Form/Blessing/ThachSanh/Anim_Model/Blessing_TS_BowStand_Montage.Blessing_TS_BowStand_Montage"
        (:OnCompleted
          (Actor|DestroyActor))))))

(event EventBeginPlay)

(event Collision|EventActorBeginOverlap
  (params (OtherActor :type Actor%20Object%20Reference)))

(event EventTick
  (params (DeltaSeconds :type Float%20%28single-precision%29)))

(fn ConstructionScript)