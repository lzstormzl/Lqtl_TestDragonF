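; Thach Sanh blessing actor that performs one of four skills (axe, long Tiba, held-then-released bow, NieuCom) through montages.
; A BSActing flag blocks overlapping skills, and each skill start runs a timeline that drives the Blessing_Dissolve parameter in MPC_Blessing.
; Bow release spawns a Niagara arrow at a mesh socket.
; When DissolveEnd is set, a reversed timeline dissolves it out, deactivates FX, hides the NieuCom mesh and destroys the actor.
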(event Custom|Skill%202
  (if (not (Variables|Default|GetBSActing?))
    (Variables|Default|SetBSActing? true)
    (Animation|PlayAnimMontage "/Game/Characters/Main/Maze/Form/Blessing/ThachSanh/Anim_Model/Blessing_TS_Tiba_Long_Montage.Blessing_TS_Tiba_Long_Montage" 1.0 "None")
    (CallFunction|StartDissolveCE)))

(event Custom|Skill%201
  (if (not (Variables|Default|GetBSActing?))
    (Variables|Default|SetBSActing? true)
    (Animation|PlayAnimMontage "/Game/Characters/Main/Maze/Form/Blessing/ThachSanh/Anim_Model/Blessing_TS_Axe_Montage.Blessing_TS_Axe_Montage" 1.0 "None")
    (CallFunction|StartDissolveCE)))

(event Custom|Dissolve_End_CE
  (if (Variables|Default|GetDissolve_End?)
    (Variables|Default|SetDissolve_End? false)
    (bind _apear_dissolve (Timeline|Timeline ReverseFromEnd)
      (:Update
        (Utilities|FlowControl|Sequence
          (:then_0
            (if (> _apear_dissolve 0.01)
              (Components|Activation|Deactivate (Variables|Default|Get_FX))))
          (:then_1
            (Rendering|Material|SetScalarParameterValue "/Game/Characters/Main/Maze/Form/Blessing/ThachSanh/MPC_Blessing.MPC_Blessing" "Blessing_Dissolve" _apear_dissolve :!class /Script/Engine.KismetMaterialLibrary))))
      (:Finished
        (Utilities|FlowControl|Sequence
          (:then_0
            (Development|SetHiddeninGame (Variables|Default|GetMesh_NieuCom) true false))
          (:then_1
            (Utilities|IsValid self
              (:Is%20Valid
                (Actor|DestroyActor)
                (Variables|Default|SetBSActing? false)))))))))

(event Custom|Skill%204
  (if (not (Variables|Default|GetBSActing?))
    (Variables|Default|SetBSActing? true)
    (Animation|PlayAnimMontage "/Game/Characters/Main/Maze/Form/Blessing/ThachSanh/Anim_Model/NieuCom/Blessing_TS_NieuCom_Montage.Blessing_TS_NieuCom_Montage" 1.0 "None")
    (Development|SetHiddeninGame (Variables|Default|GetMesh_NieuCom) false false)
    (CallFunction|StartDissolveCE)))

(event Custom|Skill%203%20End
  (bind _mesh (Variables|Character|GetMesh))
  (Animation|PlayAnimMontage "/Game/Characters/Main/Maze/Form/Blessing/ThachSanh/Anim_Model/Bow_Stand/Cast_Spell_Bow_End_Montage.Cast_Spell_Bow_End_Montage" 1.0 "None")
  (Niagara|SpawnSystematLocation "/Game/Common/_MazeLong/Fx/Blessing/ThachSanh/Arrow/NS_Blessing_TS_Arrow_Velocity.NS_Blessing_TS_Arrow_Velocity" (Transformation|GetSocketLocation _mesh "Fx_Arrow") (Transformation|GetSocketRotation _mesh "Fx_Arrow")))

(event Custom|Start_Dissolve_CE
  (bind _apear_dissolve (Timeline|Blessing PlayFromStart)
    (:Update
      (Rendering|Material|SetScalarParameterValue "/Game/Characters/Main/Maze/Form/Blessing/ThachSanh/MPC_Blessing.MPC_Blessing" "Blessing_Dissolve" _apear_dissolve :!class /Script/Engine.KismetMaterialLibrary))))

(event Custom|Skill%203%20Start
  (if (not (Variables|Default|GetBSActing?))
    (Variables|Default|SetBSActing? true)
    (Utilities|FlowControl|Sequence
      (:then_0
        (Animation|PlayAnimMontage "/Game/Characters/Main/Maze/Form/Blessing/ThachSanh/Anim_Model/Bow_Stand/Cast_Spell_Bow_Hold_Montage.Cast_Spell_Bow_Hold_Montage" 1.0 "None")
        (CallFunction|StartDissolveCE)))))

(event EventBeginPlay)

(event Collision|EventActorBeginOverlap
  (params (OtherActor :type Actor%20Object%20Reference)))

(event EventTick
  (params (DeltaSeconds :type Float%20%28single-precision%29))
  (Utilities|FlowControl|Sequence
    (:then_0
      (CallFunction|DissolveEndCE))))

(fn ConstructionScript)