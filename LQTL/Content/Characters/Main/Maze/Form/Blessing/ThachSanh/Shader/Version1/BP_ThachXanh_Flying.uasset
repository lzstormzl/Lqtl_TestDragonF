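; BP_ThachXanh_Flying is a character that follows the player, apparently a flying companion in the maze.
; On BeginPlay it caches a walk speed slightly faster than the player's BP_Maze_Long character.
; Every Tick it reissues AI MoveTo toward a point offset to the player's right.
; It also measures player distance each Tick, switching to a fixed speed when near and restoring the cached speed otherwise.
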(event Custom|ChasePlayer
  (bind _returnvalue (Game|GetPlayerCharacter 0))
  (AI|AIMoveTo self (+ (Transformation|GetActorLocation _returnvalue) (* (Transformation|GetActorRightVector _returnvalue) 1.2e+02)) 0 5e+01 false))

(event EventBeginPlay
  (bind _output_get (Variables|/Script/Engine.CharacterMovementComponent|SetMaxWalkSpeed (Variables|Character|GetCharacterMovement) (+ (Variables|/Script/Engine.CharacterMovementComponent|GetMaxWalkSpeed (Variables|/Script/Engine.Character|GetCharacterMovement (.AsBP%20Maze%20Long (Utilities|Casting|CastToBP_Maze_Long (Game|GetPlayerCharacter 0))))) 1e+02)))
  (Variables|Default|SetTemWalkSpeed _output_get))

(event Collision|EventActorBeginOverlap
  (params (OtherActor :type Actor%20Object%20Reference)))

(event EventTick
  (params (DeltaSeconds :type Float%20%28single-precision%29))
  (bind _charactermovement (Variables|Character|GetCharacterMovement))
  (Utilities|FlowControl|Sequence
    (:then_0
      (CallFunction|ChasePlayer))
    (:then_1
      (bind _output_get (Variables|Default|SetDistanceToPlayer (Transformation|GetDistanceTo self (Game|GetPlayerCharacter 0)))))
    (:then_2
      (if (< (Variables|Default|GetDistanceToPlayer) 1.9e+02)
        (Variables|/Script/Engine.CharacterMovementComponent|SetMaxWalkSpeed _charactermovement 3e+02)
        (else
          (Variables|/Script/Engine.CharacterMovementComponent|SetMaxWalkSpeed _charactermovement (Variables|Default|GetTemWalkSpeed)))))))

(fn ConstructionScript)