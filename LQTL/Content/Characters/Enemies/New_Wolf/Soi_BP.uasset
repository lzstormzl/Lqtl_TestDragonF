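; Wolf enemy character Blueprint that extends a parent class, handles its own death and supplies a fixed defensive strafe radius.
; After a delayed BeginPlay, it binds to the combat unit component's OnDeath event.
; Death clears focus, turns the mesh into a physics ragdoll and raises a combat flag counter.
; A timeline then drives a dynamic material's Dissolve parameter after a short wait, and the actor is destroyed when it finishes.
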(event EventBeginPlay
  (Utilities|FlowControl|DelayUntilNextTick)
  (|CallParentFunction)
  (Utilities|FlowControl|Delay 0.5)
  ;[1 0.2491 0.1635] Event binding
  (EventDispatchers|BindEventtoOnDeath (Variables|Default|GetBPC_CombatUnit) (EventDispatchers|CreateEvent :!event Custom|Event%20On%20Death)))

(event Custom|Event%20On%20Death
  (params (Initigator :type Actor%20Object%20Reference))
  (bind _mesh (Variables|Character|GetMesh))
  (Utilities|FlowControl|Sequence
    (:then_0
      (CallFunction|OnUnfocused)
      (Physics|SetSimulatePhysics (Variables|Character|GetMesh) true)
      (Collision|SetCollisionProfileName (Variables|Character|GetMesh) "Ragdoll" true :!class /Script/Engine.PrimitiveComponent)
      (Default|IncreaseCombatFlagsCounter (Variables|Default|GetBPC_CombatUnit) (|BitmaskLiteral 2))
      (bind _returnvalue (Rendering|Material|CreateDynamicMaterialInstance _mesh 0 (Rendering|Material|GetMaterial _mesh 0) "None" :!class /Script/Engine.PrimitiveComponent))
      (bind _output_get (Variables|Default|SetDissolve%20Material _returnvalue))
      (Rendering|Material|SetMaterial (Variables|Character|GetMesh) 0 _output_get))
    (:then_1
      (Utilities|FlowControl|Delay 2.0)
      (bind _alpha (Timeline|Timeline PlayFromStart)
        (:Update
          (Rendering|Material|SetScalarParameterValue (Variables|Default|GetDissolve%20Material) "Dissolve" _alpha :!class /Script/Engine.MaterialInstanceDynamic))
        (:Finished
          (Rendering|SetCastShadow (Variables|Character|GetMesh) false)
          (Actor|DestroyActor))))))

(fn ConstructionScript
  (|CallParentFunction))

(fn GetRangeDefend(StrafeRadius)
  (return 5e+02))