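; Enemy character that fights the player under AIC_Enemies control, with stats, move sets and combos read from data tables.
; Components handle stats, attacks and hitboxes; incoming damage passes through team and player-blessing checks.
; Spirit break interrupts the AI and enables critical hits, while attacks reserve and return tokens on their target.
; It also manages health bar and lock-on widgets, execution montages and movement speeds with a slow debuff.
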(event OnAttackHit(BPC_HitboxHandler)
  (params (Hit%20Actor :type Actor%20Object%20Reference) (Attack%20Data :type S%20Attack%20Data%20Structure) (Hit%20Count :type Integer) (In%20Hit%20Direction :type Vector :default "0, 0, 0"))
  ;[0.03229 0.03125 0.03125] Initialize
  (Class|BPIDamagable|OnDamaged(Message) Hit%20Actor Attack%20Data self In%20Hit%20Direction)
  (switch string (.Name (Utilities|Struct|BreakS_AttackComboData (Variables|Data|GetChoosen%20Combo)))
    (:Default
      (Niagara|SpawnSystematLocation "/Game/Characters/Main/Maze/Fx/Trail_Impact/NS_Hit_Impact_MazeLong.NS_Hit_Impact_MazeLong" (Transformation|GetActorLocation Hit%20Actor) "0, 0, 0" "1.000000,1.000000,1.000000" true true "ManualRelease"))))

(event OnAttackInitiated(BPC_AttackActionHandler)
  (params (Attack%20Data :type S%20Attack%20Action%20Data%20Structure))
  ;[0.03229 0.03125 0.03125] Initialize
  (Default|ResetOverlapIDTrack (Variables|Default|GetBPC_HitboxHandler)))

(event OnComponentBeginOverlap(CapsuleComponent)
  (params (OverlappedComponent :type Primitive%20Component%20Object%20Reference) (OtherActor :type Actor%20Object%20Reference) (OtherComp :type Primitive%20Component%20Object%20Reference) (OtherBodyIndex :type Integer) (bFromSweep :type Boolean) (SweepResult :type Hit%20Result%20Structure%20%28by%20ref%29))
  (bind _output_get (Variables|Default|SetSoaked%20Value (Math|Float|Clamp(Float) (+ (Variables|Default|GetSoaked%20Value) 5e+01) 0.0 (Variables|Default|GetMax%20Soaked%20Value))))
  (Default|SetSoakedValue (Variables|Focus|GetHealth%20Bar%20Widget) _output_get)
  (Callbacks|OnCombatInitiated))

(event Custom|Set%20Focus%20Active
  (params (Focused :type Boolean))
  ;[0.02 0.02 0.02 1 32] Widget Control On Focus
  (if Focused
    (Utilities|FlowControl|Sequence
      (:then_0
        (Widget|SetRenderOpacity (Variables|Focus|GetHealth%20Bar%20Widget) 1.0))
      (:then_1
        (bind _alpha (Timeline|Timeline_0 Stop)
          (:Update
            (Utilities|FlowControl|Sequence
              (:then_0
                (Widget|SetRenderOpacity (Variables|Focus|GetHealth%20Bar%20Widget) (Math|Float|Lerp (Variables|/Script/UMG.Widget|GetRenderOpacity (Variables|Focus|GetHealth%20Bar%20Widget)) 0.0 _alpha)))
              (:then_1
                (if (not (Default|GetSpiritBreakState (Variables|Default|GetBPC_CombatUnit)))
                  (Widget|SetRenderOpacity (Variables|Focus|GetLock%20On%20Indicator%20Widget) (Math|Float|Lerp (Variables|/Script/UMG.Widget|GetRenderOpacity (Variables|Focus|GetLock%20On%20Indicator%20Widget)) 0.0 _alpha)))))))))
    (else
      (Utilities|Time|ClearandInvalidateTimerbyHandle (Variables|Focus|GetHide%20Healthbar%20Display%20Timer))
      (Timeline|Timeline_0 PlayFromStart))))

(event Custom|On%20Destroyed
  (params (DestroyedActor :type Actor%20Object%20Reference))
  (Default|SetCurrentStat (Variables|Default|GetBPC_CombatUnit) (Utilities|Struct|MakeS_CombatResource 0.0 0.0) self))

(event Custom|Heal%20and%20BackCamp
  (bind _bpc_combatunit (Variables|Default|GetBPC_CombatUnit))
  ;[0.617 1 0.5834] Heal When Back Camp
  (Default|AddCurrentStat _bpc_combatunit (Utilities|Struct|MakeS_CombatResource 0.0 (/ (.health (Utilities|Struct|BreakS_CombatResource (Default|GetMaxStat _bpc_combatunit))) 1e+01) 0.0 5e+01 0.0) self))

(event Custom|Handle%20Spirit%20Break
  (params (State :type Boolean))
  (bind _bpc_combatunit (Variables|Default|GetBPC_CombatUnit))
  (bind _as_aic_enermy (Variables|AI|GetAs%20AIC%20Enermy))
  ;[0.03229 0.03125 0.03125] Initialize
  (if State
    (Utilities|IsValid _as_aic_enermy
      (:Is%20Valid
        (Default|SetStateStagger(Interrupt+) _as_aic_enermy true)
        (AI|ClearFocus _as_aic_enermy)
        (Utilities|FlowControl|Delay 0.5)
        (Animation|StopAnimMontage (Animation|GetCurrentMontage :!class /Script/Engine.Character))
        (Default|HandleSpiritBreak _bpc_combatunit (Variables|Default|GetSpirit%20Break%20Time) (Utilities|Struct|BreakS_HitReactData (Utilities|Struct|BreakS_CharacterCombatData (Data|GetCharacterCombatData))))
        (EventDispatchers|BindEventtoOnSpiritBreakEnded _bpc_combatunit (delegate Custom|On%20Spirit%20Break%20Ended))))))

(event Custom|On%20Spirit%20Break%20Ended
  (bind _as_aic_enermy (Variables|AI|GetAs%20AIC%20Enermy))
  (Utilities|IsValid _as_aic_enermy
    (:Is%20Valid
      (Utilities|FlowControl|Delay 0.2)
      (Default|SetStateStagger(Interrupt+) _as_aic_enermy false))))

(event Custom|PlayExecutionMontage
  ;[0 0 0] Execution
  (Default|SetStateStagger(Interrupt+) (Variables|AI|GetAs%20AIC%20Enermy) false)
  (Animation|Montage|PlayMontage (Variables|Character|GetMesh) (.Montage (Data|GetExecutionMontage))))

(event Custom|Remove_debuff_giam_speed
  (Variables|Default|SetIsDebuff_giam_speed false)
  (Utilities|Time|ClearandInvalidateTimerbyHandle (Variables|Default|GetRemove_debuff_giam_speed%20Timer)))

(event EventGetInfoMotionWarp
  (params (Montion%20Warp%20Data :type S%20Motion%20Warp%20Data%20Structure))
  (Variables|/Game/GeneralCombat/Blueprints/Components/BPC_AttackActionHandler.BPC_AttackActionHandler_C|SetS%20Motion%20Warp%20Data (Variables|Default|GetBPC_AttackActionHandler) Montion%20Warp%20Data))

(event EventBeginPlay
  (bind _combat_data (Data|GetCharacterCombatData))
  ;[0.03229 0.03125 0.03125] Initialize
  (bind _asaic_enemies (Utilities|Casting|CastToAIC_Enemies (AI|GetAIController self)))
  (Variables|AI|SetAs%20AIC%20Enermy _asaic_enemies)
  (CallFunction|InitializeWorldWidget)
  (Default|SetCharacterCombatData (Variables|Default|GetBPC_CombatUnit) _combat_data self)
  (Default|SetCurrentStat (Variables|Default|GetBPC_CombatUnit) (.MaxStats (Utilities|Struct|BreakS_CharacterCombatData _combat_data)) self)
  (Default|InitializeComponent (Variables|Default|GetBPC_AttackActionHandler) (Variables|Character|GetMesh))
  (Default|SetSoakedValue (Variables|Focus|GetHealth%20Bar%20Widget) (Variables|Default|GetSoaked%20Value))
  (EventDispatchers|BindEventtoOnSpiritBreakStateUpdated (Variables|Default|GetBPC_CombatUnit) (delegate Custom|Handle%20Spirit%20Break))
  (Game|BindEventtoOnDestroyed (delegate Custom|On%20Destroyed)))

(event EventStoreAttackTokensMelee
  (params (AttackTarget :type Actor%20Object%20Reference) (Amount%20Melee :type Integer))
  (bind _reserveattacktokens_range (Variables|Combatticket|GetReserveAttackTokens_Range))
  (bind (_value _returnvalue) (Utilities|Map|Find _reserveattacktokens_range AttackTarget))
  ;[0.04249 0.1714 0.1781] Combat Ticket
  (Utilities|Map|Add (Variables|Combatticket|GetReserveAttackTokens_Range) AttackTarget (Math|Integer|SelectInt (+ Amount%20Melee _value) Amount%20Melee _returnvalue)))

(event EventReturnAttackTokenMelee
  (params (Amount%20Melee :type Integer))
  ;[0.04249 0.1714 0.1781] Combat Ticket
  (Default|ReturnAttackTokenMelee (Variables|Default|GetBPC_CombatTicketSystem) Amount%20Melee))

(event EventReturnAttackTokenRange
  (params (Amount%20Range :type Integer))
  ;[0.04249 0.1714 0.1781] Combat Ticket
  (Default|ReturnAttackTokenRange (Variables|Default|GetBPC_CombatTicketSystem) Amount%20Range))

(event EventDebuffGiamSpeed
  (Variables|Default|SetIsDebuff_giam_speed true)
  (bind _returnvalue (Utilities|Time|SetTimerbyEvent (EventDispatchers|CreateEvent :!event Custom|Remove_debuff_giam_speed) 2.0))
  (Variables|Default|SetRemove_debuff_giam_speed%20Timer _returnvalue))

(event EventAttackEnd
  (params (AttackTarget :type Actor%20Object%20Reference))
  (bind _tokenusedincurrentattack_melee (Variables|Combatticket|GetTokenUsedInCurrentAttack_Melee))
  (bind _tokenusedincurrentattack_range (Variables|Combatticket|GetTokenUsedInCurrentAttack_Range))
  ;[0.04249 0.1714 0.1781] Combat Ticket
  (Class|BPIDamageSystem|ReturnAttackTokenMelee(Message) AttackTarget _tokenusedincurrentattack_melee)
  (Class|BPIDamageSystem|ReturnAttackTokenRange(Message) AttackTarget _tokenusedincurrentattack_range)
  (CallFunction|StoreAttackTokensMelee AttackTarget (* _tokenusedincurrentattack_melee -1))
  (CallFunction|StoreAttackTokensRange AttackTarget (* _tokenusedincurrentattack_range -1)))

(event EventAttack
  (params (Attack%20Target :type Actor%20Object%20Reference) (Combo%20Choosen :type S%20Attack%20Combo%20Data%20Structure))
  ;[1 0.06413 0] Attack
  (Default|SetCurrentAttackCombo (Variables|Default|GetBPC_AttackActionHandler) Combo%20Choosen)
  (Default|TryRegisterAttack (Variables|Default|GetBPC_AttackActionHandler) true))

(event EventStoreAttackTokensRange
  (params (AttackTarget :type Actor%20Object%20Reference) (Amount%20Range :type Integer))
  (bind _reserveattacktokens_melee (Variables|Combatticket|GetReserveAttackTokens_Melee))
  (bind (_value _returnvalue) (Utilities|Map|Find _reserveattacktokens_melee AttackTarget))
  ;[0.04249 0.1714 0.1781] Combat Ticket
  (Utilities|Map|Add (Variables|Combatticket|GetReserveAttackTokens_Melee) AttackTarget (Math|Integer|SelectInt (+ Amount%20Range _value) Amount%20Range _returnvalue)))

(event Custom|Event%20On%20Focused
  ;[0.02 0.02 0.02 1 32] Lock On Target
  (Variables|Focus|SetFocused true)
  (CallFunction|SetFocusActive true)
  (Widget|SetRenderOpacity (Variables|Focus|GetLock%20On%20Indicator%20Widget) 1.0)
  (Utilities|Time|ClearandInvalidateTimerbyHandle (Variables|Focus|GetHide%20Healthbar%20Display%20Timer)))

(event Custom|Event%20On%20Unfocused
  ;[0.02 0.02 0.02 1 32] Lock On Target
  (Variables|Focus|SetFocused false)
  (CallFunction|SetFocusActive false))

(event EventOnDamaged
  (params (Source%20Attack :type S%20Attack%20Data%20Structure) (Initigator :type Actor%20Object%20Reference) (Hit%20Direction :type Vector :default "0, 0, 0"))
  ;[0.02 0.02 0.02 1 32] Damagable
  (bind _teamnumber (Class|BPIDamageSystem|GetTeamNumber(Message) Initigator))
  (if (not (== _teamnumber 2))
    (bind _dmg_info_after_modifier (CallFunction|ModifierDmgBeforeApply Source%20Attack))
    (Default|ApplyDamage (Variables|Default|GetBPC_CombatUnit) _dmg_info_after_modifier Initigator Hit%20Direction)
    (Default|EnemyReturnonHit (.Out%20Character (CallFunction|GetPlayerCombatCharacter)))))

(event OnSpiritBreakStateUpdated(BPC_CombatUnit)
  (params (State :type Boolean))
  (bind _as_aic_enermy (Variables|AI|GetAs%20AIC%20Enermy))
  (if State
    (Variables|Default|SetCanBeCriticalHit State)
    (Widget|SetRenderOpacity (Variables|Focus|GetLock%20On%20Indicator%20Widget) 1.0)
    (Utilities|IsValid _as_aic_enermy
      (:Is%20Valid
        (Default|SetStateSpiritBreak _as_aic_enermy false)))
    (else
      (Variables|Default|SetCanBeCriticalHit false))))

(event OnStatUpdated(BPC_CombatUnit)
  (params (New%20Data :type S%20Combat%20Resource%20Structure) (Delta%20Data :type S%20Combat%20Resource%20Structure) (Initigator :type Actor%20Object%20Reference))
  (if (!= Initigator self)
    (Callbacks|OnCombatInitiated)))

(event OnDeath(BPC_CombatUnit)
  (params (Actor :type Actor%20Object%20Reference))
  (bind _out_character (CallFunction|GetPlayerCombatCharacter))
  (bind _advanced_camera_handler (Variables|/Game/GeneralCombat/Blueprints/Pawns/BP_DefaultCombatCharacter.BP_DefaultCombatCharacter_C|GetAdvanced%20Camera%20Handler _out_character))
  (if (== (Variables|/Game/GeneralCombat/Blueprints/Components/BPC_AdvancedCameraHandler.BPC_AdvancedCameraHandler_C|GetLock%20On%20Target _advanced_camera_handler) Actor)
    (Widget|SetRenderOpacity (Variables|BP_Enemy_C|GetLock%20On%20Indicator%20Widget self) 0.0)
    (Default|SetLockonActor _advanced_camera_handler)))

(event OnSpiritBreakEnded(BPC_CombatUnit)
  (bind _bpc_combatunit (Variables|Default|GetBPC_CombatUnit))
  (Utilities|IsValid (Variables|AI|GetAs%20AIC%20Enermy)
    (:Is%20Valid
      (if (<= (Utilities|Struct|BreakS_CombatResource (Default|GetCurrentStat _bpc_combatunit)) 0.0)
        (Default|AddCurrentStat _bpc_combatunit (Utilities|Struct|MakeS_CombatResource 0.0 0.0 0.0 (Utilities|Struct|BreakS_CombatResource (Default|GetMaxStat (Variables|Default|GetBPC_CombatUnit))) 0.0) self))
      (Utilities|FlowControl|Delay 0.5)
      (Default|SetStateSpiritBreak (Variables|AI|GetAs%20AIC%20Enermy) false))))

(fn ConstructionScript
  (Variables|Default|SetTeam%20Number 2))

(fn GetEnemyData
  (bind _enemydata (Variables|Data|GetEnemyData))
  (bind _returnvalue (Utilities|GetDataTableRow (.datatable _enemydata) (.rowname _enemydata))
    (:then
      (return _returnvalue))))

(fn GetMoveSetData
  (bind _returnvalue (Utilities|GetDataTableRow "/Game/GeneralCombat/Data/DataTables/GeneralCombat/DT_MoveSets.DT_MoveSets" (.MoveSetName (Utilities|Struct|BreakS_AIUnitData (Data|GetEnemyData))))
    (:then
      (return _returnvalue))))

(fn GetListComboData
  (for _array_element (.CombosName (Utilities|Struct|BreakS_MoveSetData (Data|GetMoveSetData)))
    (bind _returnvalue (Utilities|GetDataTableRow "/Game/GeneralCombat/Data/DataTables/GeneralCombat/DT_AttackComboData.DT_AttackComboData" _array_element)
      (:then
        (Utilities|Array|AddUnique (Variables|Data|GetList%20Combo) _returnvalue))))
  (return (Variables|Data|GetList%20Combo)))

(fn GetListAttackActionData
  (params (Combo%20Data :type S%20Attack%20Combo%20Data%20Structure))
  (Utilities|Array|Clear (Variables|Data|GetList%20Attack%20))
  (for _array_element (.AttacksName (Utilities|Struct|BreakS_AttackComboData Combo%20Data))
    (bind _returnvalue (Utilities|GetDataTableRow (.datatable _array_element) (.rowname _array_element))
      (:then
        (Utilities|Array|AddUnique (Variables|Data|GetList%20Attack%20) _returnvalue))))
  (return (Variables|Data|GetList%20Attack%20)))

(fn InitializeWorldWidget
  (Utilities|FlowControl|Sequence
    (:then_0
      ;[0.02 0.02 0.02 1 30] Heath Bar
      (bind _returnvalue (UserInterface|CreateWidget "/Game/GeneralCombat/Blueprints/Widgets/Combat/HealthBar/WB_NormalEnemyHealthBar.WB_NormalEnemyHealthBar_C"))
      (bind _output_get (Variables|Focus|SetHealth%20Bar%20Widget _returnvalue))
      (Default|Initialize _output_get (Variables|Default|GetBPC_CombatUnit) (Data|GetCharacterCombatData))
      (Widget|SetRenderOpacity (Variables|Focus|GetHealth%20Bar%20Widget) 0.0)
      (UserInterface|SetWidget (Variables|Default|GetWidget_HealthBar) (Variables|Focus|GetHealth%20Bar%20Widget))
      (Transformation|SetWorldRotation (Variables|Default|GetWidget_HealthBar) "0.000000,90.000000,0.000000" false false)
      (Transformation|AttachComponentToComponent (Variables|Default|GetWidget_HealthBar) (Variables|Character|GetMesh) "Head" "SnapToTarget" "KeepWorld" "KeepWorld" true))
    (:then_1
      ;[0.02 0.02 0.02 1 30] Lock On Target
      (bind _returnvalue_2 (UserInterface|CreateWidget "/Game/GeneralCombat/Blueprints/Widgets/Combat/Indicators/WB_LockTargetIndicator.WB_LockTargetIndicator_C"))
      (bind _output_get_2 (Variables|Focus|SetLock%20On%20Indicator%20Widget _returnvalue_2))
      (Default|Initialize _output_get_2 (Variables|Default|GetBPC_CombatUnit))
      (Widget|SetRenderOpacity (Variables|Focus|GetLock%20On%20Indicator%20Widget) 0.0)
      (UserInterface|SetWidget (Variables|Default|GetWidget_LockOnIndicator) (Variables|Focus|GetLock%20On%20Indicator%20Widget))
      (Transformation|AttachComponentToComponent (Variables|Default|GetWidget_LockOnIndicator) (Variables|Character|GetMesh) "CenterMass" "SnapToTarget" "KeepWorld" "KeepWorld" true))))

(fn GetCharacterCombatData
  (bind _bpc_combatunit (Variables|Default|GetBPC_CombatUnit))
  (bind _default_character_combat_data (Variables|/Game/GeneralCombat/Blueprints/Components/BPC_CombatUnit.BPC_CombatUnit_C|GetDefault%20Character%20Combat%20Data _bpc_combatunit))
  (bind _returnvalue (Utilities|GetDataTableRow (.datatable _default_character_combat_data) (.rowname _default_character_combat_data))
    (:then
      (return _returnvalue))))

(fn OnCombatInitiated
  (if (not (Variables|Focus|GetFocused))
    (CallFunction|SetFocusActive true)
    (bind _returnvalue (Utilities|Time|SetTimerbyEvent (EventDispatchers|CreateEvent :!event OnUnfocused) 5.0))
    (Variables|Focus|SetHide%20Healthbar%20Display%20Timer _returnvalue)))

(fn OnStatUpdated
  (params (Stat :type S%20Combat%20Resource%20Structure%20%28by%20ref%29) (Initigator :type Actor%20Object%20Reference)))

(fn GetCurrentMesh
  (return (Variables|Character|GetMesh)))

(fn GetExecutionMontage
  (bind _executionmontage (Variables|Default|GetExecutionMontage)
    (:then
      (return _executionmontage true))
    (:else
      (return 0 false))))

(fn ModifierDmgBeforeApply
  (params (Dmg%20info%20before%20modifier :type S%20Attack%20Data%20Structure))
  (bind _out_character (CallFunction|GetPlayerCombatCharacter))
  (bind (_attackbasestat _selfeffectbasestat _attackelement _attackflags) (Utilities|Struct|BreakS_AttackData Dmg%20info%20before%20modifier))
  (bind _bpc_blessing (Variables|/Game/GeneralCombat/Blueprints/Pawns/BP_DefaultCombatCharacter.BP_DefaultCombatCharacter_C|GetBPC_Blessing _out_character))
  (bind (_shield _health _spiritwater _spiritorb _stagger) (Utilities|Struct|BreakS_CombatResource _attackbasestat))
  (Utilities|FlowControl|Sequence
    (:then_0
      (switch Utilities|FlowControl|Switch|SwitchonE_Blessing (Variables|/Game/ThirdPerson/BPC_Blessing.BPC_Blessing_C|GetBlessing%20Choosing _bpc_blessing)
        (:NewEnumerator1
          (if (Utilities|Map|Contains (Variables|/Game/ThirdPerson/BPC_Blessing.BPC_Blessing_C|GetActivating%20Effects _bpc_blessing) "NewEnumerator0")
            (LocalVariables|SetSoure%20dmg (Utilities|Struct|MakeS_AttackData (Utilities|Struct|MakeS_CombatResource _shield _health _spiritwater _spiritorb (+ _stagger 15.0)) _selfeffectbasestat _attackelement _attackflags))
            (else
              (LocalVariables|SetSoure%20dmg ""))))))
    (:then_1
      (return (LocalVariables|GetSoure%20dmg)))))

(fn AttackStart
  (params (AttackTarget :type Actor%20Object%20Reference) (TokenNeededMelee :type Integer) (TokenNeededRange :type Integer))
  (bind _success (Class|BPIDamageSystem|ReserveAttackTokenMelee(Message) AttackTarget TokenNeededMelee))
  (bind _success_2 (Class|BPIDamageSystem|ReserveAttackTokenRange(Message) AttackTarget TokenNeededRange))
  (if (or _success_2 _success)
    (CallFunction|StoreAttackTokensMelee AttackTarget TokenNeededMelee)
    (CallFunction|StoreAttackTokensRange AttackTarget TokenNeededRange)
    (Variables|Combatticket|SetTokenUsedInCurrentAttack_Melee TokenNeededMelee)
    (Variables|Combatticket|SetTokenUsedInCurrentAttack_Range TokenNeededRange)
    (return true)
    (else
      (return false))))

(fn DestroyHitbox
  (params (Hitbox%20Data :type S%20Hitbox%20Data%20Structure))
  (Default|DestroyHitbox (Variables|Default|GetBPC_HitboxHandler) Hitbox%20Data)
  (return true))

(fn GayDmgonEnemy
  (params (S%20attack%20data%20in :type S%20Attack%20Data%20New%20Structure))
  (bind (_hpdamage _spiritorbdamage _staggerdamage) (Utilities|Struct|BreakS_Attack_Data_new S%20attack%20data%20in))
  (Default|ApplyDamage (Variables|Default|GetBPC_CombatUnit) (Utilities|Struct|MakeS_AttackData (Utilities|Struct|MakeS_CombatResource 0.0 _hpdamage 0.0 _spiritorbdamage _staggerdamage) "(shield=0.000000,health=0.000000,spiritWater=0.000000,spiritOrb=0.000000,stagger=0.000000)" "None" 0) 0 "0, 0, 0")
  (return))

(fn GenerateHitbox
  (params (Hitbox%20Data :type S%20Hitbox%20Data%20Structure))
  (bind _hitbox_generated (Default|GenerateHitbox (Variables|Default|GetBPC_HitboxHandler) Hitbox%20Data))
  (return _hitbox_generated))

(fn GetAttackTarget
  (return (Variables|/Game/GeneralCombat/AI/Enemies/AIC_Controller/AIC_Enemies.AIC_Enemies_C|GetAttack%20Target (Variables|AI|GetAs%20AIC%20Enermy))))

(fn GetCenterMassLocation
  (return (Transformation|GetSocketLocation (Variables|Character|GetMesh) "CenterMass")))

(fn GetLockonLocation
  (return (Transformation|GetSocketLocation (Variables|Character|GetMesh) "LockOn")))

(fn GetRangeDefend(StrafeRadius)
  (return 5e+02))

(fn GetEnemyRef
  (return self))

(fn GetPatrolRoute
  (return 0))

(fn GetTeamNumber
  (return (Variables|Default|GetTeam%20Number)))

(fn ReserveAttackTokenMelee
  (params (Amount%20Melee :type Integer))
  (return false))

(fn ReserveAttackTokenRange
  (params (Amount%20Range :type Integer))
  (return false))

(fn SetMovementSpeed
  (params (Speed :type E_AI_Movement_State%20Enum :default "NewEnumerator0"))
  (if (Variables|Default|GetIsDebuff_giam_speed)
    (bind _output_get (Variables|/Script/Engine.CharacterMovementComponent|SetMaxWalkSpeed (Variables|Character|GetCharacterMovement) (Utilities|Select :Index Speed :NewEnumerator0 0.0 :NewEnumerator1 2.8e+02 :NewEnumerator2 1.2e+02 :NewEnumerator3 5.6e+02 :NewEnumerator4 448.0 :NewEnumerator5 7.2e+02)))
    (return _output_get)
    (else
      (bind _output_get_2 (Variables|/Script/Engine.CharacterMovementComponent|SetMaxWalkSpeed (Variables|Character|GetCharacterMovement) (Utilities|Select :Index Speed :NewEnumerator0 0.0 :NewEnumerator1 3.5e+02 :NewEnumerator2 1.5e+02 :NewEnumerator3 7e+02 :NewEnumerator4 2.5e+02 :NewEnumerator5 9e+02)))
      (return _output_get_2))))