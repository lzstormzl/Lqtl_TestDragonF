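; Tiger enemy character Blueprint, built on a parent class, that handles the enemy's death.
; Shortly after BeginPlay it binds to the combat unit component's OnDeath event.
; On death it flags the enemy AI controller as dead, stops the current montage and disables mesh collision.
; After a short delay it plays a montage, then hides and destroys the actor on completion or blend-out.
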(event EventBeginPlay
  (|CallParentFunction)
  (Utilities|FlowControl|Delay 0.5)
  ;[1 0.2491 0.1635] Event binding
  (EventDispatchers|BindEventtoOnDeath (Variables|Default|GetBPC_CombatUnit) (EventDispatchers|CreateEvent :!event Custom|Event%20On%20Death)))

(event Collision|EventActorBeginOverlap
  (params (OtherActor :type Actor%20Object%20Reference)))

(event EventTick
  (params (DeltaSeconds :type Float%20%28single-precision%29)))

(event Custom|Event%20On%20Death
  (params (Initigator :type Actor%20Object%20Reference))
  (bind _as_aic_enermy (Variables|Default|GetAs%20AIC%20Enermy))
  (Utilities|IsValid _as_aic_enermy
    (:Is%20Valid
      (Default|SetStateDeath _as_aic_enermy true)
      (Animation|StopAnimMontage (Animation|GetCurrentMontage :!class /Script/Engine.Character))
      (Collision|SetCollisionEnabled (Variables|Character|GetMesh) "NoCollision")
      (Utilities|FlowControl|Delay 0.5)
      (Animation|Montage|PlayMontage (Variables|Character|GetMesh) 0
        (:OnCompleted
          _)
        (:OnBlendOut
          _))
      (Rendering|SetActorHiddenInGame true)
      (Actor|DestroyActor))
    (:Is%20Not%20Valid
      (Development|PrintString "Death _ not valid aic"))))

(fn ConstructionScript
  (|CallParentFunction))