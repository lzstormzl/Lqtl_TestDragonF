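; BP_BuffManager is an early-stage actor for granting data-table-driven buffs in the social game systems.
; AddBuffToActor accepts only the player character, looks up the BuffID row in BuffDataTable and clamps the amount to its MaxStack.
; The count starts from zero rather than an existing stack and is not applied to the actor.
; The HUD refresh and instant stat-trigger loop are disconnected, and the loop body is empty.
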(event EventBeginPlay)

(event Collision|EventActorBeginOverlap
  (params (OtherActor :type Actor%20Object%20Reference)))

(event EventTick
  (params (DeltaSeconds :type Float%20%28single-precision%29)))

(fn ConstructionScript)

(fn AddBufftoActor
  (params (BuffID :type Name) (Amount :type Integer) (Actor :type Actor%20Object%20Reference))
  (bind _returnvalue (+ 0 Amount))
  (Utilities|IsValid Actor
    (:Is%20Valid
      (if (== Actor (Game|GetPlayerCharacter 0))
        (bind _returnvalue_2 (Utilities|GetDataTableRow "/Game/GeneralSocial/Config/DataTableConfig/Buff/BuffDataTable.BuffDataTable" BuffID)
          (:then
            (if (> _returnvalue (.MaxStack (Utilities|Struct|BreakBuffnDebuffStructDefine _returnvalue_2)))
              (LocalVariables|SetCurrentCount (.MaxStack (Utilities|Struct|BreakBuffnDebuffStructDefine _returnvalue_2)))
              (else
                (LocalVariables|SetCurrentCount _returnvalue)))))))))