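; Quest objective that completes when the player finishes a specific dialogue.
; On branching objective initialization it binds to the DialogueComponent's dialogue-finish event.
; The handler checks the DialogueID by data table and row name, then unbinds, completes the objective and prints a debug message.
; Removing the objective also unbinds the event.
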(event EventInitializeBranchingObjective
  (|CallParentFunction)
  (EventDispatchers|BindEventtoOnDialogueFinish (.DialogueComponent (Variables|Default|GetDialogueComponent)) (EventDispatchers|CreateEvent :!event BPTalktoObjectiveAutoGenFunc)))

(fn BPTalktoObjectiveAutoGenFunc
  (params (DialogueID :type Data%20Table%20Row%20Handle%20Structure))
  (bind (_datatable _rowname) (Utilities|Struct|BreakDataTableRowHandle DialogueID))
  (bind (_datatable_2 _rowname_2) (Utilities|Struct|BreakDataTableRowHandle (Variables|Default|GetDialogueID)))
  (if (and (== _datatable _datatable_2) (== _rowname _rowname_2))
    (EventDispatchers|UnbindEventfromOnDialogueFinish (.DialogueComponent (Variables|Default|GetDialogueComponent)) (EventDispatchers|CreateEvent :!event BPTalktoObjectiveAutoGenFunc))
    (CallFunction|CompleteObjective)
    (Development|PrintString 0 "Complete Objective")))

(fn RemoveObjective
  (|CallParentFunction)
  (EventDispatchers|UnbindEventfromOnDialogueFinish (.DialogueComponent (Variables|Default|GetDialogueComponent)) (EventDispatchers|CreateEvent :!event BPTalktoObjectiveAutoGenFunc)))