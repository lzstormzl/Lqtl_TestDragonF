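; BP_LocationObjective is a quest objective that completes when the player character enters a location volume.
; Activating it as a normal or special event objective binds an overlap handler to the Location component.
; The handler completes the objective when the overlapping actor's class is exactly Main_Social_BP.
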(fn LocationReached
  (Collision|BindEventtoOnComponentBeginOverlap (Variables|Default|GetLocation) (EventDispatchers|CreateEvent :!event OnOverlapLocation)))

(fn ActiveNormalObjective
  (CallFunction|LocationReached))

(fn ActiveSpecialEventObjective
  (CallFunction|LocationReached))

(fn OnOverlapLocation
  (params (OverlappedComponent :type Primitive%20Component%20Object%20Reference) (OtherActor :type Actor%20Object%20Reference) (OtherComp :type Primitive%20Component%20Object%20Reference) (OtherBodyIndex :type Integer) (bFromSweep :type Boolean) (SweepResult :type Hit%20Result%20Structure%20%28by%20ref%29))
  (if (== (Utilities|GetClass OtherActor) "/Game/Characters/Main/Social/Main_Social_BP.Main_Social_BP_C")
    (CallFunction|CompleteObjective)
    (return)))