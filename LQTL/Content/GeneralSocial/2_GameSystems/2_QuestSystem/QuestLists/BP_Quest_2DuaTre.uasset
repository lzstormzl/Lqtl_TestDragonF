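; Quest actor for "2DuaTre" that switches the TronTim calendar event on when the quest starts and off when it completes.
; Both steps show the game instance's screen transition and wait for its TransIn animation to finish, using a self-unbinding delegate.
; Behind the transition, the Calendar Manager triggers or completes the event and starts a new phase, then the widget closes.
; Parent completion logic is deferred until that sequence ends.
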(event Custom|DoLogic
  (bind _calendarmanager (CallFunction|GetCalendarManager))
  (bind _asthuy_tinh_game_instance (Game|GetGameInstance))
  (bind _screentransition (Variables|/Game/GeneralSocial/ThuyTinh_GameInstance.ThuyTinh_GameInstance_C|GetScreenTransition _asthuy_tinh_game_instance))
  (Class|UserWidget|UnbindfromAnimationFinished _screentransition (Variables|/Game/GeneralSocial/1_Social/4_Widget/ScreenTransitionWidget.ScreenTransitionWidget_C|GetTransIn _screentransition) (delegate Custom|DoLogic))
  (Default|TriggerEvent _calendarmanager "TronTim")
  (Default|CallOnStartNewPhase _calendarmanager)
  (Default|CloseWidget (Variables|/Game/GeneralSocial/ThuyTinh_GameInstance.ThuyTinh_GameInstance_C|GetScreenTransition (.AsThuy%20Tinh%20Game%20Instance (Game|GetGameInstance)))))

(event Custom|DoExtraLogicCompleteQuest
  (bind _asthuy_tinh_game_instance (Game|GetGameInstance))
  (bind _screentransition (Variables|/Game/GeneralSocial/ThuyTinh_GameInstance.ThuyTinh_GameInstance_C|GetScreenTransition _asthuy_tinh_game_instance))
  (Class|UserWidget|UnbindfromAnimationFinished _screentransition (Variables|/Game/GeneralSocial/1_Social/4_Widget/ScreenTransitionWidget.ScreenTransitionWidget_C|GetTransIn _screentransition) (delegate Custom|DoExtraLogicCompleteQuest))
  (Default|CompleteEvent (CallFunction|GetCalendarManager) (Utilities|Name|MakeLiteralName "TronTim"))
  (Default|CallOnStartNewPhase (CallFunction|GetCalendarManager))
  (Default|CloseWidget (Variables|/Game/GeneralSocial/ThuyTinh_GameInstance.ThuyTinh_GameInstance_C|GetScreenTransition (.AsThuy%20Tinh%20Game%20Instance (Game|GetGameInstance))))
  (|CallParentFunction))

(event EventBeginPlay
  (|CallParentFunction) ; This node is disabled and will not be called.\nDrag off pins to build functionality.
)

(event Collision|EventActorBeginOverlap
  (params (OtherActor :type Actor%20Object%20Reference)))

(event EventTick
  (params (DeltaSeconds :type Float%20%28single-precision%29)))

(event EventInitialQuest
  (bind _asthuy_tinh_game_instance (Game|GetGameInstance))
  (bind _screentransition (Variables|/Game/GeneralSocial/ThuyTinh_GameInstance.ThuyTinh_GameInstance_C|GetScreenTransition _asthuy_tinh_game_instance))
  (|CallParentFunction)
  (Default|ShowWidget _screentransition)
  (Class|UserWidget|BindtoAnimationFinished _screentransition (Variables|/Game/GeneralSocial/1_Social/4_Widget/ScreenTransitionWidget.ScreenTransitionWidget_C|GetTransIn _screentransition) (delegate Custom|DoLogic)))

(event EventCompleteQuest
  (bind _asthuy_tinh_game_instance (Game|GetGameInstance))
  (bind _screentransition (Variables|/Game/GeneralSocial/ThuyTinh_GameInstance.ThuyTinh_GameInstance_C|GetScreenTransition _asthuy_tinh_game_instance))
  (Default|ShowWidget _screentransition)
  (Class|UserWidget|BindtoAnimationFinished _screentransition (Variables|/Game/GeneralSocial/1_Social/4_Widget/ScreenTransitionWidget.ScreenTransitionWidget_C|GetTransIn _screentransition) (delegate Custom|DoExtraLogicCompleteQuest)))

(fn ConstructionScript
  (|CallParentFunction))