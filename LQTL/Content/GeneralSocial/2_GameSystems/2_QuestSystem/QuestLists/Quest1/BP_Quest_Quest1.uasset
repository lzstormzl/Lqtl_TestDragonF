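; Quest actor for Quest1 in the social game's quest system, extending a parent quest class.
; On BeginPlay it spawns a location trigger in the LabSocialMap level only, passing itself as that trigger's quest reference.
; When InitialQuest runs, it calls the parent logic, then immediately asks the quest manager to complete this quest by class.
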(event EventBeginPlay
  (|CallParentFunction)
  (bind _returnvalue (Game|GetCurrentLevelName true))
  (if (Utilities|Enum|Equal(Enum) _returnvalue "LabSocialMap")
    (Game|SpawnActorfromClass "/Game/GeneralSocial/2_GameSystems/2_QuestSystem/QuestLists/Quest1/BP_Quest_LocationTrigger.BP_Quest_LocationTrigger_C" (Math|Transform|MakeTransform "0, 0, 0" "0, 0, 0" "1.000000,1.000000,1.000000") "Undefined" "MultiplyWithRoot" 0 self 0)))

(event Collision|EventActorBeginOverlap
  (params (OtherActor :type Actor%20Object%20Reference))
  (|CallParentFunction OtherActor) ; This node is disabled and will not be called.\nDrag off pins to build functionality.
)

(event EventTick
  (params (DeltaSeconds :type Float%20%28single-precision%29))
  (|CallParentFunction DeltaSeconds) ; This node is disabled and will not be called.\nDrag off pins to build functionality.
)

(event EventInitialQuest
  (|CallParentFunction)
  (bind _questmanager (CallFunction|GetQuestManager))
  (CallFunction|CompleteQuest _questmanager "None" "BP_Quest_Quest1_C"))

(fn ConstructionScript
  (|CallParentFunction))