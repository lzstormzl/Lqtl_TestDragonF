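; BP_CompanionBase is a base companion NPC that grants stat bonuses to the player.
; PlusCompanionStat sends its Tri, Dung, Cam and Kien bonuses to player character 0 through PlusPlayerStats messages, one per stat type.
; MinusCompanionStat sends the same amounts negated to remove them.
; BeginPlay and construction only call the parent, and nothing here triggers either stat event.
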(event Custom|PlusCompanionStat
  (bind _returnvalue (Game|GetPlayerCharacter 0))
  (Class|BPIThuyTinhSocial|PlusPlayerStats(Message) _returnvalue "None" (Variables|Stats|Bonus|GetTriBonus))
  (Class|BPIThuyTinhSocial|PlusPlayerStats(Message) _returnvalue "None" (Variables|Stats|Bonus|GetDungBonus) "NewEnumerator1")
  (Class|BPIThuyTinhSocial|PlusPlayerStats(Message) _returnvalue "None" (Variables|Stats|Bonus|GetCamBonus) "NewEnumerator2")
  (Class|BPIThuyTinhSocial|PlusPlayerStats(Message) _returnvalue "None" (Variables|Stats|Bonus|GetKienBonus) "NewEnumerator3"))

(event Custom|MinusCompanionStat
  (bind _returnvalue (Game|GetPlayerCharacter 0))
  (Class|BPIThuyTinhSocial|PlusPlayerStats(Message) _returnvalue "None" (* (Variables|Stats|Bonus|GetTriBonus) -1))
  (Class|BPIThuyTinhSocial|PlusPlayerStats(Message) _returnvalue "None" (* (Variables|Stats|Bonus|GetDungBonus) -1) "NewEnumerator1")
  (Class|BPIThuyTinhSocial|PlusPlayerStats(Message) _returnvalue "None" (* (Variables|Stats|Bonus|GetCamBonus) -1) "NewEnumerator2")
  (Class|BPIThuyTinhSocial|PlusPlayerStats(Message) _returnvalue "None" (* (Variables|Stats|Bonus|GetKienBonus) -1) "NewEnumerator3"))

(event EventBeginPlay
  (|CallParentFunction))

(fn ConstructionScript
  (|CallParentFunction))