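; BP_Entity is a character or object blueprint that can show a quest navigation marker over itself.
; TurnOnQuestNavigation shows the QuestNavigator component when the entity's CurrentMap is "None" and its CanMoveToMap list contains the requested map, and hides it otherwise.
; Getter functions expose the entity's Name and its QuestNavigator component.
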(fn ConstructionScript)

(fn OpenNavigatorWidget
  (Rendering|SetVisibility (Variables|Default|GetQuestNavigator) true false))

(fn TurnonQuestNavigation
  (params (MapNavigation :type Name))
  (if (and (== (Variables|Default|GetCurrentMap) "") (Utilities|Array|ContainsItem (Variables|Default|GetCanMoveToMap) MapNavigation))
    (CallFunction|OpenNavigatorWidget)
    (else
      (Rendering|SetVisibility (Variables|Default|GetQuestNavigator) false false))))

(fn GetName
  (return (Variables|Default|GetName)))

(fn GetQuestNavigatorSocket
  (return (Variables|Default|GetQuestNavigator)))