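; BP_Door_Dialogue is a door object that starts a dialogue with the player when its NPC logic runs.
; It overrides DoNPCOwnLogic, calls the parent, then has the social player character start dialogue from the table and row in its DialogueID0 handle.
; The other events are disabled stubs and the construction script only calls the parent, so all other behavior is inherited.
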(event EventBeginPlay
  (|CallParentFunction) ; This node is disabled and will not be called.\nDrag off pins to build functionality.
)

(event Collision|EventActorBeginOverlap
  (params (OtherActor :type Actor%20Object%20Reference))
  (|CallParentFunction OtherActor) ; This node is disabled and will not be called.\nDrag off pins to build functionality.
)

(event EventTick
  (params (DeltaSeconds :type Float%20%28single-precision%29))
  (|CallParentFunction DeltaSeconds) ; This node is disabled and will not be called.\nDrag off pins to build functionality.
)

(event EventDoNPCOwnLogic
  (bind _dialogueid_0 (Variables|Default|GetDialogueID_0))
  (bind (_datatable _rowname) (Utilities|Struct|BreakDataTableRowHandle _dialogueid_0))
  (|CallParentFunction)
  (Default|StartDialogue (CallFunction|GetPlayerCharacterSocial) _datatable _rowname))

(fn ConstructionScript
  (|CallParentFunction))